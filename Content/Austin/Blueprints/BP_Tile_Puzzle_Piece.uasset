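; BP_Tile_Puzzle_Piece is a Lights Out-style puzzle tile that switches between on and off materials.
; When the 2D side-scroller character overlaps PuzzleSpace, it flips its own Active state and that of each BorderingSpace tile, printing each neighbour's new state.
; TileCheck sets the cube material from Active and re-arms itself on a one-second timer, so flipped neighbours update visually on their next poll.
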(event OnComponentBeginOverlap(PuzzleSpace)
  (params (OverlappedComponent :type Primitive%20Component%20Object%20Reference) (OtherActor :type Actor%20Object%20Reference) (OtherComp :type Primitive%20Component%20Object%20Reference) (OtherBodyIndex :type Integer) (bFromSweep :type Boolean) (SweepResult :type Hit%20Result%20Structure%20%28by%20ref%29))
  (if (== (Utilities|GetClass OtherActor) "/Game/2DSideScrollerBP/Blueprints/2DSideScrollerCharacter.2DSideScrollerCharacter_C")
    (if (Variables|Default|GetActive?)
      (Variables|Default|SetActive? false)
      (else
        (Variables|Default|SetActive? true)))
    (for _array_element (Variables|Default|GetBorderingSpace)
      (if (Variables|BP_Tile_Puzzle_Piece_C|GetActive? _array_element)
        (Variables|BP_Tile_Puzzle_Piece_C|SetActive? _array_element false)
        (Development|PrintString "Inactive")
        (else
          (Variables|BP_Tile_Puzzle_Piece_C|SetActive? _array_element true)
          (Development|PrintString "Active")))
      (CallFunction|TileCheck))))

(event Custom|Tile%20Check
  (bind _cube (Variables|Default|GetCube))
  (Utilities|Time|SetTimerbyEvent (delegate Custom|Tile%20Check) 1.0)
  (if (Variables|Default|GetActive?)
    (Rendering|Material|SetMaterial _cube 0 "/Game/Austin/Materials/M_TileOn.M_TileOn")
    (else
      (Rendering|Material|SetMaterial _cube 0 "/Game/Austin/Materials/M_TileOff.M_TileOff"))))

(event EventBeginPlay
  (CallFunction|TileCheck))

(event EventTick
  (params (DeltaSeconds :type Float%20%28single-precision%29)))

(fn ConstructionScript)
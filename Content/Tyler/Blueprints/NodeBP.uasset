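; NodeBP is a room node actor that reacts when the third-person character enters or leaves its Box trigger.
; If the node is Locked, the overlap shows or hides its Widget, which is hidden at BeginPlay.
; Otherwise it forwards the begin and end overlap events to a HUB reference, passing its RoomType.
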(event OnComponentBeginOverlap(Box)
  (params (OverlappedComponent :type Primitive%20Component%20Object%20Reference) (OtherActor :type Actor%20Object%20Reference) (OtherComp :type Primitive%20Component%20Object%20Reference) (OtherBodyIndex :type Integer) (bFromSweep :type Boolean) (SweepResult :type Hit%20Result%20Structure%20%28by%20ref%29))
  (if (== (Utilities|GetClass OtherActor) "/Game/ThirdPerson/Blueprints/BP_ThirdPersonCharacter.BP_ThirdPersonCharacter_C")
    (if (Variables|Default|GetLocked)
      (Rendering|SetVisibility (Variables|Default|GetWidget) true false)
      (else
        (Default|FromNodeBeginOverlap (Variables|Default|GetHUB) (Variables|Default|GetRoomType))))))

(event OnComponentEndOverlap(Box)
  (params (OverlappedComponent :type Primitive%20Component%20Object%20Reference) (OtherActor :type Actor%20Object%20Reference) (OtherComp :type Primitive%20Component%20Object%20Reference) (OtherBodyIndex :type Integer))
  (if (== (Utilities|GetClass OtherActor) "/Game/ThirdPerson/Blueprints/BP_ThirdPersonCharacter.BP_ThirdPersonCharacter_C")
    (if (Variables|Default|GetLocked)
      (Rendering|SetVisibility (Variables|Default|GetWidget) false false)
      (else
        (Default|FromNodeEndOverlap (Variables|Default|GetHUB) (Variables|Default|GetRoomType))))))

(event EventBeginPlay
  (Rendering|SetVisibility (Variables|Default|GetWidget) false false))

(fn ConstructionScript)
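; Coin Crawl combat room, started and ended from the HUB and won when the room timer finishes.
; Start gathers the players and spawns eight enemies of two AI types around the room's perimeter.
; Each kill spawns a replacement at a random position, always the first type because RandomInteger(1) only returns 0.
; Ending or winning destroys Minion-tagged actors; the coin-carry event is empty.
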(event Custom|StartCarryingCoin
  ;[1 1 1] Game Controls
)

(event EventBeginfromHUB
  ;[1 1 1] Game Setup
  (Variables|Default|SetLoop true)
  (Variables|Default|SetAllDead? false)
  (CallFunction|StartRoomGetAllPlayersfromHUB)
  (CallFunction|SpawnEnemy "-1000.000000,-1000.000000,0.000000" "NewEnumerator0" false)
  (CallFunction|SpawnEnemy "-1000.000000,0.000000,0.000000" "NewEnumerator3" false)
  (CallFunction|SpawnEnemy "-1000.000000,1000.000000,0.000000" "NewEnumerator0" false)
  (CallFunction|SpawnEnemy "0.000000,-1000.000000,0.000000" "NewEnumerator3" false)
  (CallFunction|SpawnEnemy "0.000000,1000.000000,0.000000" "NewEnumerator0" false)
  (CallFunction|SpawnEnemy "1000.000000,-1000.000000,0.000000" "NewEnumerator0" false)
  (CallFunction|SpawnEnemy "1000.000000,0.000000,0.000000" "NewEnumerator3" false)
  (CallFunction|SpawnEnemy "1000.000000,1000.000000,0.000000" "NewEnumerator0" false))

(event EventEnemyKilled
  (bind _returnvalue (Math|Random|RandomFloatinRange -1e+03 1e+03))
  (bind _returnvalue_2 (Math|Vector|MakeVector _returnvalue _returnvalue 0.0))
  ;[1 0.3018 0.3217] Enemy Respawn
  (Variables|Default|SetSpawnRoll (Math|Random|RandomInteger 1))
  (Utilities|FlowControl|Sequence
    (:then_0
      (if (== (Variables|Default|GetSpawnRoll) 0)
        (CallFunction|SpawnEnemy _returnvalue_2 "NewEnumerator0" false)))
    (:then_1
      (if (== (Variables|Default|GetSpawnRoll) 1)
        (CallFunction|SpawnEnemy _returnvalue_2 "NewEnumerator3" false)))))

(event EventRoomTimerFinished
  ;[1 1 1] Game Controls
  (CallFunction|RoomWon)
  (bind _outactors (Actor|GetAllActorswithTag "Minion"))
  (for _array_element _outactors
    (Actor|DestroyActor _array_element)))

(event EventEndfromHUB
  ;[1 1 1] Game Controls
  (CallFunction|KillAllMeleeEnemies)
  (bind _outactors (Actor|GetAllActorswithTag "Minion"))
  (for _array_element _outactors
    (Actor|DestroyActor _array_element)))

(event EventTick
  (params (DeltaSeconds :type Float%20%28single-precision%29))
  ;[1 1 1] Game Controls
)

(fn ConstructionScript
  (|CallParentFunction))
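; Child laser beam actor for the light puzzle, coloring itself through a dynamic material on BeginPlay.
; Each tick, a thin box trace along its up vector scales the mesh to the hit or full range.
; It tracks the last hit actor to drive BPI_Lasers messages, reflector-based repositioning and removal of following lasers.
; CancelTargetHit notifies or deactivates that target and optionally destroys the beam; several helper functions are empty stubs.
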(event EventBeginPlay
  (CallFunction|ChangeColor))

(event EventTick
  (params (DeltaSeconds :type Float%20%28single-precision%29))
  (CallFunction|SetEndPoint))

(fn ConstructionScript
  (|CallParentFunction))

(fn ChangeColor
  (bind _returnvalue (Rendering|Material|CreateDynamicMaterialInstance (Variables|Default|GetStaticMesh) 0 "/Game/Tyler/Blueprints/Rooms/LightPuzzle/M_Laser.M_Laser" "None" :!class /Script/Engine.PrimitiveComponent))
  (Rendering|Material|SetVectorParameterValue _returnvalue "Color" (Variables|Default|GetLaserColor) :!class /Script/Engine.MaterialInstanceDynamic))

(fn SetEndPoint
  (bind _returnvalue (Transformation|GetActorLocation))
  (bind _returnvalue_2 (Transformation|GetActorUpVector))
  (bind _returnvalue_3 (* _returnvalue_2 2.0))
  (bind _returnvalue_4 (+ _returnvalue _returnvalue_3))
  (bind _outhit (Collision|BoxTraceByChannel _returnvalue_4 (+ _returnvalue_4 (* _returnvalue_2 (Variables|Default|GetL-Range))) "0.500000,0.500000,0.500000" "0, 0, 0" "TraceTypeQuery1" false 0 "None"))
  (bind _output_get (Variables|Default|SetL-HitInfo _outhit))
  (Variables|Default|SetLaser%20Hit%20Actor (.HitActor (Collision|BreakHitResult _output_get)))
  (Transformation|SetWorldScale3D (Variables|Default|GetStaticMesh) (Math|Vector|MakeVector 0.1 0.1 (Math|Float|SelectFloat (/ (+ (.Distance (Collision|BreakHitResult _output_get)) 1.0) 1e+02) (/ (Variables|Default|GetL-Range) 1e+02) (.bBlockingHit (Collision|BreakHitResult _output_get)))))
  (bind _laser_hit_actor (Variables|Default|GetLaser%20Hit%20Actor)
    (:then
      (bind _asbp_laser_cube (Utilities|Casting|CastToBP_LaserCube _laser_hit_actor)
        (:then
          (if (Utilities|Array|IsEmpty (Variables|/Game/Tyler/Blueprints/Rooms/LightPuzzle/BP_LaserParent.BP_LaserParent_C|GetLasersAttached _asbp_laser_cube))
            (Utilities|FlowControl|Sequence :!label _label
              (:then_0
                (if (== (Variables|Default|GetLast%20Hit%20Actor) (Variables|Default|GetLaser%20Hit%20Actor))
                  (bind _asbp_laser_reflecter (Utilities|Casting|CastToBP_LaserReflecter (Variables|Default|GetLast%20Hit%20Actor)))
                  (Transformation|SetActorLocation (.ImpactPoint (Collision|BreakHitResult (Variables|Default|GetL-HitInfo))) false false)
                  (Transformation|SetActorRotation (Default|CalculateRotate _asbp_laser_reflecter (.ImpactPoint (Collision|BreakHitResult (Variables|Default|GetL-HitInfo))) (.TraceStart (Collision|BreakHitResult (Variables|Default|GetL-HitInfo))) (.ImpactNormal (Collision|BreakHitResult (Variables|Default|GetL-HitInfo)))))
                  (Development|PrintString "1")
                  (else
                    (Utilities|FlowControl|Sequence
                      (:then_0
                        (if (Utilities|DoesObjectImplementInterface (Variables|Default|GetLast%20Hit%20Actor) "/Game/Tyler/Blueprints/BlueprintInterface/BPI_Lasers.BPI_Lasers_C")
                          (Default|RemoveFollowingLasers (Variables|Default|GetSpawnReference) self)))
                      (:then_1
                        (if (Utilities|DoesObjectImplementInterface (Variables|Default|GetLaser%20Hit%20Actor) "/Game/Tyler/Blueprints/BlueprintInterface/BPI_Lasers.BPI_Lasers_C")
                          (Class|BPILasers|LaserRefract(Message) (Variables|Default|GetLast%20Hit%20Actor) true (Variables|Default|GetL-HitInfo) self)))))))
              (:then_1
                (bind _laser_hit_actor_2 (Variables|Default|GetLaser%20Hit%20Actor)
                  (:then
                    (Variables|Default|SetLast%20Hit%20Actor _laser_hit_actor_2))
                  (:else))))))
        (:CastFailed
          (goto _label))))
    (:else
      (if (Utilities|DoesObjectImplementInterface (Variables|Default|GetLaser%20Hit%20Actor) "/Game/Tyler/Blueprints/BlueprintInterface/BPI_Lasers.BPI_Lasers_C")
        (Class|BPILasers|LaserRefract(Message) (Variables|Default|GetLast%20Hit%20Actor) true (Variables|Default|GetL-HitInfo) self)
        (else
          (Variables|Default|SetLast%20Hit%20Actor (Variables|Default|GetLaser%20Hit%20Actor)))))))

(fn UpdateID
  (params (Append :type String))
  (return (Utilities|String|Append (Variables|Default|GetLaser_ID) Append)))

(fn CancelTargetHit
  (params (Override :type Boolean))
  (Utilities|FlowControl|Sequence
    (:then_0
      (bind _last_hit_actor (Variables|Default|GetLast%20Hit%20Actor)
        (:then
          (bind _asbp_laser_parent (Utilities|Casting|CastToBP_LaserParent _last_hit_actor))
          (if (and (Utilities|DoesObjectImplementInterface _asbp_laser_parent "/Game/Tyler/Blueprints/BlueprintInterface/BPI_Lasers.BPI_Lasers_C") (Utilities|Array|IsEmpty (Variables|/Game/Tyler/Blueprints/Rooms/LightPuzzle/BP_LaserParent.BP_LaserParent_C|GetLasersAttached _asbp_laser_parent)))
            (Class|BPILasers|LaserRefract(Message) :self (Variables|Default|GetLast%20Hit%20Actor) :NewParam self)
            (else
              (Variables|/Game/Tyler/Blueprints/Rooms/LightPuzzle/BP_LaserParent.BP_LaserParent_C|SetActive? _asbp_laser_parent false))))
        (:else)))
    (:then_1
      (if Override
        (return false)
        (else
          (Actor|DestroyActor)
          (return true))))))

(fn UpdateLaserSize
  (params (Hit%20Result :type Hit%20Result%20Structure%20%28by%20ref%29) (Range :type Float%20%28double-precision%29)))

(fn DifferentActorHit
  (params (Hit%20Actor :type Object%20Object%20Reference) (P-HitInformation :type Hit%20Result%20Structure)))

(fn SameActorHit
  (params (Hit%20Result :type Hit%20Result%20Structure%20%28by%20ref%29)))

(fn NothingHit
  (params (P-HitInformation :type Hit%20Result%20Structure)))

(fn LaserRefract
  (params (Hit :type Boolean) (HitResult :type Hit%20Result%20Structure) (NewParam :type BP%20Laser%20Child%20Object%20Reference))
  (return 0))
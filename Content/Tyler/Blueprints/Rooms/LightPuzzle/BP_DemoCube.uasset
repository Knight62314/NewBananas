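; BP_DemoCube is a light-puzzle cube that redirects a laser hitting it.
; LaserRefract spawns a same-colored BP_LaserChild along the cube's arrow, attaches it to the mesh and registers it with the cube and the laser's SpawnReference.
; A non-hit call with a valid laser clears all lasers.
; The guard against repeated hits is disconnected, so every hit call spawns another child.
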(event EventBeginPlay)

(event Collision|EventActorBeginOverlap
  (params (OtherActor :type Actor%20Object%20Reference)))

(event EventTick
  (params (DeltaSeconds :type Float%20%28single-precision%29)))

(fn ConstructionScript
  (|CallParentFunction))

(fn LaserRefract
  (params (Hit :type Boolean) (HitResult :type Hit%20Result%20Structure) (Laser%20Hit :type BP%20Laser%20Child%20Object%20Reference))
  (bind _arrow (Variables|Default|GetArrow))
  (Utilities|IsValid Laser%20Hit
    (:Is%20Valid
      (Variables|Default|SetSpawnReference (Variables|/Game/Tyler/Blueprints/Rooms/LightPuzzle/BP_LaserParent.BP_LaserParent_C|GetSpawnReference Laser%20Hit))
      (bind _output_get (Variables|Default|SetActive? Hit))
      (if _output_get
        (bind _returnvalue (Game|SpawnActorfromClass "/Game/Tyler/Blueprints/Rooms/LightPuzzle/BP_LaserChild.BP_LaserChild_C" (Math|Transform|MakeTransform (Transformation|GetWorldLocation _arrow) (Math|Rotator|MakeRotfromZ (Math|Vector|GetForwardVector _arrow)) "1.000000,1.000000,1.000000") "Undefined" "MultiplyWithRoot" 0 0 (Default|UpdateID Laser%20Hit "C") (Variables|/Game/Tyler/Blueprints/Rooms/LightPuzzle/BP_LaserParent.BP_LaserParent_C|GetLaserColor Laser%20Hit) (Variables|Default|GetSpawnReference) "(R=0.000000,G=0.000000,B=0.000000,A=0.000000)" 0))
        (Transformation|AttachComponentToComponent _returnvalue (Variables|Default|GetStaticMesh) "None" "KeepWorld" "KeepWorld" "KeepRelative" false)
        (Utilities|Array|Add (Variables|Default|GetLasersAttached) _returnvalue)
        (Utilities|Array|Add (Variables|/Game/Tyler/Blueprints/Rooms/LightPuzzle/BP_LaserSpawn.BP_LaserSpawn_C|GetChild%20Lasers (Variables|Default|GetSpawnReference)) _returnvalue)
        (return 0)
        (else
          (CallFunction|ClearAllLasers))))))
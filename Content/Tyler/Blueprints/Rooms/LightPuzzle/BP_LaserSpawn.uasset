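; BP_LaserSpawn is the emitter of the light puzzle, spawning the first BP_LaserChild at its arrow with its color, display-name ID and a self reference.
; It tracks child lasers in an array.
; RemoveFollowingLasers walks it backwards, using substring ID matching to find a given laser and its descendants, cancels their target hits and removes those that report success.
; LaserRefract is an empty stub here.
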(event EventBeginPlay
  (bind _lasercolor (Variables|Default|GetLaserColor))
  (Variables|Default|SetSpawnReference self)
  (Variables|Default|SetID (Utilities|GetDisplayName self))
  (bind _returnvalue (Game|SpawnActorfromClass "/Game/Tyler/Blueprints/Rooms/LightPuzzle/BP_LaserChild.BP_LaserChild_C" (Math|Transform|MakeTransform (Transformation|GetWorldLocation (Variables|Default|GetArrow)) (Transformation|GetActorRotation) "1.000000,1.000000,1.000000") "Undefined" "MultiplyWithRoot" 0 0 (Variables|Default|GetID) _lasercolor (Variables|Default|GetSpawnReference) "(R=0.000000,G=0.000000,B=0.000000,A=0.000000)" 0))
  (Utilities|Array|Add (Variables|Default|GetChild%20Lasers) _returnvalue)
  (Variables|Default|SetSpawnLaserColor _lasercolor))

(fn ConstructionScript
  (|CallParentFunction))

(fn RemoveFollowingLasers
  (params (Laser%20Reference :type BP%20Laser%20Child%20Object%20Reference))
  (LocalVariables|SetID%20Removed (Variables|/Game/Tyler/Blueprints/Rooms/LightPuzzle/BP_LaserChild.BP_LaserChild_C|GetLaser_ID Laser%20Reference))
  (bind _arrayelement (Utilities|Array|ReverseforEachLoop (Variables|Default|GetChild%20Lasers))
    (:LoopBody
      (Utilities|IsValid _arrayelement
        (:Is%20Valid
          (if (Utilities|String|Contains (Variables|/Game/Tyler/Blueprints/Rooms/LightPuzzle/BP_LaserChild.BP_LaserChild_C|GetLaser_ID _arrayelement) (LocalVariables|GetID%20Removed))
            (bind _remove (Default|CancelTargetHit _arrayelement (Utilities|Enum|Equal(Enum) (Variables|/Game/Tyler/Blueprints/Rooms/LightPuzzle/BP_LaserChild.BP_LaserChild_C|GetLaser_ID _arrayelement) (LocalVariables|GetID%20Removed))))
            (if _remove
              (Utilities|Array|RemoveItem (Variables|Default|GetChild%20Lasers) _arrayelement))))))))

(fn LaserRefract
  (params (Hit :type Boolean) (HitResult :type Hit%20Result%20Structure) (Laser%20Hit :type BP%20Laser%20Child%20Object%20Reference))
  (return 0))
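; Laser puzzle room with red, green and blue lasers, started from the HUB.
; On the server, setup picks six distinct slots from twelve, then spawns emitters, targets and five reflectors (rotations randomized at BeginPlay) via server-to-multicast events.
; Four player-triggered buttons spawn laser cubes, gated by one shared flag that resets five seconds after overlap ends.
; A timer polls targets, returning to the HUB once all match; a box overlap also returns there.
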(event OnComponentBeginOverlap(Box)
  (params (OverlappedComponent :type Primitive%20Component%20Object%20Reference) (OtherActor :type Actor%20Object%20Reference) (OtherComp :type Primitive%20Component%20Object%20Reference) (OtherBodyIndex :type Integer) (bFromSweep :type Boolean) (SweepResult :type Hit%20Result%20Structure%20%28by%20ref%29))
  ;[1 1 1] Laser Puzzle
  ;;[0 1 0.5652] End Puzzle
  (if (== (Utilities|GetClass OtherActor) "/Game/ThirdPerson/Blueprints/BP_ThirdPersonCharacter.BP_ThirdPersonCharacter_C")
    (Default|MovetoHUBFunction (Variables|Default|GetHUB) self)))

(event OnComponentBeginOverlap(North)
  (params (OverlappedComponent :type Primitive%20Component%20Object%20Reference) (OtherActor :type Actor%20Object%20Reference) (OtherComp :type Primitive%20Component%20Object%20Reference) (OtherBodyIndex :type Integer) (bFromSweep :type Boolean) (SweepResult :type Hit%20Result%20Structure%20%28by%20ref%29))
  ;[1 1 1] Laser Puzzle
  ;;[1 0.1534 0.9369] Laser Cube Spawners
  (if (== (Utilities|GetClass OtherActor) "/Game/ThirdPerson/Blueprints/BP_ThirdPersonCharacter.BP_ThirdPersonCharacter_C")
    (CallFunction|NorthServerData)))

(event OnComponentEndOverlap(North)
  (params (OverlappedComponent :type Primitive%20Component%20Object%20Reference) (OtherActor :type Actor%20Object%20Reference) (OtherComp :type Primitive%20Component%20Object%20Reference) (OtherBodyIndex :type Integer))
  ;[1 1 1] Laser Puzzle
  ;;[1 0.1534 0.9369] Laser Cube Spawners
  (Utilities|FlowControl|Delay 5.0)
  (Variables|Default|SetButtonPressed? false))

(event OnComponentBeginOverlap(South)
  (params (OverlappedComponent :type Primitive%20Component%20Object%20Reference) (OtherActor :type Actor%20Object%20Reference) (OtherComp :type Primitive%20Component%20Object%20Reference) (OtherBodyIndex :type Integer) (bFromSweep :type Boolean) (SweepResult :type Hit%20Result%20Structure%20%28by%20ref%29))
  ;[1 1 1] Laser Puzzle
  ;;[1 0.1534 0.9369] Laser Cube Spawners
  (if (== (Utilities|GetClass OtherActor) "/Game/ThirdPerson/Blueprints/BP_ThirdPersonCharacter.BP_ThirdPersonCharacter_C")
    (CallFunction|SouthServerData)))

(event OnComponentEndOverlap(South)
  (params (OverlappedComponent :type Primitive%20Component%20Object%20Reference) (OtherActor :type Actor%20Object%20Reference) (OtherComp :type Primitive%20Component%20Object%20Reference) (OtherBodyIndex :type Integer))
  ;[1 1 1] Laser Puzzle
  ;;[1 0.1534 0.9369] Laser Cube Spawners
  (Utilities|FlowControl|Delay 5.0)
  (Variables|Default|SetButtonPressed? false))

(event OnComponentBeginOverlap(West)
  (params (OverlappedComponent :type Primitive%20Component%20Object%20Reference) (OtherActor :type Actor%20Object%20Reference) (OtherComp :type Primitive%20Component%20Object%20Reference) (OtherBodyIndex :type Integer) (bFromSweep :type Boolean) (SweepResult :type Hit%20Result%20Structure%20%28by%20ref%29))
  ;[1 1 1] Laser Puzzle
  ;;[1 0.1534 0.9369] Laser Cube Spawners
  (if (== (Utilities|GetClass OtherActor) "/Game/ThirdPerson/Blueprints/BP_ThirdPersonCharacter.BP_ThirdPersonCharacter_C")
    (CallFunction|WestServerData)))

(event OnComponentEndOverlap(West)
  (params (OverlappedComponent :type Primitive%20Component%20Object%20Reference) (OtherActor :type Actor%20Object%20Reference) (OtherComp :type Primitive%20Component%20Object%20Reference) (OtherBodyIndex :type Integer))
  ;[1 1 1] Laser Puzzle
  ;;[1 0.1534 0.9369] Laser Cube Spawners
  (Utilities|FlowControl|Delay 5.0)
  (Variables|Default|SetButtonPressed? false))

(event OnComponentBeginOverlap(East)
  (params (OverlappedComponent :type Primitive%20Component%20Object%20Reference) (OtherActor :type Actor%20Object%20Reference) (OtherComp :type Primitive%20Component%20Object%20Reference) (OtherBodyIndex :type Integer) (bFromSweep :type Boolean) (SweepResult :type Hit%20Result%20Structure%20%28by%20ref%29))
  ;[1 1 1] Laser Puzzle
  ;;[1 0.1534 0.9369] Laser Cube Spawners
  (if (== (Utilities|GetClass OtherActor) "/Game/ThirdPerson/Blueprints/BP_ThirdPersonCharacter.BP_ThirdPersonCharacter_C")
    (CallFunction|EastServerData)))

(event OnComponentEndOverlap(East)
  (params (OverlappedComponent :type Primitive%20Component%20Object%20Reference) (OtherActor :type Actor%20Object%20Reference) (OtherComp :type Primitive%20Component%20Object%20Reference) (OtherBodyIndex :type Integer))
  ;[1 1 1] Laser Puzzle
  ;;[1 0.1534 0.9369] Laser Cube Spawners
  (Utilities|FlowControl|Delay 5.0)
  (Variables|Default|SetButtonPressed? false))

(event Custom|Game%20Setup
  ;[1 1 1] Laser Puzzle
  ;;[0 0 0] Laser Starts
  ;;;[1 0 0] Red Start Location
  (bind _output_get (Variables|Default|SetRedStart (.OutItem (Utilities|Array|Random (Variables|Default|GetRedStarts)))))
  (Utilities|Array|Add (Variables|Default|GetTakenLocations) _output_get)
  ;;;[0 1 0] Green Start Location
  (Variables|Default|SetCurrent (.OutItem (Utilities|Array|Random (Variables|Default|GetGreenStarts))))
  (while (Utilities|Array|ContainsItem (Variables|Default|GetTakenLocations) (Variables|Default|GetCurrent))
    (Variables|Default|SetCurrent (.OutItem (Utilities|Array|Random (Variables|Default|GetGreenStarts)))))
  (bind _output_get_2 (Variables|Default|SetGreenStart (Variables|Default|GetCurrent)))
  (Utilities|Array|Add (Variables|Default|GetTakenLocations) _output_get_2)
  ;;;[0 0 1] Blue Start Location
  (Variables|Default|SetCurrent (.OutItem (Utilities|Array|Random (Variables|Default|GetBlueStarts))))
  (while (Utilities|Array|ContainsItem (Variables|Default|GetTakenLocations) (Variables|Default|GetCurrent))
    (Variables|Default|SetCurrent (.OutItem (Utilities|Array|Random (Variables|Default|GetBlueStarts)))))
  (bind _output_get_3 (Variables|Default|SetBlueStart (Variables|Default|GetCurrent)))
  (Utilities|Array|Add (Variables|Default|GetTakenLocations) _output_get_3)
  ;;[0.401 0.401 0.401] Laser Ends
  ;;;[1 0 0] Red End Location
  (Variables|Default|SetCurrent (.OutItem (Utilities|Array|Random (Variables|Default|GetRedEnds))))
  (while (Utilities|Array|ContainsItem (Variables|Default|GetTakenLocations) (Variables|Default|GetCurrent))
    (Variables|Default|SetCurrent (.OutItem (Utilities|Array|Random (Variables|Default|GetRedEnds)))))
  (bind _output_get_4 (Variables|Default|SetRedEnd (Variables|Default|GetCurrent)))
  (Utilities|Array|Add (Variables|Default|GetTakenLocations) _output_get_4)
  ;;;[0 1 0] Green End Location
  (Variables|Default|SetCurrent (.OutItem (Utilities|Array|Random (Variables|Default|GetGreenEnds))))
  (while (Utilities|Array|ContainsItem (Variables|Default|GetTakenLocations) (Variables|Default|GetCurrent))
    (Variables|Default|SetCurrent (.OutItem (Utilities|Array|Random (Variables|Default|GetGreenEnds)))))
  (bind _output_get_5 (Variables|Default|SetGreenEnd (Variables|Default|GetCurrent)))
  (Utilities|Array|Add (Variables|Default|GetTakenLocations) _output_get_5)
  ;;;[0 0 1] Blue End Location
  (Variables|Default|SetCurrent (.OutItem (Utilities|Array|Random (Variables|Default|GetBlueEnds))))
  (while (Utilities|Array|ContainsItem (Variables|Default|GetTakenLocations) (Variables|Default|GetCurrent))
    (Variables|Default|SetCurrent (.OutItem (Utilities|Array|Random (Variables|Default|GetBlueEnds)))))
  (bind _output_get_6 (Variables|Default|SetBlueEnd (Variables|Default|GetCurrent)))
  (Utilities|Array|Add (Variables|Default|GetTakenLocations) _output_get_6)
  (CallFunction|ServerData))

(event Custom|End%20Game
  ;[1 1 1] Laser Puzzle
  ;;[0 1 0.5652] End Puzzle
  (Utilities|FlowControl|Delay 2.0)
  (Default|MovetoHUBFunction (Variables|Default|GetHUB) self)
  (Variables|Default|SetRedMatch? false)
  (Variables|Default|SetBlueMatch? false)
  (Variables|Default|SetGreenMatch? false))

(event Custom|SouthMulti
  ;[1 1 1] Laser Puzzle
  ;;[1 0.1534 0.9369] Laser Cube Spawners
  (if (not (Variables|Default|GetButtonPressed?))
    (Variables|Default|SetButtonPressed? true)
    (Game|SpawnActorfromClass "/Game/Tyler/Blueprints/Rooms/LightPuzzle/BP_LaserCubeOne.BP_LaserCubeOne_C" (Math|Transform|MakeTransform (+ (Transformation|GetWorldLocation (Variables|Default|GetSouth%20Button)) "0.000000,0.000000,50.000000") "0.000000,90.000000,0.000000" "1.000000,1.000000,1.000000") "Undefined" "MultiplyWithRoot" 0 "(R=0.000000,G=0.000000,B=0.000000,A=0.000000)" 0 "(R=0.000000,G=0.000000,B=0.000000,A=0.000000)" 0)))

(event Custom|WestServerData
  ;[1 1 1] Laser Puzzle
  ;;[1 0.1534 0.9369] Laser Cube Spawners
  (CallFunction|WestMulti))

(event Custom|WestMulti
  ;[1 1 1] Laser Puzzle
  ;;[1 0.1534 0.9369] Laser Cube Spawners
  (if (not (Variables|Default|GetButtonPressed?))
    (Variables|Default|SetButtonPressed? true)
    (Game|SpawnActorfromClass "/Game/Tyler/Blueprints/Rooms/LightPuzzle/BP_LaserCubeOne.BP_LaserCubeOne_C" (Math|Transform|MakeTransform (+ (Transformation|GetWorldLocation (Variables|Default|GetWest%20Button)) "0.000000,0.000000,50.000000") "0.000000,180.000000,0.000000" "1.000000,1.000000,1.000000") "Undefined" "MultiplyWithRoot" 0 "(R=0.000000,G=0.000000,B=0.000000,A=0.000000)" 0 "(R=0.000000,G=0.000000,B=0.000000,A=0.000000)" 0)))

(event Custom|EastServerData
  ;[1 1 1] Laser Puzzle
  ;;[1 0.1534 0.9369] Laser Cube Spawners
  (CallFunction|EastMulti))

(event Custom|EastMulti
  ;[1 1 1] Laser Puzzle
  ;;[1 0.1534 0.9369] Laser Cube Spawners
  (if (not (Variables|Default|GetButtonPressed?))
    (Variables|Default|SetButtonPressed? true)
    (Game|SpawnActorfromClass "/Game/Tyler/Blueprints/Rooms/LightPuzzle/BP_LaserCubeOne.BP_LaserCubeOne_C" (Math|Transform|MakeTransform (+ (Transformation|GetWorldLocation (Variables|Default|GetEast%20Button)) "0.000000,0.000000,50.000000") "0, 0, 0" "1.000000,1.000000,1.000000") "Undefined" "MultiplyWithRoot" 0 "(R=0.000000,G=0.000000,B=0.000000,A=0.000000)" 0 "(R=0.000000,G=0.000000,B=0.000000,A=0.000000)" 0)))

(event Custom|Multicast
  (bind _startloc2 (Variables|Default|GetStartLoc2))
  (bind _startloc3 (Variables|Default|GetStartLoc3))
  (bind _startloc4 (Variables|Default|GetStartLoc4))
  (bind _startloc5 (Variables|Default|GetStartLoc5))
  (bind _startloc6 (Variables|Default|GetStartLoc6))
  (bind _startloc8 (Variables|Default|GetStartLoc8))
  (bind _startloc7 (Variables|Default|GetStartLoc7))
  (bind _startloc9 (Variables|Default|GetStartLoc9))
  (bind _startloc10 (Variables|Default|GetStartLoc10))
  (bind _startloc11 (Variables|Default|GetStartLoc11))
  (bind _startloc (Variables|Default|GetStartLoc))
  (bind _startloc1 (Variables|Default|GetStartLoc1))
  (bind _startloc2_2 (Variables|Default|GetStartLoc2))
  (bind _startloc3_2 (Variables|Default|GetStartLoc3))
  (bind _startloc4_2 (Variables|Default|GetStartLoc4))
  (bind _startloc5_2 (Variables|Default|GetStartLoc5))
  (bind _startloc6_2 (Variables|Default|GetStartLoc6))
  (bind _startloc8_2 (Variables|Default|GetStartLoc8))
  (bind _startloc7_2 (Variables|Default|GetStartLoc7))
  (bind _startloc9_2 (Variables|Default|GetStartLoc9))
  (bind _startloc10_2 (Variables|Default|GetStartLoc10))
  (bind _startloc11_2 (Variables|Default|GetStartLoc11))
  (bind _greenstart (Variables|Default|GetGreenStart))
  (bind _bluestart (Variables|Default|GetBlueStart))
  (bind _startloc_2 (Variables|Default|GetStartLoc))
  (bind _startloc1_2 (Variables|Default|GetStartLoc1))
  (bind _startloc2_3 (Variables|Default|GetStartLoc2))
  (bind _startloc3_3 (Variables|Default|GetStartLoc3))
  (bind _startloc4_3 (Variables|Default|GetStartLoc4))
  (bind _startloc5_3 (Variables|Default|GetStartLoc5))
  (bind _startloc6_3 (Variables|Default|GetStartLoc6))
  (bind _startloc8_3 (Variables|Default|GetStartLoc8))
  (bind _startloc7_3 (Variables|Default|GetStartLoc7))
  (bind _startloc9_3 (Variables|Default|GetStartLoc9))
  (bind _startloc10_3 (Variables|Default|GetStartLoc10))
  (bind _startloc11_3 (Variables|Default|GetStartLoc11))
  (bind _redstart (Variables|Default|GetRedStart))
  (bind _startloc_3 (Variables|Default|GetStartLoc))
  (bind _startloc1_3 (Variables|Default|GetStartLoc1))
  (bind _array (Utilities|Array|MakeArray _startloc_2 _startloc1_2 _startloc2_3 _startloc3_3 _startloc4_3 _startloc5_3 _startloc6_3 _startloc7_3 _startloc8_3 _startloc9_3 _startloc10_3 _startloc11_3))
  (bind _array_2 (Utilities|Array|MakeArray _startloc_3 _startloc1_3 _startloc2 _startloc3 _startloc4 _startloc5 _startloc6 _startloc7 _startloc8 _startloc9 _startloc10 _startloc11))
  (bind _array_3 (Utilities|Array|MakeArray _startloc _startloc1 _startloc2_2 _startloc3_2 _startloc4_2 _startloc5_2 _startloc6_2 _startloc7_2 _startloc8_2 _startloc9_2 _startloc10_2 _startloc11_2))
  (bind _output (Utilities|Array|Get(acopy) _array _redstart))
  (bind _output_2 (Utilities|Array|Get(acopy) _array_2 _greenstart))
  (bind _output_3 (Utilities|Array|Get(acopy) _array_3 _bluestart))
  ;[1 1 1] Laser Puzzle
  ;;[0.431 1 0.2445] Place Spawners & Targets
  (Utilities|FlowControl|Sequence
    (:then_0
      (bind _returnvalue (Game|SpawnActorfromClass "/Game/Tyler/Blueprints/Rooms/LightPuzzle/BP_LaserSpawn.BP_LaserSpawn_C" (Math|Transform|MakeTransform (Transformation|GetWorldLocation _output) (Transformation|GetWorldRotation _output) "1.000000,1.000000,1.000000") "Undefined" "MultiplyWithRoot" 0 0 (Variables|Default|GetRed) 0 "(R=0.000000,G=0.000000,B=0.000000,A=1.000000)" 0))
      (Variables|Default|SetSpawnPoint _returnvalue))
    (:then_1
      (bind _returnvalue_2 (Game|SpawnActorfromClass "/Game/Tyler/Blueprints/Rooms/LightPuzzle/BP_LaserSpawn.BP_LaserSpawn_C" (Math|Transform|MakeTransform (Transformation|GetWorldLocation _output_2) (Transformation|GetWorldRotation _output_2) "1.000000,1.000000,1.000000") "Undefined" "MultiplyWithRoot" 0 0 (Variables|Default|GetGreen) 0 "(R=0.000000,G=0.000000,B=0.000000,A=1.000000)" 0))
      (Variables|Default|SetSpawnPoint1 _returnvalue_2))
    (:then_2
      (bind _returnvalue_3 (Game|SpawnActorfromClass "/Game/Tyler/Blueprints/Rooms/LightPuzzle/BP_LaserSpawn.BP_LaserSpawn_C" (Math|Transform|MakeTransform (Transformation|GetWorldLocation _output_3) (Transformation|GetWorldRotation _output_3) "1.000000,1.000000,1.000000") "Undefined" "MultiplyWithRoot" 0 0 (Variables|Default|GetBlue) 0 "(R=0.000000,G=0.000000,B=0.000000,A=1.000000)" 0))
      (Variables|Default|SetSpawnPoint2 _returnvalue_3))
    (:then_3
      (bind _returnvalue_4 (Game|SpawnActorfromClass "/Game/Tyler/Blueprints/Rooms/LightPuzzle/BP_LaserTarget.BP_LaserTarget_C" (Math|Transform|MakeTransform (Transformation|GetWorldLocation (Utilities|Array|Get(acopy) (Utilities|Array|MakeArray (Variables|Default|GetStartLoc) (Variables|Default|GetStartLoc1) (Variables|Default|GetStartLoc2) (Variables|Default|GetStartLoc3) (Variables|Default|GetStartLoc4) (Variables|Default|GetStartLoc5) (Variables|Default|GetStartLoc6) (Variables|Default|GetStartLoc7) (Variables|Default|GetStartLoc8) (Variables|Default|GetStartLoc9) (Variables|Default|GetStartLoc10) (Variables|Default|GetStartLoc11)) (Variables|Default|GetRedEnd))) (Transformation|GetActorRotation) "1.000000,1.000000,1.000000") "Undefined" "MultiplyWithRoot" 0 "(R=0.000000,G=0.000000,B=0.000000,A=1.000000)" 0 (Variables|Default|GetRed) 0))
      (bind _output_get (Variables|Default|SetEndPoint _returnvalue_4))
      (Game|SpawnActorfromClass "/Game/Tyler/Blueprints/Rooms/LightPuzzle/BP_LaserChild.BP_LaserChild_C" (Math|Transform|MakeTransform (Transformation|GetWorldLocation (Variables|/Game/Tyler/Blueprints/Rooms/LightPuzzle/BP_LaserTarget.BP_LaserTarget_C|GetArrow _output_get)) (Transformation|GetActorRotation) "1.000000,1.000000,1.000000") "Undefined" "MultiplyWithRoot" 0 0 "" (Variables|Default|GetRed) 0 "(R=0.000000,G=0.000000,B=0.000000,A=0.000000)" 0)
      (Variables|Default|SetRedMatch? false))
    (:then_4
      (bind _returnvalue_5 (Game|SpawnActorfromClass "/Game/Tyler/Blueprints/Rooms/LightPuzzle/BP_LaserTarget.BP_LaserTarget_C" (Math|Transform|MakeTransform (Transformation|GetWorldLocation (Utilities|Array|Get(acopy) (Utilities|Array|MakeArray (Variables|Default|GetStartLoc) (Variables|Default|GetStartLoc1) (Variables|Default|GetStartLoc2) (Variables|Default|GetStartLoc3) (Variables|Default|GetStartLoc4) (Variables|Default|GetStartLoc5) (Variables|Default|GetStartLoc6) (Variables|Default|GetStartLoc7) (Variables|Default|GetStartLoc8) (Variables|Default|GetStartLoc9) (Variables|Default|GetStartLoc10) (Variables|Default|GetStartLoc11)) (Variables|Default|GetGreenEnd))) (Transformation|GetActorRotation) "1.000000,1.000000,1.000000") "Undefined" "MultiplyWithRoot" 0 "(R=0.000000,G=0.000000,B=0.000000,A=1.000000)" 0 (Variables|Default|GetGreen) 0))
      (bind _output_get_2 (Variables|Default|SetEndPoint1 _returnvalue_5))
      (Game|SpawnActorfromClass "/Game/Tyler/Blueprints/Rooms/LightPuzzle/BP_LaserChild.BP_LaserChild_C" (Math|Transform|MakeTransform (Transformation|GetWorldLocation (Variables|/Game/Tyler/Blueprints/Rooms/LightPuzzle/BP_LaserTarget.BP_LaserTarget_C|GetArrow _output_get_2)) (Transformation|GetActorRotation) "1.000000,1.000000,1.000000") "Undefined" "MultiplyWithRoot" 0 0 "" (Variables|Default|GetGreen) 0 "(R=0.000000,G=0.000000,B=0.000000,A=0.000000)" 0)
      (Variables|Default|SetGreenMatch? false))
    (:then_5
      (bind _returnvalue_6 (Game|SpawnActorfromClass "/Game/Tyler/Blueprints/Rooms/LightPuzzle/BP_LaserTarget.BP_LaserTarget_C" (Math|Transform|MakeTransform (Transformation|GetWorldLocation (Utilities|Array|Get(acopy) (Utilities|Array|MakeArray (Variables|Default|GetStartLoc) (Variables|Default|GetStartLoc1) (Variables|Default|GetStartLoc2) (Variables|Default|GetStartLoc3) (Variables|Default|GetStartLoc4) (Variables|Default|GetStartLoc5) (Variables|Default|GetStartLoc6) (Variables|Default|GetStartLoc7) (Variables|Default|GetStartLoc8) (Variables|Default|GetStartLoc9) (Variables|Default|GetStartLoc10) (Variables|Default|GetStartLoc11)) (Variables|Default|GetBlueEnd))) (Transformation|GetActorRotation) "1.000000,1.000000,1.000000") "Undefined" "MultiplyWithRoot" 0 "(R=0.000000,G=0.000000,B=0.000000,A=1.000000)" 0 (Variables|Default|GetBlue) 0))
      (bind _output_get_3 (Variables|Default|SetEndPoint2 _returnvalue_6))
      (Game|SpawnActorfromClass "/Game/Tyler/Blueprints/Rooms/LightPuzzle/BP_LaserChild.BP_LaserChild_C" (Math|Transform|MakeTransform (Transformation|GetWorldLocation (Variables|/Game/Tyler/Blueprints/Rooms/LightPuzzle/BP_LaserTarget.BP_LaserTarget_C|GetArrow _output_get_3)) (Transformation|GetActorRotation) "1.000000,1.000000,1.000000") "Undefined" "MultiplyWithRoot" 0 0 "" (Variables|Default|GetBlue) 0 "(R=0.000000,G=0.000000,B=0.000000,A=0.000000)" 0)
      (Variables|Default|SetBlueMatch? false)
      ;;[1 0.2836 0.01124] Reflecters Spawn
      (Utilities|FlowControl|Sequence
        (:then_0
          (bind _returnvalue_7 (Game|SpawnActorfromClass "/Game/Tyler/Blueprints/Rooms/LightPuzzle/BP_LaserReflecter.BP_LaserReflecter_C" (Math|Transform|MakeTransform (Transformation|GetWorldLocation (Variables|Default|GetReflector)) (Utilities|Array|Get(acopy) (Variables|Default|GetRotationArray) (Variables|Default|GetReflectRotation_C)) "1.000000,1.000000,1.000000") "Undefined" "MultiplyWithRoot" 0 "(R=0.000000,G=0.000000,B=0.000000,A=0.000000)" 0 "(R=0.000000,G=0.000000,B=0.000000,A=0.000000)" 0))
          (Variables|Default|SetReflect1 _returnvalue_7))
        (:then_1
          (bind _returnvalue_8 (Game|SpawnActorfromClass "/Game/Tyler/Blueprints/Rooms/LightPuzzle/BP_LaserReflecter.BP_LaserReflecter_C" (Math|Transform|MakeTransform (Transformation|GetWorldLocation (Variables|Default|GetReflector1)) (Utilities|Array|Get(acopy) (Variables|Default|GetRotationArray) (Variables|Default|GetReflectRotation_BR)) "1.000000,1.000000,1.000000") "Undefined" "MultiplyWithRoot" 0 "(R=0.000000,G=0.000000,B=0.000000,A=0.000000)" 0 "(R=0.000000,G=0.000000,B=0.000000,A=0.000000)" 0))
          (Variables|Default|SetReflect2 _returnvalue_8))
        (:then_2
          (bind _returnvalue_9 (Game|SpawnActorfromClass "/Game/Tyler/Blueprints/Rooms/LightPuzzle/BP_LaserReflecter.BP_LaserReflecter_C" (Math|Transform|MakeTransform (Transformation|GetWorldLocation (Variables|Default|GetReflector2)) (Utilities|Array|Get(acopy) (Variables|Default|GetRotationArray) (Variables|Default|GetReflectRotation_BL)) "1.000000,1.000000,1.000000") "Undefined" "MultiplyWithRoot" 0 "(R=0.000000,G=0.000000,B=0.000000,A=0.000000)" 0 "(R=0.000000,G=0.000000,B=0.000000,A=0.000000)" 0))
          (Variables|Default|SetReflect3 _returnvalue_9))
        (:then_3
          (bind _returnvalue_10 (Game|SpawnActorfromClass "/Game/Tyler/Blueprints/Rooms/LightPuzzle/BP_LaserReflecter.BP_LaserReflecter_C" (Math|Transform|MakeTransform (Transformation|GetWorldLocation (Variables|Default|GetReflector3)) (Utilities|Array|Get(acopy) (Variables|Default|GetRotationArray) (Variables|Default|GetReflectRotation_TL)) "1.000000,1.000000,1.000000") "Undefined" "MultiplyWithRoot" 0 "(R=0.000000,G=0.000000,B=0.000000,A=0.000000)" 0 "(R=0.000000,G=0.000000,B=0.000000,A=0.000000)" 0))
          (Variables|Default|SetReflect4 _returnvalue_10))
        (:then_4
          (bind _returnvalue_11 (Game|SpawnActorfromClass "/Game/Tyler/Blueprints/Rooms/LightPuzzle/BP_LaserReflecter.BP_LaserReflecter_C" (Math|Transform|MakeTransform (Transformation|GetWorldLocation (Variables|Default|GetReflector4)) (Utilities|Array|Get(acopy) (Variables|Default|GetRotationArray) (Variables|Default|GetReflectRotation_TR)) "1.000000,1.000000,1.000000") "Undefined" "MultiplyWithRoot" 0 "(R=0.000000,G=0.000000,B=0.000000,A=0.000000)" 0 "(R=0.000000,G=0.000000,B=0.000000,A=0.000000)" 0))
          (Variables|Default|SetReflect5 _returnvalue_11))))))

(event Custom|ServerData
  ;[1 1 1] Laser Puzzle
  ;;[0.401 0.401 0.401] Laser Ends
  (CallFunction|Multicast))

(event Custom|EndGameCheckerServer
  ;[1 1 1] Laser Puzzle
  ;;[1 0.8532 0.1876] Check Solved
  (CallFunction|EndGameCheckerClient))

(event Custom|NorthServerData
  ;[1 1 1] Laser Puzzle
  ;;[1 0.1534 0.9369] Laser Cube Spawners
  (CallFunction|NorthMulti))

(event Custom|EndGameCheckerClient
  ;[1 1 1] Laser Puzzle
  ;;[1 0.8532 0.1876] Check Solved
  (Utilities|Time|SetTimerbyEvent (delegate Custom|EndGameCheckerClient) 0.5 (== (Variables|Default|GetSolved?) false))
  (if (not (Variables|Default|GetSolved?))
    (Utilities|FlowControl|Sequence
      (:then_0
        (if (Variables|/Game/Tyler/Blueprints/Rooms/LightPuzzle/BP_LaserTarget.BP_LaserTarget_C|GetSolved? (Variables|Default|GetEndPoint))
          (Variables|Default|SetRedMatch? true)
          (if (Math|Boolean|ANDBoolean (Variables|Default|GetRedMatch?) (Variables|Default|GetBlueMatch?) (Variables|Default|GetGreenMatch?)) :!label _label
            (if (not (Variables|Default|GetSolved?))
              (Variables|Default|SetSolved? true)
              (CallFunction|EndGame)))))
      (:then_1
        (if (Variables|/Game/Tyler/Blueprints/Rooms/LightPuzzle/BP_LaserTarget.BP_LaserTarget_C|GetSolved? (Variables|Default|GetEndPoint1))
          (Variables|Default|SetGreenMatch? true)
          (goto _label)))
      (:then_2
        (if (Variables|/Game/Tyler/Blueprints/Rooms/LightPuzzle/BP_LaserTarget.BP_LaserTarget_C|GetSolved? (Variables|Default|GetEndPoint2))
          (Variables|Default|SetBlueMatch? true)
          (goto _label))))))

(event Custom|NorthMulti
  ;[1 1 1] Laser Puzzle
  ;;[1 0.1534 0.9369] Laser Cube Spawners
  (if (not (Variables|Default|GetButtonPressed?))
    (Variables|Default|SetButtonPressed? true)
    (Game|SpawnActorfromClass "/Game/Tyler/Blueprints/Rooms/LightPuzzle/BP_LaserCubeOne.BP_LaserCubeOne_C" (Math|Transform|MakeTransform (+ (Transformation|GetWorldLocation (Variables|Default|GetNorth%20Button)) "0.000000,0.000000,50.000000") "0.000000,270.000000,0.000000" "1.000000,1.000000,1.000000") "Undefined" "MultiplyWithRoot" 0 "(R=0.000000,G=0.000000,B=0.000000,A=0.000000)" 0 "(R=0.000000,G=0.000000,B=0.000000,A=0.000000)" 0)))

(event Custom|SouthServerData
  ;[1 1 1] Laser Puzzle
  ;;[1 0.1534 0.9369] Laser Cube Spawners
  (CallFunction|SouthMulti))

(event EventBeginPlay
  ;[1 1 1] Laser Puzzle
  ;;[1 1 1] List All Possible Locations and Rotations
  (Variables|Default|SetRedStarts (Utilities|Array|MakeArray 0 1 2 3 4 5 6 7 8 9 10 11))
  (Variables|Default|SetGreenStarts (Utilities|Array|MakeArray 0 1 2 3 4 5 6 7 8 9 10 11))
  (Variables|Default|SetBlueStarts (Utilities|Array|MakeArray 0 1 2 3 4 5 6 7 8 9 10 11))
  (Variables|Default|SetRedEnds (Utilities|Array|MakeArray 0 1 2 3 4 5 6 7 8 9 10 11))
  (Variables|Default|SetGreenEnds (Utilities|Array|MakeArray 0 1 2 3 4 5 6 7 8 9 10 11))
  (Variables|Default|SetBlueEnds (Utilities|Array|MakeArray 0 1 2 3 4 5 6 7 8 9 10 11))
  (Variables|Default|SetReflectRotation_TL (Math|Random|RandomIntegerinRange 0 3))
  (Variables|Default|SetReflectRotation_TR (Math|Random|RandomIntegerinRange 0 3))
  (Variables|Default|SetReflectRotation_C (Math|Random|RandomIntegerinRange 0 3))
  (Variables|Default|SetReflectRotation_BL (Math|Random|RandomIntegerinRange 0 3))
  (Variables|Default|SetReflectRotation_BR (Math|Random|RandomIntegerinRange 0 3))
  (Variables|Default|SetRotationArray (Utilities|Array|MakeArray (Variables|Default|Get45) (Variables|Default|Get135) (Variables|Default|Get225) (Variables|Default|Get315))))

(event EventBeginfromHUB
  ;[1 1 1] Laser Puzzle
  (Variables|Default|SetSolved? false)
  (if (Networking|IsServer)
    (CallFunction|GameSetup)
    (CallFunction|EndGameCheckerServer)))

(fn ConstructionScript
  (|CallParentFunction))

(fn OnRepBlueEnds)
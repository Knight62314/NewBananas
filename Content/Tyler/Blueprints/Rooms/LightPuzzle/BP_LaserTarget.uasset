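; BP_LaserTarget is a light puzzle target that is solved by a laser of the matching color.
; LaserRefract stores the hit state in Active and passes the laser's color to PuzzleSolved.
; On a color match, PuzzleSolved applies a dynamic M_Solid material, colored by the laser when active or gray otherwise, and sets Solved, which is never cleared here.
; The sphere overlap color check is disconnected debug logic.
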(event OnComponentBeginOverlap(Sphere)
  (params (OverlappedComponent :type Primitive%20Component%20Object%20Reference) (OtherActor :type Actor%20Object%20Reference) (OtherComp :type Primitive%20Component%20Object%20Reference) (OtherBodyIndex :type Integer) (bFromSweep :type Boolean) (SweepResult :type Hit%20Result%20Structure%20%28by%20ref%29)))

(event EventBeginPlay)

(event Collision|EventActorBeginOverlap
  (params (OtherActor :type Actor%20Object%20Reference)))

(event EventTick
  (params (DeltaSeconds :type Float%20%28single-precision%29)))

(fn ConstructionScript
  (|CallParentFunction))

(fn PuzzleSolved
  (params (Line%20Color :type Linear%20Color%20Structure))
  (if (== (Variables|Default|GetTargetColor) Line%20Color)
    (bind _returnvalue (Rendering|Material|CreateDynamicMaterialInstance (Variables|Default|GetStaticMesh) 0 "/Game/LevelPrototyping/Materials/M_Solid.M_Solid" "None" :!class /Script/Engine.PrimitiveComponent))
    (Rendering|Material|SetVectorParameterValue _returnvalue "Base Color" (Math|Color|SelectColor Line%20Color "(R=0.312500,G=0.312500,B=0.312500,A=1.000000)" (Variables|Default|GetActive?)) :!class /Script/Engine.MaterialInstanceDynamic)
    (Variables|Default|SetSolved? true)))

(fn LaserRefract
  (params (Hit :type Boolean) (HitResult :type Hit%20Result%20Structure) (Laser%20Hit :type BP%20Laser%20Child%20Object%20Reference))
  (Variables|Default|SetActive? Hit)
  (CallFunction|PuzzleSolved (Variables|/Game/Tyler/Blueprints/Rooms/LightPuzzle/BP_LaserParent.BP_LaserParent_C|GetLaserColor Laser%20Hit))
  (return 0))
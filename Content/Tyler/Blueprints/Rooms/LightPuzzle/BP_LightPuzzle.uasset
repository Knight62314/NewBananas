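; Light puzzle room in which players cycle three point lights through white, red, green and blue to match a random combination.
; The server rolls the combination when the hub starts the puzzle.
; Trigger boxes select a light, and overlap or interact advances it, with an index decrement on non-server instances.
; Only light three changes run the solution check; success calls the hub's move function after a delay, as does another trigger box.
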(event OnComponentBeginOverlap(Box1)
  (params (OverlappedComponent :type Primitive%20Component%20Object%20Reference) (OtherActor :type Actor%20Object%20Reference) (OtherComp :type Primitive%20Component%20Object%20Reference) (OtherBodyIndex :type Integer) (bFromSweep :type Boolean) (SweepResult :type Hit%20Result%20Structure%20%28by%20ref%29))
  ;[1 1 1] Light Puzzle
  ;;[0.07239 0.1488 1] Light 1 Gate
  (if (== (Utilities|GetClass OtherActor) "/Game/ThirdPerson/Blueprints/BP_ThirdPersonCharacter.BP_ThirdPersonCharacter_C")
    (Variables|Default|SetInteract1? true)
    (CallFunction|ServerInteract)))

(event OnComponentEndOverlap(Box1)
  (params (OverlappedComponent :type Primitive%20Component%20Object%20Reference) (OtherActor :type Actor%20Object%20Reference) (OtherComp :type Primitive%20Component%20Object%20Reference) (OtherBodyIndex :type Integer))
  ;[1 1 1] Light Puzzle
  ;;[0.07239 0.1488 1] Light 1 Gate
  (if (== (Utilities|GetClass OtherActor) "/Game/ThirdPerson/Blueprints/BP_ThirdPersonCharacter.BP_ThirdPersonCharacter_C")
    (Variables|Default|SetInteract1? false)))

(event OnComponentBeginOverlap(Box2)
  (params (OverlappedComponent :type Primitive%20Component%20Object%20Reference) (OtherActor :type Actor%20Object%20Reference) (OtherComp :type Primitive%20Component%20Object%20Reference) (OtherBodyIndex :type Integer) (bFromSweep :type Boolean) (SweepResult :type Hit%20Result%20Structure%20%28by%20ref%29))
  ;[1 1 1] Light Puzzle
  ;;[0.1608 1 0.1287] Light 2 Gate
  (if (== (Utilities|GetClass OtherActor) "/Game/ThirdPerson/Blueprints/BP_ThirdPersonCharacter.BP_ThirdPersonCharacter_C")
    (Variables|Default|SetInteract2? true)
    (CallFunction|ServerInteract)))

(event OnComponentEndOverlap(Box2)
  (params (OverlappedComponent :type Primitive%20Component%20Object%20Reference) (OtherActor :type Actor%20Object%20Reference) (OtherComp :type Primitive%20Component%20Object%20Reference) (OtherBodyIndex :type Integer))
  ;[1 1 1] Light Puzzle
  ;;[0.1608 1 0.1287] Light 2 Gate
  (if (== (Utilities|GetClass OtherActor) "/Game/ThirdPerson/Blueprints/BP_ThirdPersonCharacter.BP_ThirdPersonCharacter_C")
    (Variables|Default|SetInteract2? false)))

(event OnComponentBeginOverlap(Box3)
  (params (OverlappedComponent :type Primitive%20Component%20Object%20Reference) (OtherActor :type Actor%20Object%20Reference) (OtherComp :type Primitive%20Component%20Object%20Reference) (OtherBodyIndex :type Integer) (bFromSweep :type Boolean) (SweepResult :type Hit%20Result%20Structure%20%28by%20ref%29))
  ;[1 1 1] Light Puzzle
  ;;[1 0 0] Light 3 Gate
  (if (== (Utilities|GetClass OtherActor) "/Game/ThirdPerson/Blueprints/BP_ThirdPersonCharacter.BP_ThirdPersonCharacter_C")
    (Variables|Default|SetInteract3? true)
    (CallFunction|ServerInteract)))

(event OnComponentEndOverlap(Box3)
  (params (OverlappedComponent :type Primitive%20Component%20Object%20Reference) (OtherActor :type Actor%20Object%20Reference) (OtherComp :type Primitive%20Component%20Object%20Reference) (OtherBodyIndex :type Integer))
  ;[1 1 1] Light Puzzle
  ;;[1 0 0] Light 3 Gate
  (if (== (Utilities|GetClass OtherActor) "/Game/ThirdPerson/Blueprints/BP_ThirdPersonCharacter.BP_ThirdPersonCharacter_C")
    (Variables|Default|SetInteract3? false)))

(event OnComponentBeginOverlap(Box)
  (params (OverlappedComponent :type Primitive%20Component%20Object%20Reference) (OtherActor :type Actor%20Object%20Reference) (OtherComp :type Primitive%20Component%20Object%20Reference) (OtherBodyIndex :type Integer) (bFromSweep :type Boolean) (SweepResult :type Hit%20Result%20Structure%20%28by%20ref%29))
  ;[1 1 1] Hub Controls
  (if (== (Utilities|GetClass OtherActor) "/Game/ThirdPerson/Blueprints/BP_ThirdPersonCharacter.BP_ThirdPersonCharacter_C")
    (Default|MovetoHUBFunction (Variables|Default|GetHUB) self)))

(event Custom|Game%20Setup
  ;[1 1 1] Light Puzzle
  ;;[0 0 0] Puzzle Interact & Color Control
)

(event Custom|End%20Puzzle
  ;[1 1 1] Light Puzzle
  ;;[0.09369 1 0.9901] Puzzle Solved?
  ;;;[0.1354 1 0.2244] End Puzzle
  (if (Variables|Default|GetAllCorrect?)
    (Utilities|FlowControl|Delay 2.0)
    (Default|MovetoHUBFunction (Variables|Default|GetHUB) self)))

(event Custom|Multicast
  ;[1 1 1] Light Puzzle
  ;;[0.09369 1 0.9901] Puzzle Solved?
  (if (Variables|Default|GetStart)
    (Utilities|FlowControl|Sequence
      (:then_0
        ;;;[1 0.6202 0.04575] Color Match
        (if (== (Variables|Default|GetCIndex1) (Variables|Default|GetCColor1))
          (Variables|Default|Set1Correct? true)
          ;;;[0.1451 0.3307 1] Check Outcomes
          (if (and (and (Variables|Default|Get1Correct?) (Variables|Default|Get2Correct?)) (Variables|Default|Get3Correct?)) :!label _label
            (Development|PrintString "Complete")
            (Variables|Default|SetStart false)
            (Variables|Default|SetAllCorrect? true)
            (CallFunction|EndPuzzle))
          (else
            (Variables|Default|Set1Correct? false))))
      (:then_1
        (if (== (Variables|Default|GetCIndex2) (Variables|Default|GetCColor2))
          (Variables|Default|Set2Correct? true)
          (goto _label)
          (else
            (Variables|Default|Set2Correct? false))))
      (:then_2
        (if (== (Variables|Default|GetCIndex3) (Variables|Default|GetCColor3))
          (Variables|Default|Set3Correct? true)
          (goto _label)
          (else
            (Variables|Default|Set3Correct? false)))))))

(event Custom|ServerInteract
  ;[1 1 1] Light Puzzle
  ;;[0 0 0] Puzzle Interact & Color Control
  (CallFunction|PlayerInteract))

(event Custom|PlayerInteract
  ;[1 1 1] Light Puzzle
  ;;[0 0 0] Puzzle Interact & Color Control
  (Utilities|FlowControl|Sequence
    (:then_0
      (if (Networking|IsServer)
        _
        (else
          (Variables|Default|SetCIndex1 (- (Variables|Default|GetCIndex1) 1))))
      (if (Math|Boolean|ANDBoolean (Variables|Default|GetInteract1?) (!= (Variables|Default|GetInteract2?) true) (!= (Variables|Default|GetInteract3?) true))
        (bind _result (Math|Integer|IncrementInt (Variables|Default|GetCIndex1))
          (:%20%20
            (if (<= _result 4)
              _
              (else
                (Variables|Default|SetCIndex1 1)))
            (CallFunction|UpdateLightOne)))))
    (:then_1
      (if (Networking|IsServer)
        _
        (else
          (Variables|Default|SetCIndex2 (- (Variables|Default|GetCIndex2) 1))))
      (if (Math|Boolean|ANDBoolean (Variables|Default|GetInteract2?) (!= (Variables|Default|GetInteract1?) true) (!= (Variables|Default|GetInteract3?) true))
        (bind _result_2 (Math|Integer|IncrementInt (Variables|Default|GetCIndex2))
          (:%20%20
            (if (<= _result_2 4)
              _
              (else
                (Variables|Default|SetCIndex2 1)))
            (CallFunction|UpdateLightTwo)))))
    (:then_2
      (if (Networking|IsServer)
        _
        (else
          (Variables|Default|SetCIndex3 (- (Variables|Default|GetCIndex3) 1))))
      (if (Math|Boolean|ANDBoolean (Variables|Default|GetInteract3?) (!= (Variables|Default|GetInteract1?) true) (!= (Variables|Default|GetInteract2?) true))
        (bind _result_3 (Math|Integer|IncrementInt (Variables|Default|GetCIndex3))
          (:%20%20
            (if (<= _result_3 4)
              _
              (else
                (Variables|Default|SetCIndex3 1)))
            (CallFunction|UpdateLightThree)
            (CallFunction|Multicast)))))))

(event Custom|Setup
  ;[1 1 1] Light Puzzle
  ;;[1 0.133 0.9246] Puzzle Setup
  (Variables|Default|SetCColor1 (Math|Random|RandomIntegerinRange 1 4))
  (Variables|Default|SetCColor2 (Math|Random|RandomIntegerinRange 1 4))
  (Variables|Default|SetCColor3 (Math|Random|RandomIntegerinRange 1 4))
  (Development|PrintString (Utilities|String|ToString(Integer) (Variables|Default|GetCColor1)) true true "(R=0.000000,G=0.660000,B=1.000000,A=1.000000)" 1e+01)
  (Development|PrintString (Utilities|String|ToString(Integer) (Variables|Default|GetCColor2)) true true "(R=0.000000,G=0.660000,B=1.000000,A=1.000000)" 1e+01)
  (Development|PrintString (Utilities|String|ToString(Integer) (Variables|Default|GetCColor3)) true true "(R=0.000000,G=0.660000,B=1.000000,A=1.000000)" 1e+01))

(event EventOnInteract
  (params (Actor :type Actor%20Object%20Reference))
  ;[1 1 1] Light Puzzle
  ;;[0 0 0] Puzzle Interact & Color Control
  (CallFunction|ServerInteract))

(event EventBeginfromHUB
  ;[1 1 1] Light Puzzle
  ;;[1 0.133 0.9246] Puzzle Setup
  (if (Networking|IsServer)
    (CallFunction|Setup)))

(event EventBeginPlay
  ;[1 1 1] Light Puzzle
  ;;[1 0.133 0.9246] Puzzle Setup
  (Variables|Default|SetStart true)
  (Variables|Default|SetCIndex1 1)
  (Variables|Default|SetCIndex2 1)
  (Variables|Default|SetCColor3 1))

(fn ConstructionScript
  (|CallParentFunction))

(fn UpdateLightOne
  (bind _pointlight1 (Variables|Default|GetPointLight1))
  (bind _pointlight1_2 (Variables|Default|GetPointLight1))
  (if (Networking|IsServer)
    (switch int (Variables|Default|GetCIndex1)
      (:1
        (Rendering|Components|Light|SetLightColor _pointlight1_2 "(R=1.000000,G=1.000000,B=1.000000,A=1.000000)" true))
      (:2
        (Rendering|Components|Light|SetLightColor _pointlight1_2 "(R=255.000000,G=0.000000,B=0.000000,A=1.000000)" true))
      (:3
        (Rendering|Components|Light|SetLightColor _pointlight1_2 "(R=0.000000,G=255.000000,B=0.000000,A=1.000000)" true))
      (:4
        (Rendering|Components|Light|SetLightColor _pointlight1_2 "(R=0.000000,G=0.000000,B=255.000000,A=1.000000)" true)))
    (else
      (switch int (Variables|Default|GetCIndex1)
        (:1
          (Rendering|Components|Light|SetLightColor _pointlight1 "(R=1.000000,G=1.000000,B=1.000000,A=1.000000)" true))
        (:2
          (Rendering|Components|Light|SetLightColor _pointlight1 "(R=255.000000,G=0.000000,B=0.000000,A=1.000000)" true))
        (:3
          (Rendering|Components|Light|SetLightColor _pointlight1 "(R=0.000000,G=255.000000,B=0.000000,A=1.000000)" true))
        (:4
          (Rendering|Components|Light|SetLightColor _pointlight1 "(R=0.000000,G=0.000000,B=255.000000,A=1.000000)" true))))))

(fn UpdateLightTwo
  (bind _pointlight2 (Variables|Default|GetPointLight2))
  (switch int (Variables|Default|GetCIndex2)
    (:1
      (Rendering|Components|Light|SetLightColor _pointlight2 "(R=1.000000,G=1.000000,B=1.000000,A=1.000000)" true))
    (:2
      (Rendering|Components|Light|SetLightColor _pointlight2 "(R=255.000000,G=0.000000,B=0.000000,A=1.000000)" true))
    (:3
      (Rendering|Components|Light|SetLightColor _pointlight2 "(R=0.000000,G=255.000000,B=0.000000,A=1.000000)" true))
    (:4
      (Rendering|Components|Light|SetLightColor _pointlight2 "(R=0.000000,G=0.000000,B=255.000000,A=1.000000)" true))))

(fn UpdateLightThree
  (bind _pointlight3 (Variables|Default|GetPointLight3))
  (switch int (Variables|Default|GetCIndex3)
    (:1
      (Rendering|Components|Light|SetLightColor _pointlight3 "(R=1.000000,G=1.000000,B=1.000000,A=1.000000)" true))
    (:2
      (Rendering|Components|Light|SetLightColor _pointlight3 "(R=255.000000,G=0.000000,B=0.000000,A=1.000000)" true))
    (:3
      (Rendering|Components|Light|SetLightColor _pointlight3 "(R=0.000000,G=255.000000,B=0.000000,A=1.000000)" true))
    (:4
      (Rendering|Components|Light|SetLightColor _pointlight3 "(R=0.000000,G=0.000000,B=255.000000,A=1.000000)" true))))
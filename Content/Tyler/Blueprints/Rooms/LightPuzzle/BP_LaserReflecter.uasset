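; Laser-puzzle reflector that bounces laser beams and turns 90 degrees when damaged.
; Damage calls RotateServer then RotateClient, which briefly teleports the mesh down while rotating it, with a flag blocking re-entry.
; LaserRefract spawns a child laser along the mirrored hit direction, inheriting color and an updated ID.
; When a hit ends, matching child lasers are removed, either relaying the clear to interface-implementing actors they hit or being destroyed.
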(event Custom|Rotate%20Server
  (CallFunction|RotateClient))

(event Custom|RotateClient
  (bind _staticmesh (Variables|Default|GetStaticMesh))
  (if (not (Variables|Default|GetCollision?))
    (Variables|Default|SetCollision? true)
    (Transformation|SetRelativeLocation _staticmesh "0.000000,0.000000,-400.000000" false true)
    (bind _output_get (Variables|Default|SetReflector%20Current%20Rotation (Variables|/Script/Engine.SceneComponent|GetRelativeRotation _staticmesh)))
    (bind _output_get_2 (Variables|Default|SetReflector%20Updated%20Rotation (Math|Rotator|CombineRotators _output_get "0.000000,90.000000,0.000000")))
    (Transformation|SetRelativeRotation _staticmesh _output_get_2 false false)
    (Utilities|FlowControl|Delay 0.2)
    (Transformation|SetRelativeLocation _staticmesh "0.000000,0.000000,0.000000" false true)
    (Variables|Default|SetCollision? false)))

(event Game|Damage|EventAnyDamage
  (params (Damage :type Float%20%28single-precision%29) (DamageType :type Damage%20Type%20Object%20Reference) (InstigatedBy :type Controller%20Object%20Reference) (DamageCauser :type Actor%20Object%20Reference))
  (CallFunction|RotateServer))

(fn ConstructionScript
  (|CallParentFunction))

(fn CalculateRotate
  (params (Impact%20Point :type Vector) (Trace%20Start :type Vector) (Impact%20Normal :type Vector))
  (return (Math|Rotator|MakeRotfromZ (Math|Vector|MirrorVectorbyNormal (- Impact%20Point Trace%20Start) Impact%20Normal))))

(fn ClearAllAttachted
  (params (ID%20Clear :type String))
  (bind _arrayelement (Utilities|Array|ReverseforEachLoop (Variables|Default|GetLasersAttached))
    (:LoopBody
      (Utilities|IsValid _arrayelement
        (:Is%20Valid
          (if (Utilities|String|Contains (Variables|/Game/Tyler/Blueprints/Rooms/LightPuzzle/BP_LaserChild.BP_LaserChild_C|GetLaser_ID _arrayelement) ID%20Clear)
            (bind _last_hit_actor (Variables|/Game/Tyler/Blueprints/Rooms/LightPuzzle/BP_LaserChild.BP_LaserChild_C|GetLast%20Hit%20Actor _arrayelement)
              (:then
                (if (Utilities|DoesObjectImplementInterface _last_hit_actor "/Game/Tyler/Blueprints/BlueprintInterface/BPI_Lasers.BPI_Lasers_C")
                  (Class|BPILasers|LaserRefract(Message) :self _last_hit_actor :Laser%20Hit _arrayelement)
                  (else
                    (Actor|DestroyActor _arrayelement :!label _label))))
              (:else
                (goto _label)))
            (Utilities|Array|RemoveItem (Variables|Default|GetLasersAttached) _arrayelement)))))))

(fn LaserRefract
  (params (Hit :type Boolean) (HitResult :type Hit%20Result%20Structure) (Laser%20Hit :type BP%20Laser%20Child%20Object%20Reference))
  (bind (_bblockinghit _binitialoverlap _time _distance _location _impactpoint _normal _impactnormal _physmat _hitactor _hitcomponent _hitbonename _bonename _hititem _elementindex _faceindex _tracestart) (Collision|BreakHitResult HitResult))
  (if Hit
    (bind _returnvalue (Game|SpawnActorfromClass "/Game/Tyler/Blueprints/Rooms/LightPuzzle/BP_LaserChild.BP_LaserChild_C" (Math|Transform|MakeTransform _impactpoint (CallFunction|CalculateRotate _impactpoint _tracestart _impactnormal) "1.000000,1.000000,1.000000") "Undefined" "MultiplyWithRoot" 0 0 (Default|UpdateID Laser%20Hit "B") (Variables|/Game/Tyler/Blueprints/Rooms/LightPuzzle/BP_LaserParent.BP_LaserParent_C|GetLaserColor Laser%20Hit) (Variables|/Game/Tyler/Blueprints/Rooms/LightPuzzle/BP_LaserParent.BP_LaserParent_C|GetSpawnReference Laser%20Hit) "(R=0.000000,G=0.000000,B=0.000000,A=0.000000)" 0))
    (Utilities|Array|Add (Variables|Default|GetLasersAttached) _returnvalue)
    (Utilities|Array|Add (Variables|/Game/Tyler/Blueprints/Rooms/LightPuzzle/BP_LaserSpawn.BP_LaserSpawn_C|GetChild%20Lasers (Variables|/Game/Tyler/Blueprints/Rooms/LightPuzzle/BP_LaserParent.BP_LaserParent_C|GetSpawnReference Laser%20Hit)) _returnvalue)
    (return _returnvalue)
    (else
      (CallFunction|ClearAllAttachted (Variables|/Game/Tyler/Blueprints/Rooms/LightPuzzle/BP_LaserChild.BP_LaserChild_C|GetLaser_ID Laser%20Hit)))))
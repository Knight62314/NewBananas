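; BP_Pylon3 is a pylon in the light puzzle room that sets its point light's color when touched by the third-person character.
; A box overlap with that exact character class calls ServerColor, which relays to ClientColor, a split whose names suggest networked play.
; ClientColor switches on the Color variable to apply one of four fixed colors.
; Nothing in this Blueprint changes Color.
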(event OnComponentBeginOverlap(Box)
  (params (OverlappedComponent :type Primitive%20Component%20Object%20Reference) (OtherActor :type Actor%20Object%20Reference) (OtherComp :type Primitive%20Component%20Object%20Reference) (OtherBodyIndex :type Integer) (bFromSweep :type Boolean) (SweepResult :type Hit%20Result%20Structure%20%28by%20ref%29))
  (if (== (Utilities|GetClass OtherActor) "/Game/ThirdPerson/Blueprints/BP_ThirdPersonCharacter.BP_ThirdPersonCharacter_C")
    (CallFunction|ServerColor)))

(event Custom|Server%20Color
  (CallFunction|ClientColor))

(event Custom|Client%20Color
  (bind _pointlight (Variables|Default|GetPointLight))
  (switch int (Variables|Default|GetColor)
    (:1
      (Rendering|Components|Light|SetLightColor _pointlight "(R=1.000000,G=0.000000,B=1.000000,A=1.000000)" true))
    (:2
      (Rendering|Components|Light|SetLightColor _pointlight "(R=255.000000,G=0.000000,B=0.000000,A=1.000000)" true))
    (:3
      (Rendering|Components|Light|SetLightColor _pointlight "(R=0.000000,G=255.000000,B=0.000000,A=1.000000)" true))
    (:4
      (Rendering|Components|Light|SetLightColor _pointlight "(R=0.000000,G=0.000000,B=255.000000,A=1.000000)" true))))

(event EventBeginPlay)

(event Collision|EventActorBeginOverlap
  (params (OtherActor :type Actor%20Object%20Reference)))

(event EventTick
  (params (DeltaSeconds :type Float%20%28single-precision%29)))

(fn ConstructionScript)
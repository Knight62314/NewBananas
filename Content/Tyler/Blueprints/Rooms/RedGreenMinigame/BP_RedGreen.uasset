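; Red Light Green Light minigame room that swings a turret between red and green light states, linked to a HUB.
; From BeginPlay, a self-rescheduling random timer triggers timelines that yaw the turret and recolor its point light.
; The RedLight flag clears as green starts but sets only after the red turn finishes; no movement detection is wired.
; A player overlapping the box calls the HUB's move function.
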(event OnComponentBeginOverlap(Box)
  (params (OverlappedComponent :type Primitive%20Component%20Object%20Reference) (OtherActor :type Actor%20Object%20Reference) (OtherComp :type Primitive%20Component%20Object%20Reference) (OtherBodyIndex :type Integer) (bFromSweep :type Boolean) (SweepResult :type Hit%20Result%20Structure%20%28by%20ref%29))
  (if (== (Utilities|GetClass OtherActor) "/Game/ThirdPerson/Blueprints/BP_ThirdPersonCharacter.BP_ThirdPersonCharacter_C")
    (Default|MovetoHUBFunction (Variables|Default|GetHUB) self)))

(event Custom|Rotate
  ;[1 1 1] Red Light Green Light
  ;;[1 0.05729 0.05729] Rotate Turret Over Time
  (if (Variables|Default|GetRedLight)
    (Variables|Default|SetRedLight false)
    (bind _rotate (Timeline|GreenLightRotateSpeed PlayFromStart)
      (:Update
        (Transformation|SetRelativeRotation (Variables|Default|GetTurret) (Math|Rotator|MakeRotator 0.0 0.0 _rotate) false false)
        ;;;[0.007734 1 0.9303] Light Color
        (Rendering|Components|Light|SetLightColor (Variables|Default|GetPointLight) "(R=0.032855,G=0.666667,B=0.058960,A=1.000000)" true)))
    (else
      (bind _rotate_2 (Timeline|RedLightRotateSpeed PlayFromStart)
        (:Update
          (Transformation|SetRelativeRotation (Variables|Default|GetTurret) (Math|Rotator|MakeRotator 0.0 0.0 _rotate_2) false false)
          (Rendering|Components|Light|SetLightColor (Variables|Default|GetPointLight) "(R=0.666667,G=0.013261,B=0.000000,A=1.000000)" true))
        (:Finished
          (Variables|Default|SetRedLight true))))))

(event Custom|Game%20Count
  ;[1 1 1] Red Light Green Light
  ;;[0.3122 1 0.371] Turret Rotation (Random Time Between Rotations)
  (if (Variables|Default|GetStart)
    _
    (else
      _))
  (Utilities|Time|SetTimerbyEvent (delegate Custom|Game%20Count) (Math|Random|RandomFloatinRange 1.0 5.0))
  (CallFunction|Rotate)
  (Development|PrintString "Hello"))

(event EventBeginPlay
  ;[1 1 1] Red Light Green Light
  ;;[0.2266 0.4129 1] Game Setup
  (CallFunction|GameCount))

(event EventBeginfromHUB
  (Development|PrintString "RoomTest1"))

(fn ConstructionScript
  (|CallParentFunction))
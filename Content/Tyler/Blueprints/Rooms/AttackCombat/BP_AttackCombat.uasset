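; BP_AttackCombat is a combat room where players must destroy an attack objective, losing if the room timer finishes first.
; BeginfromHUB shows the attack UI, spawns a grid of nine melee enemies and the objective, and each kill spawns a replacement at a random position.
; A one-second re-armed timer polls the objective to trigger the win.
; EndfromHUB stops polling, removes widgets, then after a delay clears enemies and revives characters.
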(event Custom|Objective%20Destoryed
  (if (Variables|Default|GetLoop)
    (Utilities|Time|SetTimerbyEvent (delegate Custom|Objective%20Destoryed) 1.0)
    (if (Variables|/Game/Tyler/Blueprints/Rooms/AttackCombat/BP_AttackObjective.BP_AttackObjective_C|GetIsDestoryed? (Variables|Default|GetObjective))
      (Actor|DestroyActor (Variables|Default|GetObjective))
      (CallFunction|RoomWon))))

(event EventBeginfromHUB
  (CallFunction|KillAllMeleeEnemies)
  (bind _returnvalue (UserInterface|CreateWidget "/Game/Tyler/Blueprints/Rooms/AttackCombat/W_AttackUI.W_AttackUI_C"))
  (bind _output_get (Variables|Default|SetAttackUI _returnvalue))
  (UserInterface|Viewport|AddtoViewport _output_get 0)
  (CallFunction|SpawnMeleeEnemy "-1000.000000,-1000.000000,0.000000")
  (CallFunction|SpawnMeleeEnemy "-1000.000000,0.000000,0.000000")
  (CallFunction|SpawnMeleeEnemy "-1000.000000,1000.000000,0.000000")
  (CallFunction|SpawnMeleeEnemy "0.000000,-1000.000000,0.000000")
  (CallFunction|SpawnMeleeEnemy "0.000000,1000.000000,0.000000")
  (CallFunction|SpawnMeleeEnemy "1000.000000,-1000.000000,0.000000")
  (CallFunction|SpawnMeleeEnemy "1000.000000,0.000000,0.000000")
  (CallFunction|SpawnMeleeEnemy "1000.000000,1000.000000,0.000000")
  (CallFunction|SpawnMeleeEnemy "0, 0, 0")
  (bind _returnvalue_2 (Game|SpawnActorfromClass "/Game/Tyler/Blueprints/Rooms/AttackCombat/BP_AttackObjective.BP_AttackObjective_C" (Math|Transform|MakeTransform (Transformation|GetWorldLocation (Variables|Default|GetArrow)) "0, 0, 0" "1.000000,1.000000,1.000000") "Undefined" "MultiplyWithRoot" 0 0))
  (bind _output_get_2 (Variables|Default|SetObjective _returnvalue_2))
  (if (not (Variables|/Game/Tyler/Blueprints/Rooms/AttackCombat/BP_AttackObjective.BP_AttackObjective_C|GetIsDestoryed? _output_get_2))
    (CallFunction|ObjectiveDestoryed)))

(event EventEnemyKilled
  (bind _returnvalue (Math|Random|RandomFloatinRange -1e+03 1e+03))
  (CallFunction|SpawnMeleeEnemy (Math|Vector|MakeVector _returnvalue _returnvalue 0.0)))

(event EventRoomTimerFinished
  (CallFunction|RoomLost))

(event EventEndfromHUB
  (Variables|Default|SetLoop false)
  (Viewport|RemoveAllWidgets)
  (Utilities|FlowControl|Delay 3.0)
  (CallFunction|KillAllMeleeEnemies)
  (bind _outactors (Actor|GetAllActorsOfClass "/Game/ThirdPerson/Blueprints/BP_ThirdPersonCharacter.BP_ThirdPersonCharacter_C"))
  (for _array_element _outactors
    (Default|ReviveServer _array_element)))

(fn ConstructionScript
  (|CallParentFunction))
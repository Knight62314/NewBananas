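; BP_AttackObjective is a damageable, bobbing objective for the attack combat room.
; Any damage passes through DamageReceiveServer to ReceiveDamage, which ignores invalid causers, then either lowers health or flags the objective destroyed when health would run out.
; Non-lethal hits push the normalized health to every top-level W_AttackUI widget.
; Tick moves the mesh on a sine wave around its starting relative location.
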(event Custom|DamageReceiveServer
  (params (Health :type Float%20%28double-precision%29) (DamageType :type Damage%20Type%20Class%20Reference) (DamageCauser :type Actor%20Object%20Reference))
  (CallFunction|ReceiveDamage Health DamageType DamageCauser))

(event Custom|ReceiveDamage
  (params (Health :type Float%20%28double-precision%29) (DamageType :type Damage%20Type%20Class%20Reference) (Damage%20Causer :type Actor%20Object%20Reference))
  (Utilities|IsValid Damage%20Causer
    (:Is%20Valid
      (Variables|Default|SetDamage%20Causer Damage%20Causer)
      (Variables|Default|SetDamage%20Type DamageType)
      (if (<= (- (Variables|Default|GetHealth) Health) 0.0)
        (Variables|Default|SetIsDestoryed? true)
        (else
          (bind _output_get (Variables|Default|SetHealth (- (Variables|Default|GetHealth) Health)))
          (CallFunction|UpdateHealthBar _output_get))))))

(event EventBeginPlay
  (Utilities|Time|SetTimerbyEvent 0 1.0)
  (Variables|Default|SetObjectiveRelativeLocation (Variables|/Script/Engine.SceneComponent|GetRelativeLocation (Variables|Default|GetStaticMesh))))

(event EventTick
  (params (DeltaSeconds :type Float%20%28single-precision%29))
  (bind _objectiverelativelocation (Variables|Default|GetObjectiveRelativeLocation))
  (Transformation|SetRelativeLocation (Variables|Default|GetStaticMesh) (Math|Vector|MakeVector (.x _objectiverelativelocation) (.y _objectiverelativelocation) (+ (.z _objectiverelativelocation) (* (Math|Trig|Sin(Degrees) (* (Actor|GetGameTimeSinceCreation) (Variables|Default|GetBobbing%20Speed))) (Variables|Default|GetBobbing%20Distance)))) false false))

(event Game|Damage|EventAnyDamage
  (params (Damage :type Float%20%28single-precision%29) (DamageType :type Damage%20Type%20Object%20Reference) (InstigatedBy :type Controller%20Object%20Reference) (DamageCauser :type Actor%20Object%20Reference))
  (CallFunction|DamageReceiveServer Damage (Utilities|GetClass DamageType) DamageCauser))

(fn ConstructionScript)

(fn UpdateHealthBar
  (params (Health :type Float%20%28double-precision%29))
  (bind _foundwidgets (Widget|GetAllWidgetsOfClass "/Game/Tyler/Blueprints/Rooms/AttackCombat/W_AttackUI.W_AttackUI_C" true))
  (for _array_element _foundwidgets
    (bind _output_get (Variables|/Game/Tyler/Blueprints/Rooms/AttackCombat/W_AttackUI.W_AttackUI_C|SetHealth _array_element (/ Health 1e+02)))
    (Default|UpdateWidget _array_element _output_get)))
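; Networked pinball minigame room, started from the HUB, that returns there when five points are scored or a player overlaps an exit box.
; Player-triggered boxes slide the launcher along timelines, fire a BP_Pinball by impulse and shift pegs vertically.
; Setup lowers one of two peg groups, picked randomly on BeginPlay.
; Actions pass through Server/Client event pairs, with ball hits on scoring boxes counted on the server.
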(event OnComponentBeginOverlap(Box_0)
  (params (OverlappedComponent :type Primitive%20Component%20Object%20Reference) (OtherActor :type Actor%20Object%20Reference) (OtherComp :type Primitive%20Component%20Object%20Reference) (OtherBodyIndex :type Integer) (bFromSweep :type Boolean) (SweepResult :type Hit%20Result%20Structure%20%28by%20ref%29))
  (if (and (== (Utilities|GetClass OtherActor) "/Game/ThirdPerson/Blueprints/BP_ThirdPersonCharacter.BP_ThirdPersonCharacter_C") (not (Variables|Default|GetSolved)))
    (Variables|Default|SetSolved true)
    (Default|MovetoHUBFunction (Variables|Default|GetHUB) self)))

(event OnComponentBeginOverlap(Box1)
  (params (OverlappedComponent :type Primitive%20Component%20Object%20Reference) (OtherActor :type Actor%20Object%20Reference) (OtherComp :type Primitive%20Component%20Object%20Reference) (OtherBodyIndex :type Integer) (bFromSweep :type Boolean) (SweepResult :type Hit%20Result%20Structure%20%28by%20ref%29))
  ;[0.9574 1 0.5664] Move Launcher
  (CallFunction|RightButtonServer))

(event OnComponentBeginOverlap(Box2)
  (params (OverlappedComponent :type Primitive%20Component%20Object%20Reference) (OtherActor :type Actor%20Object%20Reference) (OtherComp :type Primitive%20Component%20Object%20Reference) (OtherBodyIndex :type Integer) (bFromSweep :type Boolean) (SweepResult :type Hit%20Result%20Structure%20%28by%20ref%29))
  ;[0.9574 1 0.5664] Move Launcher
  (CallFunction|LeftButtonServer))

(event OnComponentBeginOverlap(Box5)
  (params (OverlappedComponent :type Primitive%20Component%20Object%20Reference) (OtherActor :type Actor%20Object%20Reference) (OtherComp :type Primitive%20Component%20Object%20Reference) (OtherBodyIndex :type Integer) (bFromSweep :type Boolean) (SweepResult :type Hit%20Result%20Structure%20%28by%20ref%29))
  ;[0.8234 0.5271 1] Launch Pinball
  (if (== (Utilities|GetClass OtherActor) "/Game/ThirdPerson/Blueprints/BP_ThirdPersonCharacter.BP_ThirdPersonCharacter_C")
    (CallFunction|ServerFire)))

(event OnComponentBeginOverlap(Box6)
  (params (OverlappedComponent :type Primitive%20Component%20Object%20Reference) (OtherActor :type Actor%20Object%20Reference) (OtherComp :type Primitive%20Component%20Object%20Reference) (OtherBodyIndex :type Integer) (bFromSweep :type Boolean) (SweepResult :type Hit%20Result%20Structure%20%28by%20ref%29))
  (if (== (Utilities|GetClass OtherActor) "/Game/ThirdPerson/Blueprints/BP_ThirdPersonCharacter.BP_ThirdPersonCharacter_C")
    (CallFunction|ServerReorder)))

(event OnComponentBeginOverlap(Box7)
  (params (OverlappedComponent :type Primitive%20Component%20Object%20Reference) (OtherActor :type Actor%20Object%20Reference) (OtherComp :type Primitive%20Component%20Object%20Reference) (OtherBodyIndex :type Integer) (bFromSweep :type Boolean) (SweepResult :type Hit%20Result%20Structure%20%28by%20ref%29))
  ;[0.4374 1 0.9901] Calculate Score
  (if (== (Utilities|GetClass OtherActor) "/Game/Tyler/Blueprints/Rooms/PinballMinigame/BP_Pinball.BP_Pinball_C")
    (CallFunction|ServerScore)))

(event OnComponentBeginOverlap(Box8)
  (params (OverlappedComponent :type Primitive%20Component%20Object%20Reference) (OtherActor :type Actor%20Object%20Reference) (OtherComp :type Primitive%20Component%20Object%20Reference) (OtherBodyIndex :type Integer) (bFromSweep :type Boolean) (SweepResult :type Hit%20Result%20Structure%20%28by%20ref%29))
  ;[0.4374 1 0.9901] Calculate Score
  (if (== (Utilities|GetClass OtherActor) "/Game/Tyler/Blueprints/Rooms/PinballMinigame/BP_Pinball.BP_Pinball_C")
    (CallFunction|ServerScore)))

(event OnComponentBeginOverlap(Box9)
  (params (OverlappedComponent :type Primitive%20Component%20Object%20Reference) (OtherActor :type Actor%20Object%20Reference) (OtherComp :type Primitive%20Component%20Object%20Reference) (OtherBodyIndex :type Integer) (bFromSweep :type Boolean) (SweepResult :type Hit%20Result%20Structure%20%28by%20ref%29))
  ;[0.4374 1 0.9901] Calculate Score
  (if (== (Utilities|GetClass OtherActor) "/Game/Tyler/Blueprints/Rooms/PinballMinigame/BP_Pinball.BP_Pinball_C")
    (CallFunction|ServerScore)))

(event OnComponentBeginOverlap(Box10)
  (params (OverlappedComponent :type Primitive%20Component%20Object%20Reference) (OtherActor :type Actor%20Object%20Reference) (OtherComp :type Primitive%20Component%20Object%20Reference) (OtherBodyIndex :type Integer) (bFromSweep :type Boolean) (SweepResult :type Hit%20Result%20Structure%20%28by%20ref%29))
  ;[0.4374 1 0.9901] Calculate Score
  (if (== (Utilities|GetClass OtherActor) "/Game/Tyler/Blueprints/Rooms/PinballMinigame/BP_Pinball.BP_Pinball_C")
    (CallFunction|ServerScore)))

(event OnComponentEndOverlap(Box5)
  (params (OverlappedComponent :type Primitive%20Component%20Object%20Reference) (OtherActor :type Actor%20Object%20Reference) (OtherComp :type Primitive%20Component%20Object%20Reference) (OtherBodyIndex :type Integer))
  ;[0.8234 0.5271 1] Launch Pinball
  (Utilities|FlowControl|Delay 2.0)
  (Variables|Default|SetBallLaunched? false))

(event Custom|Right%20Button%20Server
  ;[0.9574 1 0.5664] Move Launcher
  (CallFunction|RightButtonClient))

(event Custom|Right%20Button%20Client
  ;[0.9574 1 0.5664] Move Launcher
  (Variables|Default|SetLauncherStartLocation (Variables|/Script/Engine.SceneComponent|GetRelativeLocation (Variables|Default|GetLauncher)))
  (bind _output_get (Variables|Default|SetLauncherEndLocation (Math|Vector|MakeVector (+ (.x (Variables|Default|GetLauncherStartLocation)) 2e+02) (.y (Variables|Default|GetLauncherStartLocation)) (.z (Variables|Default|GetLauncherStartLocation)))))
  (if (<= (.x _output_get) 1.1e+03)
    (bind _newtrack_0 (Timeline|Right%20Launcher%20Movement PlayFromStart)
      (:Update
        (Transformation|SetRelativeLocation (Variables|Default|GetLauncher) (Math|Vector|Lerp(Vector) (Variables|Default|GetLauncherStartLocation) (Variables|Default|GetLauncherEndLocation) _newtrack_0) false false)))))

(event Custom|Server%20Score
  ;[0.4374 1 0.9901] Calculate Score
  (CallFunction|ClientScore))

(event Custom|Client%20Score
  ;[0.4374 1 0.9901] Calculate Score
  (if (Networking|IsServer)
    (bind _output_get (Variables|Default|SetScore (+ (Variables|Default|GetScore) 1)))
    (else
      (Variables|Default|SetScore _output_get)))
  (Development|PrintString (Utilities|String|ToString(Integer) _output_get))
  (if (== (Variables|Default|GetScore) 5)
    (CallFunction|EndGame)))

(event Custom|End%20game
  ;[0.4374 1 0.9901] Calculate Score
  ;;[0 0 0] End Game
  (if (not (Variables|Default|GetSolved))
    (Variables|Default|SetSolved true)
    (Default|MovetoHUBFunction (Variables|Default|GetHUB) self)))

(event Custom|Left%20Button%20Server
  ;[0.9574 1 0.5664] Move Launcher
  (CallFunction|LeftButtonClient))

(event Custom|Left%20Button%20Client
  ;[0.9574 1 0.5664] Move Launcher
  (Variables|Default|SetLauncherStartLocation (Variables|/Script/Engine.SceneComponent|GetRelativeLocation (Variables|Default|GetLauncher)))
  (bind _output_get (Variables|Default|SetLauncherEndLocation (Math|Vector|MakeVector (- (.x (Variables|Default|GetLauncherStartLocation)) 2e+02) (.y (Variables|Default|GetLauncherStartLocation)) (.z (Variables|Default|GetLauncherStartLocation)))))
  (if (>= (.x _output_get) -9e+02)
    (bind _newtrack_0 (Timeline|Left%20Launcher%20Movement PlayFromStart)
      (:Update
        (Transformation|SetRelativeLocation (Variables|Default|GetLauncher) (Math|Vector|Lerp(Vector) (Variables|Default|GetLauncherEndLocation) (Variables|Default|GetLauncherStartLocation) _newtrack_0) false false)))))

(event Custom|ServerFire
  ;[0.8234 0.5271 1] Launch Pinball
  (CallFunction|ClientFire))

(event Custom|ClientFire
  ;[0.8234 0.5271 1] Launch Pinball
  (if (not (Variables|Default|GetBallLaunched?))
    (Variables|Default|SetBallLaunched? true)
    (bind _returnvalue (Game|SpawnActorfromClass "/Game/Tyler/Blueprints/Rooms/PinballMinigame/BP_Pinball.BP_Pinball_C" (Transformation|GetWorldTransform (Variables|Default|GetBallSpawn)) "AlwaysSpawn" "MultiplyWithRoot" 0 0))
    (bind _output_get (Variables|Default|SetPinball _returnvalue))
    (Physics|AddImpulse (Variables|/Game/Tyler/Blueprints/Rooms/PinballMinigame/BP_Pinball.BP_Pinball_C|GetStaticMesh _output_get) (Math|Vector|MakeVector 0.0 (Variables|Default|GetBallSpeed) 0.0) "None" true)))

(event Custom|Game%20Setup%20Server
  ;[0.4869 1 0.9502] Game Setup
  (CallFunction|GameSetupClient))

(event Custom|Game%20Setup%20Client
  ;[0.4869 1 0.9502] Game Setup
  (Utilities|FlowControl|Sequence
    (:then_0
      (if (Variables|Default|GetGroup1?)
        (bind _output_get (Variables|Default|SetGroup%201 (Utilities|Array|MakeArray (Variables|Default|GetPeg1) (Variables|Default|GetPeg2) (Variables|Default|GetPeg3) (Variables|Default|GetPeg4) (Variables|Default|GetPeg) (Variables|Default|GetPeg11) (Variables|Default|GetPeg13) (Variables|Default|GetPeg14) (Variables|Default|GetPeg8) (Variables|Default|GetPeg21) (Variables|Default|GetPeg23) (Variables|Default|GetPeg24) (Variables|Default|GetPeg26) (Variables|Default|GetPeg19))))
        (for _array_element _output_get
          (Transformation|SetWorldLocation _array_element (Math|Vector|MakeVector 0.0 0.0 (- (.z (Transformation|GetWorldLocation _array_element)) 2e+02)) false false))
        (elif (Variables|Default|GetGroup2?)
          (bind _output_get_2 (Variables|Default|SetGroup%202 (Utilities|Array|MakeArray (Variables|Default|GetPeg6) (Variables|Default|GetPeg7) (Variables|Default|GetPeg10) (Variables|Default|GetPeg15) (Variables|Default|GetPeg16) (Variables|Default|GetPeg12) (Variables|Default|GetPeg9) (Variables|Default|GetPeg5) (Variables|Default|GetPeg17) (Variables|Default|GetPeg22) (Variables|Default|GetPeg18) (Variables|Default|GetPeg25) (Variables|Default|GetPeg20))))
          (for _array_element_2 _output_get_2
            (Transformation|SetWorldLocation _array_element_2 (Math|Vector|MakeVector 0.0 0.0 (- (.z (Transformation|GetWorldLocation _array_element_2)) 2e+02)) false false)))))))

(event Custom|Server%20Reorder
  (CallFunction|ClientReorder))

(event Custom|Client%20Reorder
  (if (Variables|Default|GetGroup1?)
    (for _array_element (Variables|Default|GetGroup%201)
      (Transformation|SetWorldLocation _array_element (Math|Vector|MakeVector 0.0 0.0 (- (.z (Transformation|GetWorldLocation _array_element)) 2e+02)) false false)
      (Development|PrintString (Utilities|String|ToString(Float) (- (.z (Transformation|GetWorldLocation _array_element)) 2e+02))))
    (Variables|Default|SetGroup2? true)
    (Variables|Default|SetGroup1? false)
    (elif (Variables|Default|GetGroup2?)
      (for _array_element_2 (Variables|Default|GetGroup%201)
        (Transformation|SetWorldLocation _array_element_2 (Math|Vector|MakeVector 0.0 0.0 (+ (.z (Transformation|GetWorldLocation _array_element_2)) 2e+02)) false false))
      (Variables|Default|SetGroup1? true)
      (Variables|Default|SetGroup2? false))))

(event EventBeginPlay
  ;[0.4869 1 0.9502] Game Setup
  (if (Networking|IsServer)
    (bind _output_get (Variables|Default|SetStart%20Position (Math|Random|RandomIntegerinRange 1 2)))
    (if (== _output_get 1)
      (Variables|Default|SetGroup1? true)
      (else
        (Variables|Default|SetGroup2? true)))
    (if (Networking|IsServer)
      (Variables|Default|SetScore 0)
      (Development|PrintString (Utilities|String|ToString(Integer) (Variables|Default|GetStart%20Position))))))

(event EventBeginfromHUB
  ;[0.4869 1 0.9502] Game Setup
  (if (Networking|IsServer)
    (Development|PrintString (Utilities|String|Append "Enter From Node: " (Utilities|String|ToString(Integer) (Variables|Default|GetEnterFromNode))) true true "(R=0.000000,G=0.660000,B=1.000000,A=1.000000)" 5.0)
    (Variables|Default|SetSolved false)
    (CallFunction|GameSetupServer)))

(fn ConstructionScript
  (|CallParentFunction))
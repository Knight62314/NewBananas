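; BP_DefendCombat is a combat room Blueprint that keeps melee enemies in play until the room timer runs out.
; Starting from the hub clears existing melee enemies and spawns a ring of eight around the room's origin.
; Each kill spawns a replacement at a random point within the same square, and the timer finishing calls RoomWon.
; Logic to destroy BP_AttackObjective actors is present but unconnected.
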(event EventBeginfromHUB
  ;[1 1 1] Enemy Spawns
  (CallFunction|KillAllMeleeEnemies)
  (CallFunction|SpawnMeleeEnemy "-1000.000000,-1000.000000,0.000000" "NewEnumerator0")
  (CallFunction|SpawnMeleeEnemy "-1000.000000,0.000000,0.000000" "NewEnumerator0")
  (CallFunction|SpawnMeleeEnemy "-1000.000000,1000.000000,0.000000" "NewEnumerator0")
  (CallFunction|SpawnMeleeEnemy "0.000000,-1000.000000,0.000000" "NewEnumerator0")
  (CallFunction|SpawnMeleeEnemy "0.000000,1000.000000,0.000000" "NewEnumerator0")
  (CallFunction|SpawnMeleeEnemy "1000.000000,-1000.000000,0.000000" "NewEnumerator0")
  (CallFunction|SpawnMeleeEnemy "1000.000000,0.000000,0.000000" "NewEnumerator0")
  (CallFunction|SpawnMeleeEnemy "1000.000000,1000.000000,0.000000" "NewEnumerator0"))

(event EventEnemyKilled
  (bind _returnvalue (Math|Random|RandomFloatinRange -1e+03 1e+03))
  ;[1 1 1] Enemy Respawn
  (CallFunction|SpawnMeleeEnemy (Math|Vector|MakeVector _returnvalue _returnvalue 0.0) "NewEnumerator0"))

(event EventRoomTimerFinished
  (CallFunction|RoomWon))

(fn ConstructionScript
  (|CallParentFunction))
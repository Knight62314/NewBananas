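; Defend-combat room where players protect a spawned objective from minions until the room timer finishes.
; Starting from the HUB creates the attack UI, objective and initial enemy ring; each kill triggers a weighted random respawn at a spawn point.
; Self-rescheduling one-second timers poll for objective destruction or all players dead, either losing the room.
; Outcomes clear objective and minions; ending from the HUB also removes widgets and revives players.
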(event Custom|Objective%20Destoryed
  ;[1 1 1] Game Control
  (if (Variables|ObjectiveControl|GetLoop)
    (Utilities|Time|SetTimerbyEvent (delegate Custom|Objective%20Destoryed) 1.0)
    (if (Variables|/Game/Tyler/Blueprints/Rooms/DefendCombat/BP_DefendObjective.BP_DefendObjective_C|GetIsDestoryed? (Variables|ObjectiveControl|GetObjective))
      (Actor|DestroyActor (Variables|ObjectiveControl|GetObjective))
      (CallFunction|RoomLost)
      (bind _outactors (Actor|GetAllActorswithTag "Minion"))
      (for _array_element _outactors
        (Actor|DestroyActor _array_element)))))

(event Custom|CheckDeadPlayers
  ;[1 1 1] Game Control
  (if (Variables|ObjectiveControl|GetLoop)
    (bind _returnvalue (Utilities|Time|SetTimerbyEvent (delegate Custom|CheckDeadPlayers) 1.0))
    (Variables|PlayerDeathCount|SetDeadTimer _returnvalue)
    (for _array_element (Variables|PlayerDeathCount|GetPlayerList)
      (if (and (.Bool (Utilities|IsActorPlayer _array_element)) (Variables|/Game/ThirdPerson/Blueprints/CharacterParent_BP.CharacterParent_BP_C|GetIsDead? (.Player (Utilities|IsActorPlayer _array_element))))
        (Math|Integer|DecrementInt (Variables|PlayerDeathCount|GetPlayerNum)
          (:%20%20
            (Utilities|Array|RemoveItem (Variables|PlayerDeathCount|GetPlayerList) _array_element)))))
    (if (and (<= (Variables|PlayerDeathCount|GetPlayerNum) 0) (== (Variables|PlayerDeathCount|GetAllDead?) false))
      (Variables|PlayerDeathCount|SetAllDead? true)
      (CallFunction|RoomLost)
      (bind _outactors (Actor|GetAllActorsOfClass "/Game/Tyler/Blueprints/Rooms/DefendCombat/BP_DefendObjective.BP_DefendObjective_C"))
      (for _array_element_2 _outactors
        (Actor|DestroyActor _array_element_2))
      (bind _outactors_2 (Actor|GetAllActorswithTag "Minion"))
      (for _array_element_3 _outactors_2
        (Actor|DestroyActor _array_element_3)))))

(event EventBeginfromHUB
  ;[0.1156 1 0.1451] Game Setup
  (Variables|ObjectiveControl|SetLoop true)
  (Variables|PlayerDeathCount|SetAllDead? false)
  (bind (_players _count) (CallFunction|GetAllPlayers))
  (Variables|PlayerDeathCount|SetPlayerList _players)
  (Variables|PlayerDeathCount|SetPlayerNum _count)
  (CallFunction|KillAllMeleeEnemies)
  (bind _returnvalue (UserInterface|CreateWidget "/Game/Tyler/Blueprints/Rooms/AttackCombat/W_AttackUI.W_AttackUI_C"))
  (bind _output_get (Variables|UIElements|SetDefendUI _returnvalue))
  (UserInterface|Viewport|AddtoViewport _output_get 0)
  (bind _returnvalue_2 (Game|SpawnActorfromClass "/Game/Tyler/Blueprints/Rooms/DefendCombat/BP_DefendObjective.BP_DefendObjective_C" (Math|Transform|MakeTransform (Transformation|GetWorldLocation (Variables|Default|GetArrow)) "0, 0, 0" "1.000000,1.000000,1.000000") "Undefined" "MultiplyWithRoot" 0 0))
  (bind _output_get_2 (Variables|ObjectiveControl|SetObjective _returnvalue_2))
  (CallFunction|SpawnEnemy "-1000.000000,-1000.000000,0.000000" "NewEnumerator0" false)
  (CallFunction|SpawnEnemy "-1000.000000,0.000000,0.000000" "NewEnumerator3" false)
  (CallFunction|SpawnEnemy "-1000.000000,1000.000000,0.000000" "NewEnumerator0" false)
  (CallFunction|SpawnEnemy "0.000000,-1000.000000,0.000000" "NewEnumerator4" false)
  (CallFunction|SpawnEnemy "0.000000,1000.000000,0.000000" "NewEnumerator3" false)
  (CallFunction|SpawnEnemy "1000.000000,-1000.000000,0.000000" "NewEnumerator0" false)
  (CallFunction|SpawnEnemy "1000.000000,0.000000,0.000000" "NewEnumerator2" false)
  (CallFunction|SpawnEnemy "1000.000000,1000.000000,0.000000" "NewEnumerator0" false)
  (if (not (Variables|/Game/Tyler/Blueprints/Rooms/DefendCombat/BP_DefendObjective.BP_DefendObjective_C|GetIsDestoryed? _output_get_2))
    (CallFunction|ObjectiveDestoryed)
    (CallFunction|CheckDeadPlayers)))

(event EventEnemyKilled
  ;[0.1475 0.2192 1] Enemy Respawns
  (Variables|EnemyInformation|SetSpawnRoll (Math|Random|RandomInteger 9))
  (Variables|EnemyInformation|SetLocationRoll (Math|Random|RandomInteger 3))
  (Utilities|FlowControl|Sequence
    (:then_0
      (if (== (Variables|EnemyInformation|GetLocationRoll) 0)
        (Variables|EnemyInformation|SetSpawnLocation (Variables|/Script/Engine.SceneComponent|GetRelativeLocation (Variables|Default|GetEnemySpawnPoint)))))
    (:then_1
      (if (== (Variables|EnemyInformation|GetLocationRoll) 1)
        (Variables|EnemyInformation|SetSpawnLocation (Variables|/Script/Engine.SceneComponent|GetRelativeLocation (Variables|Default|GetEnemySpawnPoint2)))))
    (:then_2
      (if (== (Variables|EnemyInformation|GetLocationRoll) 2)
        (Variables|EnemyInformation|SetSpawnLocation (Variables|/Script/Engine.SceneComponent|GetRelativeLocation (Variables|Default|GetEnemySpawnPoint3)))))
    (:then_3
      (if (== (Variables|EnemyInformation|GetLocationRoll) 3)
        (Variables|EnemyInformation|SetSpawnLocation (Variables|/Script/Engine.SceneComponent|GetRelativeLocation (Variables|Default|GetEnemySpawnPoint4)))))
    (:then_4
      (Utilities|FlowControl|Sequence
        (:then_0
          (if (< (Variables|EnemyInformation|GetSpawnRoll) 4)
            (CallFunction|SpawnEnemy (Variables|EnemyInformation|GetSpawnLocation) "NewEnumerator0" false)))
        (:then_1
          (if (and (> (Variables|EnemyInformation|GetSpawnRoll) 3) (< (Variables|EnemyInformation|GetSpawnRoll) 7))
            (CallFunction|SpawnEnemy (Variables|EnemyInformation|GetSpawnLocation) "NewEnumerator3" false)))
        (:then_2
          (if (or (== (Variables|EnemyInformation|GetSpawnRoll) 7) (== (Variables|EnemyInformation|GetSpawnRoll) 8))
            (CallFunction|SpawnEnemy (Variables|EnemyInformation|GetSpawnLocation) "NewEnumerator1" false)))
        (:then_3
          (if (== (Variables|EnemyInformation|GetSpawnRoll) 9)
            (CallFunction|SpawnEnemy (Variables|EnemyInformation|GetSpawnLocation) "NewEnumerator2" false)))
        (:then_4
          (if (== (Variables|EnemyInformation|GetSpawnRoll) 10)
            (CallFunction|SpawnEnemy (Variables|EnemyInformation|GetSpawnLocation) "NewEnumerator4" false)))))))

(event EventRoomTimerFinished
  ;[1 1 1] Game Control
  (CallFunction|RoomWon)
  (Actor|DestroyActor (Variables|ObjectiveControl|GetObjective))
  (bind _outactors (Actor|GetAllActorswithTag "Minion"))
  (for _array_element _outactors
    (Actor|DestroyActor _array_element)))

(event EventEndfromHUB
  ;[1 1 1] Game Control
  (Variables|ObjectiveControl|SetLoop false)
  (Viewport|RemoveAllWidgets)
  (bind _outactors (Actor|GetAllActorsOfClass "/Game/ThirdPerson/Blueprints/BP_ThirdPersonCharacter.BP_ThirdPersonCharacter_C"))
  (for _array_element _outactors
    (Default|ReviveServer _array_element)
    (bind _outactors_2 (Actor|GetAllActorsOfClass "/Game/Tyler/Blueprints/Rooms/DefendCombat/BP_DefendObjective.BP_DefendObjective_C"))
    (for _array_element_2 _outactors_2
      (Actor|DestroyActor _array_element_2)
      (bind _outactors_3 (Actor|GetAllActorswithTag "Minion"))
      (for _array_element_3 _outactors_3
        (Actor|DestroyActor _array_element_3)))))

(fn ConstructionScript
  (|CallParentFunction))
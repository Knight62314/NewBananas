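; BP_PanicPlatform is a Platform Panic tile that signals when it is safe or shakes and drops.
; StartRound randomizes shake strength, then briefly flashes safe tiles blue via a dynamic material or sets IsFalling after a delay.
; Tick applies sine-wave rotation and a fixed swept drop, but only while IsShaking is set.
; SetSafeState's hardcoded true branch always flickers, leaving its ShakeWarning call, which sets IsShaking, unreachable.
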(event EventBeginPlay
  (bind _platform (Variables|Default|GetPlatform))
  (bind _returnvalue (Rendering|Material|CreateDynamicMaterialInstance _platform 0 "/Game/Tyler/Blueprints/Rooms/PlatformPanic/M_PanicPlatfrom.M_PanicPlatfrom" "None" :!class /Script/Engine.PrimitiveComponent))
  (bind _output_get (Variables|Default|SetMaterial _returnvalue))
  (Rendering|Material|SetMaterial _platform 0 _output_get)
  (Variables|Default|SetOrginalRotation (Variables|/Script/Engine.SceneComponent|GetRelativeRotation _platform))
  (Variables|Default|SetDefaultLocation (Variables|/Script/Engine.SceneComponent|GetRelativeLocation _platform)))

(event EventTick
  (params (DeltaSeconds :type Float%20%28single-precision%29))
  (bind _defaultlocation (Variables|Default|GetDefaultLocation))
  (if (Variables|Default|GetIsShaking)
    (Variables|Default|SetCurrentShakeTimer (+ (Variables|Default|GetCurrentShakeTimer) DeltaSeconds))
    (bind _output_get (Variables|Default|SetShakeAngle (* (Math|Trig|Sin(Radians) (* (Variables|Default|GetCurrentShakeTimer) (Variables|Default|GetShakeFrequency))) (Variables|Default|GetShakeStrength))))
    (Transformation|SetRelativeRotation (Variables|Default|GetPlatform) (Math|Rotator|MakeRotator 0.0 _output_get _output_get) false false)
    (if (Variables|Default|GetIsFalling)
      (Transformation|SetRelativeLocation (Variables|Default|GetPlatform) (Math|Vector|MakeVector (.x _defaultlocation) (.y _defaultlocation) (- (.z _defaultlocation) 1e+02)) true false))))

(fn ConstructionScript)

(fn SetSafeState
  (Variables|Default|SetIsSafe (Variables|Default|GetIsSafe))
  (if true
    (CallFunction|FlickerState)
    (else
      (CallFunction|ShakeWarning))))

(fn FlickerState
  (bind _material (Variables|Default|GetMaterial))
  (Rendering|Material|SetVectorParameterValue _material "FlickerColor" "(R=0.000000,G=0.305882,B=1.000000,A=1.000000)" :!class /Script/Engine.MaterialInstanceDynamic)
  (Rendering|Material|SetScalarParameterValue _material "FlickerAlpha" 1.0 :!class /Script/Engine.MaterialInstanceDynamic)
  (Utilities|Time|SetTimerbyFunctionName 0 "ResetFlicker" 0.75))

(fn ShakeWarning
  (Variables|Default|SetIsShaking true))

(fn ResetFlicker
  (Rendering|Material|SetScalarParameterValue (Variables|Default|GetMaterial) "FlickerAlpha" 0.0 :!class /Script/Engine.MaterialInstanceDynamic))

(fn StartRound
  (Variables|Default|SetIsSafe (Variables|Default|GetIsSafe))
  (Variables|Default|SetFallSpeed (Variables|Default|GetFallSpeed))
  (Variables|Default|SetFallDelay (Variables|Default|GetFallDelay))
  (Variables|Default|SetShakeStrength (Math|Random|RandomFloatinRange 5.0 15.0))
  (if (Variables|Default|GetIsSafe)
    (CallFunction|FlickerState)
    (else
      (Utilities|Time|SetTimerbyFunctionName 0 "StartFalling" (Variables|Default|GetFallDelay)))))

(fn StartFalling
  (Variables|Default|SetIsFalling true))
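; Platform Panic room actor that runs a minigame where a few random platforms are safe and the rest warn by shaking.
; BeginfromHUB spawns a grid of platforms around the actor's location, then calls StartGame after a short delay.
; StartGame shuffles a copy of the platform array to pick one to three safe BP_PanicPlatforms, which flicker, while the others start their shake warning.
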(event Custom|Start%20Game
  (Variables|Default|SetSafeCount (Math|Random|RandomIntegerinRange 1 3))
  (bind _output_get (Variables|Default|SetShuffle%20Array (Variables|Default|GetPlatforms)))
  (Utilities|Array|Shuffle _output_get)
  (Utilities|Array|Clear (Variables|Default|GetSafePlatforms))
  (for _index (range 0 (- (Variables|Default|GetSafeCount) 1))
    (Utilities|Array|Add (Variables|Default|GetSafePlatforms) (Utilities|Array|Get(acopy) (Variables|Default|GetShuffle%20Array) _index)))
  (for _array_element (Variables|Default|GetPlatforms)
    (if (Utilities|Array|ContainsItem (Variables|Default|GetSafePlatforms) _array_element)
      (bind _asbp_panic_platform (Utilities|Casting|CastToBP_PanicPlatform _array_element))
      (Default|FlickerState _asbp_panic_platform)
      (Variables|/Game/Tyler/Blueprints/Rooms/PlatformPanic/BP_PanicPlatform.BP_PanicPlatform_C|SetIsFalling _asbp_panic_platform false)
      (else
        (bind _asbp_panic_platform_2 (Utilities|Casting|CastToBP_PanicPlatform _array_element))
        (Variables|/Game/Tyler/Blueprints/Rooms/PlatformPanic/BP_PanicPlatform.BP_PanicPlatform_C|SetIsShaking _asbp_panic_platform_2 true)
        (Default|ShakeWarning _asbp_panic_platform_2)))))

(event Collision|EventActorBeginOverlap
  (params (OtherActor :type Actor%20Object%20Reference)))

(event EventTick
  (params (DeltaSeconds :type Float%20%28single-precision%29)))

(event EventBeginfromHUB
  (bind _gridsize (Variables|Default|GetGridSize))
  (bind _returnvalue (- _gridsize 1))
  (Variables|Default|SetGame%20Origin (Transformation|GetActorLocation))
  (for _index (range 0 _returnvalue)
    (for _index_2 (range 0 _returnvalue)
      (bind _output_get (Variables|Default|SetXLoc (* (Variables|Default|GetSpacing) (- _index 1))))
      (bind _output_get_2 (Variables|Default|SetYLoc (* (- _index_2 1) (Variables|Default|GetSpacing))))
      (bind _output_get_3 (Variables|Default|SetLocalPoint (Math|Vector|MakeVector _output_get _output_get_2 1e+02)))
      (Utilities|Array|Add (Variables|Default|GetSpawnPoints) (+ _output_get_3 (Variables|Default|GetGame%20Origin)))
      (bind _returnvalue_2 (Game|SpawnActorfromClass (Variables|Default|GetPlatformClass) (Math|Transform|MakeTransform (+ _output_get_3 (Variables|Default|GetGame%20Origin)) "0, 0, 0" "1.000000,1.000000,1.000000") "Undefined" "MultiplyWithRoot" 0 0 0))
      (Utilities|Array|Add (Variables|Default|GetPlatforms) _returnvalue_2))
    (Utilities|FlowControl|Delay 3.0)
    (CallFunction|StartGame)))

(event EventBeginPlay)

(fn ConstructionScript
  (|CallParentFunction))
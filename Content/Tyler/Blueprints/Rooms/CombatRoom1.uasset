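; CombatRoom1 is a combat room Blueprint that works with a HUB and holds a melee enemy encounter.
; Its BeginfromHUB event spawns one Melee_Enemy_Character at a fixed offset from the room's root.
; When an actor of exactly the BP_ThirdPersonCharacter class overlaps its Box, it calls MoveToHUBFunction on the HUB, passing itself.
; The construction script only calls its parent's.
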(event OnComponentBeginOverlap(Box)
  (params (OverlappedComponent :type Primitive%20Component%20Object%20Reference) (OtherActor :type Actor%20Object%20Reference) (OtherComp :type Primitive%20Component%20Object%20Reference) (OtherBodyIndex :type Integer) (bFromSweep :type Boolean) (SweepResult :type Hit%20Result%20Structure%20%28by%20ref%29))
  (if (== (Utilities|GetClass OtherActor) "/Game/ThirdPerson/Blueprints/BP_ThirdPersonCharacter.BP_ThirdPersonCharacter_C")
    (Default|MovetoHUBFunction (Variables|Default|GetHUB) self)))

(event EventBeginfromHUB
  (Game|SpawnActorfromClass "/Game/AI_Entities/Demo_Enemy/Melee_Enemy/Melee_Enemy_Character.Melee_Enemy_Character_C" (Math|Transform|MakeTransform (+ (Transformation|GetWorldLocation (Variables|Default|GetDefaultSceneRoot)) "-750.000000,-750.000000,50.000000") "0.000000,-90.000000,0.000000") "Undefined" "MultiplyWithRoot" 0 0))

(fn ConstructionScript
  (|CallParentFunction))
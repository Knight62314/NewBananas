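; Horde is a combat room Blueprint that pits the player against a ring of melee enemies.
; When the room begins from the hub, it spawns eight melee enemies in a square grid around an empty center.
; On each enemy kill it checks the inherited melee enemy list and declares the room won once it is empty.
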(event EventEnemyKilled
  (if (== (Utilities|Array|Length (Variables|Default|GetMeleeEnemies)) 0)
    (CallFunction|RoomWon)))

(event EventBeginfromHUB
  (CallFunction|SpawnMeleeEnemy "-1000.000000,-1000.000000,0.000000")
  (CallFunction|SpawnMeleeEnemy "0.000000,-1000.000000,0.000000")
  (CallFunction|SpawnMeleeEnemy "1000.000000,-1000.000000,0.000000")
  (CallFunction|SpawnMeleeEnemy "-1000.000000,0.000000,0.000000")
  (CallFunction|SpawnMeleeEnemy "1000.000000,0.000000,0.000000")
  (CallFunction|SpawnMeleeEnemy "-1000.000000,1000.000000,0.000000")
  (CallFunction|SpawnMeleeEnemy "0.000000,1000.000000,0.000000")
  (CallFunction|SpawnMeleeEnemy "1000.000000,1000.000000,0.000000"))

(fn ConstructionScript
  (|CallParentFunction))
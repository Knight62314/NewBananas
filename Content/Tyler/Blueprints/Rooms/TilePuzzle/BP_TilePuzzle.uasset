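; Tile puzzle room that is solved when all nine tiles are active, then hands back to the HUB.
; BeginfromHUB runs server-gated setup, spawning BP_Tile_Puzzle_Piece actors at arrow components and wiring each one's bordering tiles as a 3x3 grid.
; A self-calling 0.5-second timer polls the tiles' Active flags rather than using Tick.
; On success, EndPuzzle waits briefly, then calls the HUB's MoveToHUBFunction.
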(event Custom|End%20Puzzle
  ;[1 1 1] Tile Puzzle
  ;;[1 1 1] End Puzzle
  (if (and (Variables|Default|GetSolved?) (Variables|Default|GetEnd?))
    (Utilities|FlowControl|Delay 2.0)
    (Default|MovetoHUBFunction (Variables|Default|GetHUB) self)
    (Variables|Default|SetEnd? false)))

(event Custom|ServerSetup
  ;[1 1 1] Tile Puzzle
  (CallFunction|ClientSetup))

(event Custom|ClientSetup
  ;[1 1 1] Tile Puzzle
  ;;[1 1 1] Create Tiles
  (Utilities|FlowControl|Sequence
    (:then_0
      (bind _returnvalue (Game|SpawnActorfromClass "/Game/Tyler/Blueprints/Rooms/TilePuzzle/BP_Tile_Puzzle_Piece.BP_Tile_Puzzle_Piece_C" (Math|Transform|MakeTransform (Transformation|GetWorldLocation (Variables|Default|GetArrow1)) (Transformation|GetActorRotation) "1.000000,1.000000,1.000000") "Undefined" "MultiplyWithRoot" 0 0))
      (Variables|Default|SetS1 _returnvalue))
    (:then_1
      (bind _returnvalue_2 (Game|SpawnActorfromClass "/Game/Tyler/Blueprints/Rooms/TilePuzzle/BP_Tile_Puzzle_Piece.BP_Tile_Puzzle_Piece_C" (Math|Transform|MakeTransform (Transformation|GetWorldLocation (Variables|Default|GetArrow2)) (Transformation|GetActorRotation) "1.000000,1.000000,1.000000") "Undefined" "MultiplyWithRoot" 0 0))
      (Variables|Default|SetS2 _returnvalue_2))
    (:then_2
      (bind _returnvalue_3 (Game|SpawnActorfromClass "/Game/Tyler/Blueprints/Rooms/TilePuzzle/BP_Tile_Puzzle_Piece.BP_Tile_Puzzle_Piece_C" (Math|Transform|MakeTransform (Transformation|GetWorldLocation (Variables|Default|GetArrow3)) (Transformation|GetActorRotation) "1.000000,1.000000,1.000000") "Undefined" "MultiplyWithRoot" 0 0))
      (Variables|Default|SetS3 _returnvalue_3))
    (:then_3
      (bind _returnvalue_4 (Game|SpawnActorfromClass "/Game/Tyler/Blueprints/Rooms/TilePuzzle/BP_Tile_Puzzle_Piece.BP_Tile_Puzzle_Piece_C" (Math|Transform|MakeTransform (Transformation|GetWorldLocation (Variables|Default|GetArrow4)) (Transformation|GetActorRotation) "1.000000,1.000000,1.000000") "Undefined" "MultiplyWithRoot" 0 0))
      (Variables|Default|SetS4 _returnvalue_4))
    (:then_4
      (bind _returnvalue_5 (Game|SpawnActorfromClass "/Game/Tyler/Blueprints/Rooms/TilePuzzle/BP_Tile_Puzzle_Piece.BP_Tile_Puzzle_Piece_C" (Math|Transform|MakeTransform (Transformation|GetWorldLocation (Variables|Default|GetArrow5)) (Transformation|GetActorRotation) "1.000000,1.000000,1.000000") "Undefined" "MultiplyWithRoot" 0 0))
      (Variables|Default|SetS5 _returnvalue_5))
    (:then_5
      (bind _returnvalue_6 (Game|SpawnActorfromClass "/Game/Tyler/Blueprints/Rooms/TilePuzzle/BP_Tile_Puzzle_Piece.BP_Tile_Puzzle_Piece_C" (Math|Transform|MakeTransform (Transformation|GetWorldLocation (Variables|Default|GetArrow6)) (Transformation|GetActorRotation) "1.000000,1.000000,1.000000") "Undefined" "MultiplyWithRoot" 0 0))
      (Variables|Default|SetS6 _returnvalue_6))
    (:then_6
      (bind _returnvalue_7 (Game|SpawnActorfromClass "/Game/Tyler/Blueprints/Rooms/TilePuzzle/BP_Tile_Puzzle_Piece.BP_Tile_Puzzle_Piece_C" (Math|Transform|MakeTransform (Transformation|GetWorldLocation (Variables|Default|GetArrow7)) (Transformation|GetActorRotation) "1.000000,1.000000,1.000000") "Undefined" "MultiplyWithRoot" 0 0))
      (Variables|Default|SetS7 _returnvalue_7))
    (:then_7
      (bind _returnvalue_8 (Game|SpawnActorfromClass "/Game/Tyler/Blueprints/Rooms/TilePuzzle/BP_Tile_Puzzle_Piece.BP_Tile_Puzzle_Piece_C" (Math|Transform|MakeTransform (Transformation|GetWorldLocation (Variables|Default|GetArrow8)) (Transformation|GetActorRotation) "1.000000,1.000000,1.000000") "Undefined" "MultiplyWithRoot" 0 0))
      (Variables|Default|SetS8 _returnvalue_8))
    (:then_8
      (bind _returnvalue_9 (Game|SpawnActorfromClass "/Game/Tyler/Blueprints/Rooms/TilePuzzle/BP_Tile_Puzzle_Piece.BP_Tile_Puzzle_Piece_C" (Math|Transform|MakeTransform (Transformation|GetWorldLocation (Variables|Default|GetArrow9)) (Transformation|GetActorRotation) "1.000000,1.000000,1.000000") "Undefined" "MultiplyWithRoot" 0 0))
      (Variables|Default|SetS9 _returnvalue_9)
      ;;[1 1 1] Set Tile Nieghbors
      (Utilities|FlowControl|Sequence
        (:then_0
          (Variables|/Game/Tyler/Blueprints/Rooms/TilePuzzle/BP_Tile_Puzzle_Piece.BP_Tile_Puzzle_Piece_C|SetActive? (Variables|Default|GetS1) false)
          (Variables|/Game/Tyler/Blueprints/Rooms/TilePuzzle/BP_Tile_Puzzle_Piece.BP_Tile_Puzzle_Piece_C|SetBorderingSpace (Variables|Default|GetS1) (Utilities|Array|MakeArray (Variables|Default|GetS2) (Variables|Default|GetS6))))
        (:then_1
          (Variables|/Game/Tyler/Blueprints/Rooms/TilePuzzle/BP_Tile_Puzzle_Piece.BP_Tile_Puzzle_Piece_C|SetActive? (Variables|Default|GetS2) false)
          (Variables|/Game/Tyler/Blueprints/Rooms/TilePuzzle/BP_Tile_Puzzle_Piece.BP_Tile_Puzzle_Piece_C|SetBorderingSpace (Variables|Default|GetS2) (Utilities|Array|MakeArray (Variables|Default|GetS1) (Variables|Default|GetS3) (Variables|Default|GetS5))))
        (:then_2
          (Variables|/Game/Tyler/Blueprints/Rooms/TilePuzzle/BP_Tile_Puzzle_Piece.BP_Tile_Puzzle_Piece_C|SetActive? (Variables|Default|GetS3) false)
          (Variables|/Game/Tyler/Blueprints/Rooms/TilePuzzle/BP_Tile_Puzzle_Piece.BP_Tile_Puzzle_Piece_C|SetBorderingSpace (Variables|Default|GetS3) (Utilities|Array|MakeArray (Variables|Default|GetS2) (Variables|Default|GetS4))))
        (:then_3
          (Variables|/Game/Tyler/Blueprints/Rooms/TilePuzzle/BP_Tile_Puzzle_Piece.BP_Tile_Puzzle_Piece_C|SetActive? (Variables|Default|GetS4) false)
          (Variables|/Game/Tyler/Blueprints/Rooms/TilePuzzle/BP_Tile_Puzzle_Piece.BP_Tile_Puzzle_Piece_C|SetBorderingSpace (Variables|Default|GetS4) (Utilities|Array|MakeArray (Variables|Default|GetS3) (Variables|Default|GetS5) (Variables|Default|GetS8))))
        (:then_4
          (Variables|/Game/Tyler/Blueprints/Rooms/TilePuzzle/BP_Tile_Puzzle_Piece.BP_Tile_Puzzle_Piece_C|SetActive? (Variables|Default|GetS5) false)
          (Variables|/Game/Tyler/Blueprints/Rooms/TilePuzzle/BP_Tile_Puzzle_Piece.BP_Tile_Puzzle_Piece_C|SetBorderingSpace (Variables|Default|GetS5) (Utilities|Array|MakeArray (Variables|Default|GetS2) (Variables|Default|GetS4) (Variables|Default|GetS6) (Variables|Default|GetS7))))
        (:then_5
          (Variables|/Game/Tyler/Blueprints/Rooms/TilePuzzle/BP_Tile_Puzzle_Piece.BP_Tile_Puzzle_Piece_C|SetActive? (Variables|Default|GetS6) false)
          (Variables|/Game/Tyler/Blueprints/Rooms/TilePuzzle/BP_Tile_Puzzle_Piece.BP_Tile_Puzzle_Piece_C|SetBorderingSpace (Variables|Default|GetS6) (Utilities|Array|MakeArray (Variables|Default|GetS1) (Variables|Default|GetS5) (Variables|Default|GetS9))))
        (:then_6
          (Variables|/Game/Tyler/Blueprints/Rooms/TilePuzzle/BP_Tile_Puzzle_Piece.BP_Tile_Puzzle_Piece_C|SetActive? (Variables|Default|GetS7) false)
          (Variables|/Game/Tyler/Blueprints/Rooms/TilePuzzle/BP_Tile_Puzzle_Piece.BP_Tile_Puzzle_Piece_C|SetBorderingSpace (Variables|Default|GetS7) (Utilities|Array|MakeArray (Variables|Default|GetS5) (Variables|Default|GetS8) (Variables|Default|GetS9))))
        (:then_7
          (Variables|/Game/Tyler/Blueprints/Rooms/TilePuzzle/BP_Tile_Puzzle_Piece.BP_Tile_Puzzle_Piece_C|SetActive? (Variables|Default|GetS8) false)
          (Variables|/Game/Tyler/Blueprints/Rooms/TilePuzzle/BP_Tile_Puzzle_Piece.BP_Tile_Puzzle_Piece_C|SetBorderingSpace (Variables|Default|GetS8) (Utilities|Array|MakeArray (Variables|Default|GetS4) (Variables|Default|GetS7))))
        (:then_8
          (Variables|/Game/Tyler/Blueprints/Rooms/TilePuzzle/BP_Tile_Puzzle_Piece.BP_Tile_Puzzle_Piece_C|SetActive? (Variables|Default|GetS9) false)
          (Variables|/Game/Tyler/Blueprints/Rooms/TilePuzzle/BP_Tile_Puzzle_Piece.BP_Tile_Puzzle_Piece_C|SetBorderingSpace (Variables|Default|GetS9) (Utilities|Array|MakeArray (Variables|Default|GetS6) (Variables|Default|GetS7))))))))

(event Custom|EndPuzzleCheckServer
  ;[1 1 1] Tile Puzzle
  ;;[1 1 1] End Puzzle
  (CallFunction|EndPuzzleCheckClient))

(event Custom|EndPuzzleCheckClient
  ;[1 1 1] Tile Puzzle
  ;;[1 1 1] End Puzzle
  (Utilities|Time|SetTimerbyEvent (delegate Custom|EndPuzzleCheckClient) 0.5 (== (Variables|Default|GetSolved?) false))
  (if (Math|Boolean|ANDBoolean (Variables|/Game/Tyler/Blueprints/Rooms/TilePuzzle/BP_Tile_Puzzle_Piece.BP_Tile_Puzzle_Piece_C|GetActive? (Variables|Default|GetS1)) (Variables|/Game/Tyler/Blueprints/Rooms/TilePuzzle/BP_Tile_Puzzle_Piece.BP_Tile_Puzzle_Piece_C|GetActive? (Variables|Default|GetS2)) (Variables|/Game/Tyler/Blueprints/Rooms/TilePuzzle/BP_Tile_Puzzle_Piece.BP_Tile_Puzzle_Piece_C|GetActive? (Variables|Default|GetS3)) (Variables|/Game/Tyler/Blueprints/Rooms/TilePuzzle/BP_Tile_Puzzle_Piece.BP_Tile_Puzzle_Piece_C|GetActive? (Variables|Default|GetS4)) (Variables|/Game/Tyler/Blueprints/Rooms/TilePuzzle/BP_Tile_Puzzle_Piece.BP_Tile_Puzzle_Piece_C|GetActive? (Variables|Default|GetS5)) (Variables|/Game/Tyler/Blueprints/Rooms/TilePuzzle/BP_Tile_Puzzle_Piece.BP_Tile_Puzzle_Piece_C|GetActive? (Variables|Default|GetS6)) (Variables|/Game/Tyler/Blueprints/Rooms/TilePuzzle/BP_Tile_Puzzle_Piece.BP_Tile_Puzzle_Piece_C|GetActive? (Variables|Default|GetS7)) (Variables|/Game/Tyler/Blueprints/Rooms/TilePuzzle/BP_Tile_Puzzle_Piece.BP_Tile_Puzzle_Piece_C|GetActive? (Variables|Default|GetS8)) (Variables|/Game/Tyler/Blueprints/Rooms/TilePuzzle/BP_Tile_Puzzle_Piece.BP_Tile_Puzzle_Piece_C|GetActive? (Variables|Default|GetS9)))
    (Variables|Default|SetSolved? true)
    (CallFunction|EndPuzzle)))

(event EventBeginPlay
  ;[1 1 1] Tile Puzzle
  (Variables|Default|SetSolved? false))

(event EventTick
  (params (DeltaSeconds :type Float%20%28single-precision%29))
  ;[1 1 1] Tile Puzzle
  ;;[1 1 1] End Puzzle
)

(event EventBeginfromHUB
  ;[1 1 1] Tile Puzzle
  (if (Networking|IsServer)
    (CallFunction|ServerSetup)
    (CallFunction|EndPuzzleCheckServer)))

(fn ConstructionScript
  (|CallParentFunction))
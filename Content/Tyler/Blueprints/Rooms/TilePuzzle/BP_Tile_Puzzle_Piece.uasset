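; BP_Tile_Puzzle_Piece is one floor tile in a Lights Out style puzzle that the player toggles by stepping on it.
; Overlap by BP_ThirdPersonCharacter on PuzzleSpace flips Active on the tile and every valid tile in BorderingSpace.
; Each flip adjusts this tile's own Correct counter up or down, including flips of neighbors.
; Tick continually sets the cube's on or off material from Active, which starts false.
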(event OnComponentBeginOverlap(PuzzleSpace)
  (params (OverlappedComponent :type Primitive%20Component%20Object%20Reference) (OtherActor :type Actor%20Object%20Reference) (OtherComp :type Primitive%20Component%20Object%20Reference) (OtherBodyIndex :type Integer) (bFromSweep :type Boolean) (SweepResult :type Hit%20Result%20Structure%20%28by%20ref%29))
  ;[1 1 1] Tile Puzzle Piece
  ;;[1 0.9136 0.08939] Current Tile State
  (if (== (Utilities|GetClass OtherActor) "/Game/ThirdPerson/Blueprints/BP_ThirdPersonCharacter.BP_ThirdPersonCharacter_C")
    (if (Variables|Default|GetActive?)
      (Variables|Default|SetActive? false)
      (Variables|Default|SetCorrect (+ (Variables|Default|GetCorrect) -1))
      (else
        (Variables|Default|SetActive? true)
        (Variables|Default|SetCorrect (+ (Variables|Default|GetCorrect) 1))))
    (for _array_element (Variables|Default|GetBorderingSpace)
      (Utilities|IsValid _array_element
        (:Is%20Valid
          (if (Variables|BP_Tile_Puzzle_Piece_C|GetActive? _array_element)
            (Variables|BP_Tile_Puzzle_Piece_C|SetActive? _array_element false)
            (Variables|Default|SetCorrect (+ (Variables|Default|GetCorrect) -1))
            (else
              (Variables|BP_Tile_Puzzle_Piece_C|SetActive? _array_element true)
              (Variables|Default|SetCorrect (+ (Variables|Default|GetCorrect) 1)))))))))

(event EventTick
  (params (DeltaSeconds :type Float%20%28single-precision%29))
  (bind _cube (Variables|Default|GetCube))
  ;[1 1 1] Tile Puzzle Piece
  ;;[0.2436 0.141 1] Change Tile Color and Value
  (if (Variables|Default|GetActive?)
    (Rendering|Material|SetMaterial _cube 0 "/Game/Tyler/Blueprints/Rooms/TilePuzzle/M_TileOn.M_TileOn")
    (else
      (Rendering|Material|SetMaterial _cube 0 "/Game/Tyler/Blueprints/Rooms/TilePuzzle/M_TileOff.M_TileOff"))))

(event EventBeginPlay
  ;[1 1 1] Tile Puzzle Piece
  ;;[1 0 0] Setup
  (Variables|Default|SetActive? false))

(fn ConstructionScript)
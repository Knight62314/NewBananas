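; Knight rotation puzzle room launched from the hub, won when all four pieces face their original knight yaws.
; Setup randomizes yaws in 45-degree steps for two knights and two knife components, rolling inside the Multicast event.
; Four lever boxes select a piece; overlap or OnInteract turns it 45 degrees via timeline, gated by Active.
; Each correct turn checks the win, which calls the HUB's move function, as does player overlap with Box_0.
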(event OnComponentBeginOverlap(Box_0)
  (params (OverlappedComponent :type Primitive%20Component%20Object%20Reference) (OtherActor :type Actor%20Object%20Reference) (OtherComp :type Primitive%20Component%20Object%20Reference) (OtherBodyIndex :type Integer) (bFromSweep :type Boolean) (SweepResult :type Hit%20Result%20Structure%20%28by%20ref%29))
  ;[1 1 1] Knight Puzzle
  ;;[1 1 1] Hub Controls
  (if (== (Utilities|GetClass OtherActor) "/Game/ThirdPerson/Blueprints/BP_ThirdPersonCharacter.BP_ThirdPersonCharacter_C")
    (Default|MovetoHUBFunction (Variables|Default|GetHUB) self)))

(event OnComponentBeginOverlap(Box1)
  (params (OverlappedComponent :type Primitive%20Component%20Object%20Reference) (OtherActor :type Actor%20Object%20Reference) (OtherComp :type Primitive%20Component%20Object%20Reference) (OtherBodyIndex :type Integer) (bFromSweep :type Boolean) (SweepResult :type Hit%20Result%20Structure%20%28by%20ref%29))
  ;[1 1 1] Knight Puzzle
  ;;[0.192 1 0.2754] Lever Gates
  (CallFunction|PlayerGate OtherActor)
  (Variables|Default|SetInteract? true)
  (CallFunction|ServerInteract))

(event OnComponentEndOverlap(Box1)
  (params (OverlappedComponent :type Primitive%20Component%20Object%20Reference) (OtherActor :type Actor%20Object%20Reference) (OtherComp :type Primitive%20Component%20Object%20Reference) (OtherBodyIndex :type Integer))
  ;[1 1 1] Knight Puzzle
  ;;[0.192 1 0.2754] Lever Gates
  (CallFunction|PlayerGate OtherActor)
  (Variables|Default|SetInteract? false))

(event OnComponentBeginOverlap(Box2)
  (params (OverlappedComponent :type Primitive%20Component%20Object%20Reference) (OtherActor :type Actor%20Object%20Reference) (OtherComp :type Primitive%20Component%20Object%20Reference) (OtherBodyIndex :type Integer) (bFromSweep :type Boolean) (SweepResult :type Hit%20Result%20Structure%20%28by%20ref%29))
  ;[1 1 1] Knight Puzzle
  ;;[0.192 1 0.2754] Lever Gates
  (CallFunction|PlayerGate OtherActor)
  (Variables|Default|SetInteract1? true)
  (CallFunction|ServerInteract))

(event OnComponentEndOverlap(Box2)
  (params (OverlappedComponent :type Primitive%20Component%20Object%20Reference) (OtherActor :type Actor%20Object%20Reference) (OtherComp :type Primitive%20Component%20Object%20Reference) (OtherBodyIndex :type Integer))
  ;[1 1 1] Knight Puzzle
  ;;[0.192 1 0.2754] Lever Gates
  (CallFunction|PlayerGate OtherActor)
  (Variables|Default|SetInteract1? false))

(event OnComponentBeginOverlap(Box3)
  (params (OverlappedComponent :type Primitive%20Component%20Object%20Reference) (OtherActor :type Actor%20Object%20Reference) (OtherComp :type Primitive%20Component%20Object%20Reference) (OtherBodyIndex :type Integer) (bFromSweep :type Boolean) (SweepResult :type Hit%20Result%20Structure%20%28by%20ref%29))
  ;[1 1 1] Knight Puzzle
  ;;[0.192 1 0.2754] Lever Gates
  (CallFunction|PlayerGate OtherActor)
  (Variables|Default|SetInteract2? true)
  (CallFunction|ServerInteract))

(event OnComponentEndOverlap(Box3)
  (params (OverlappedComponent :type Primitive%20Component%20Object%20Reference) (OtherActor :type Actor%20Object%20Reference) (OtherComp :type Primitive%20Component%20Object%20Reference) (OtherBodyIndex :type Integer))
  ;[1 1 1] Knight Puzzle
  ;;[0.192 1 0.2754] Lever Gates
  (CallFunction|PlayerGate OtherActor)
  (Variables|Default|SetInteract2? false))

(event OnComponentBeginOverlap(Box4)
  (params (OverlappedComponent :type Primitive%20Component%20Object%20Reference) (OtherActor :type Actor%20Object%20Reference) (OtherComp :type Primitive%20Component%20Object%20Reference) (OtherBodyIndex :type Integer) (bFromSweep :type Boolean) (SweepResult :type Hit%20Result%20Structure%20%28by%20ref%29))
  ;[1 1 1] Knight Puzzle
  ;;[0.192 1 0.2754] Lever Gates
  (CallFunction|PlayerGate OtherActor)
  (Variables|Default|SetInteract3? true)
  (CallFunction|ServerInteract))

(event OnComponentEndOverlap(Box4)
  (params (OverlappedComponent :type Primitive%20Component%20Object%20Reference) (OtherActor :type Actor%20Object%20Reference) (OtherComp :type Primitive%20Component%20Object%20Reference) (OtherBodyIndex :type Integer))
  ;[1 1 1] Knight Puzzle
  ;;[0.192 1 0.2754] Lever Gates
  (CallFunction|PlayerGate OtherActor)
  (Variables|Default|SetInteract3? false))

(event Custom|End%20Game
  ;[1 1 1] Knight Puzzle
  ;;[1 1 1] End Puzzle
  (if (Variables|Default|GetAllCorrect?)
    (Default|MovetoHUBFunction (Variables|Default|GetHUB) self)))

(event Custom|ServerInteract
  ;[1 1 1] Knight Puzzle
  ;;[1 1 1] Hub Controls
  (CallFunction|ClientInteract))

(event Custom|ClientInteract
  (bind _knife3 (Variables|Default|GetKnife3))
  (bind _knight1 (Variables|Default|GetKnight1))
  (bind _knight2 (Variables|Default|GetKnight2))
  (bind _knife (Variables|Default|GetKnife))
  ;[1 1 1] Knight Puzzle
  ;;[1 0.2098 0.172] Check Rotation
  (if (Variables|Default|GetActive?)
    (Variables|Default|SetActive? false)
    (Utilities|FlowControl|Sequence
      (:then_0
        (if (Variables|Default|GetInteract?)
          (bind _output_get (Variables|Default|SetKnightCurrentRotation (Variables|/Script/Engine.SceneComponent|GetRelativeRotation _knife)))
          (Variables|Default|SetKnightUpdatedRotation (Math|Rotator|CombineRotators _output_get "0.000000,45.000000,0.000000"))
          (bind _knight_rotation (Timeline|Knight%20Rotation PlayFromStart)
            (:Update
              (Transformation|SetRelativeRotation _knife (Math|Rotator|Lerp(Rotator) (Variables|Default|GetKnightCurrentRotation) (Variables|Default|GetKnightUpdatedRotation) _knight_rotation true) false false)
              (Utilities|FlowControl|Delay 1.1)
              (Variables|Default|SetActive? true)
              (if (== (.yaw (Variables|Default|GetKnightUpdatedRotation)) (.yaw (Variables|Default|GetKnight%20End%20Rotation)))
                (Variables|Default|SetKnightCorrect? true)
                ;;[0.3989 0.9101 1] Win Condition
                (if (or (Variables|Default|GetAllCorrect?) (Math|Boolean|ANDBoolean (Variables|Default|GetKnightCorrect?) (Variables|Default|GetKnight1Correct?) (Variables|Default|GetKnight2Correct?) (Variables|Default|GetKnight3Correct?))) :!label _label
                  (Variables|Default|SetAllCorrect? true)
                  (CallFunction|EndGame))
                (else
                  (Variables|Default|SetKnightCorrect? false)))))))
      (:then_1
        (if (Variables|Default|GetInteract1?)
          (bind _output_get_2 (Variables|Default|SetKnight1%20CurrentRotation (Variables|/Script/Engine.SceneComponent|GetRelativeRotation _knight1)))
          (Variables|Default|SetKnight1UpdatedRotation (Math|Rotator|CombineRotators _output_get_2 "0.000000,45.000000,0.000000"))
          (bind _knight1_rotation (Timeline|Knight1%20Rotation PlayFromStart)
            (:Update
              (Transformation|SetRelativeRotation _knight1 (Math|Rotator|Lerp(Rotator) (Variables|Default|GetKnight1%20CurrentRotation) (Variables|Default|GetKnight1UpdatedRotation) _knight1_rotation true) false false)
              (Utilities|FlowControl|Delay 1.1)
              (Variables|Default|SetActive? true)
              (if (== (.yaw (Variables|Default|GetKnight1UpdatedRotation)) (.yaw (Variables|Default|GetKnight1%20End%20Rotation)))
                (Variables|Default|SetKnight1Correct? true)
                (goto _label)
                (else
                  (Variables|Default|SetKnight1Correct? false)))))))
      (:then_2
        (if (Variables|Default|GetInteract2?)
          (bind _output_get_3 (Variables|Default|SetKnight2%20CurrentRotation (Variables|/Script/Engine.SceneComponent|GetRelativeRotation _knight2)))
          (Variables|Default|SetKnight2UpdatedRotation (Math|Rotator|CombineRotators _output_get_3 "0.000000,45.000000,0.000000"))
          (bind _knight2_rotation (Timeline|Knight2%20Rotation PlayFromStart)
            (:Update
              (Transformation|SetRelativeRotation _knight2 (Math|Rotator|Lerp(Rotator) (Variables|Default|GetKnight2%20CurrentRotation) (Variables|Default|GetKnight2UpdatedRotation) _knight2_rotation true) false false)
              (Utilities|FlowControl|Delay 1.1)
              (Variables|Default|SetActive? true)
              (if (== (.yaw (Variables|Default|GetKnight2UpdatedRotation)) (.yaw (Variables|Default|GetKnight2%20End%20Rotation)))
                (Variables|Default|SetKnight2Correct? true)
                (goto _label)
                (else
                  (Variables|Default|SetKnight2Correct? false)))))))
      (:then_3
        (if (Variables|Default|GetInteract3?)
          (bind _output_get_4 (Variables|Default|SetKnight3%20CurrentRotation (Variables|/Script/Engine.SceneComponent|GetRelativeRotation _knife3)))
          (Variables|Default|SetKnight3UpdatedRotation (Math|Rotator|CombineRotators _output_get_4 "0.000000,45.000000,0.000000"))
          (bind _knight3_rotation (Timeline|Knight3%20Rotation PlayFromStart)
            (:Update
              (Transformation|SetRelativeRotation _knife3 (Math|Rotator|Lerp(Rotator) (Variables|Default|GetKnight3%20CurrentRotation) (Variables|Default|GetKnight3UpdatedRotation) _knight3_rotation true) false false)
              (Utilities|FlowControl|Delay 1.1)
              (Variables|Default|SetActive? true)
              (if (== (.yaw (Variables|Default|GetKnight3UpdatedRotation)) (.yaw (Variables|Default|GetKnight3%20End%20Rotation)))
                (Variables|Default|SetKnight3Correct? true)
                (goto _label)
                (else
                  (Variables|Default|SetKnight3Correct? false))))))))))

(event Custom|Multicast
  (bind _returnvalue (Math|Random|RandomIntegerinRange 1 8))
  (bind _knight (Variables|Default|GetKnight))
  (bind _knight1 (Variables|Default|GetKnight1))
  (bind _knight2 (Variables|Default|GetKnight2))
  (bind _knight3 (Variables|Default|GetKnight3))
  (bind _relativerotation (Variables|/Script/Engine.SceneComponent|GetRelativeRotation _knight))
  (bind _relativerotation_2 (Variables|/Script/Engine.SceneComponent|GetRelativeRotation _knight1))
  (bind _relativerotation_3 (Variables|/Script/Engine.SceneComponent|GetRelativeRotation _knight2))
  (bind _relativerotation_4 (Variables|/Script/Engine.SceneComponent|GetRelativeRotation _knight3))
  ;[1 1 1] Knight Puzzle
  ;;[1 1 1] Hub Controls
  (Variables|Default|SetRotateValue _returnvalue)
  (Variables|Default|SetRotateValue1 _returnvalue)
  (Variables|Default|SetRotateValue2 _returnvalue)
  (Variables|Default|SetRotateValue3 _returnvalue)
  (Variables|Default|SetKnight%20End%20Rotation _relativerotation)
  (Variables|Default|SetRotateDegree (* (Variables|Default|GetRotateValue) 45))
  (Variables|Default|SetKnightCurrentRotation _relativerotation)
  (Variables|Default|SetKnight1%20End%20Rotation _relativerotation_2)
  (Variables|Default|SetRotateDegree1 (* (Variables|Default|GetRotateValue1) 45))
  (Variables|Default|SetKnight1%20CurrentRotation _relativerotation_2)
  (Variables|Default|SetKnight2%20End%20Rotation _relativerotation_3)
  (Variables|Default|SetRotateDegree2 (* (Variables|Default|GetRotateValue2) 45))
  (Variables|Default|SetKnight2%20CurrentRotation _relativerotation_3)
  (Variables|Default|SetKnight3%20End%20Rotation _relativerotation_4)
  (Variables|Default|SetRotateDegree3 (* (Variables|Default|GetRotateValue3) 45))
  (Variables|Default|SetKnight3%20CurrentRotation _relativerotation_4)
  (CallFunction|PuzzleSetup))

(event Custom|ServerSetup
  ;[1 1 1] Knight Puzzle
  ;;[1 1 1] Hub Controls
  (CallFunction|Multicast))

(event Custom|PuzzleSetup
  ;[1 1 1] Knight Puzzle
  ;;[0.1591 0.2279 1] Puzzle Setup
  (Utilities|FlowControl|Sequence
    (:then_0
      (Transformation|SetWorldRotation (Variables|Default|GetKnife) (Math|Rotator|MakeRotator 9e+01 0.0 (Variables|Default|GetRotateDegree)) false false)
      ;;[0.3631 1 0.9582] Correct On Setup?
      (Variables|Default|SetKnightCurrentRotation (Variables|/Script/Engine.SceneComponent|GetRelativeRotation (Variables|Default|GetKnife)))
      (if (== (.yaw (Variables|Default|GetKnightCurrentRotation)) (.yaw (Variables|Default|GetKnight%20End%20Rotation)))
        (Variables|Default|SetKnightCorrect? true)
        (else
          (Variables|Default|SetKnightCorrect? false))))
    (:then_1
      (Transformation|SetRelativeRotation (Variables|Default|GetKnight1) (Math|Rotator|MakeRotator 0.0 0.0 (Variables|Default|GetRotateDegree1)) false false)
      (Variables|Default|SetKnight1%20CurrentRotation (Variables|/Script/Engine.SceneComponent|GetRelativeRotation (Variables|Default|GetKnight1)))
      (if (== (.yaw (Variables|Default|GetKnight1%20CurrentRotation)) (.yaw (Variables|Default|GetKnight1%20End%20Rotation)))
        (Variables|Default|SetKnight1Correct? true)
        (else
          (Variables|Default|SetKnight1Correct? false))))
    (:then_2
      (Transformation|SetRelativeRotation (Variables|Default|GetKnight2) (Math|Rotator|MakeRotator 0.0 0.0 (Variables|Default|GetRotateDegree2)) false false)
      (Variables|Default|SetKnight2%20CurrentRotation (Variables|/Script/Engine.SceneComponent|GetRelativeRotation (Variables|Default|GetKnight2)))
      (if (== (.yaw (Variables|Default|GetKnight2%20CurrentRotation)) (.yaw (Variables|Default|GetKnight2%20End%20Rotation)))
        (Variables|Default|SetKnight2Correct? true)
        (else
          (Variables|Default|SetKnight2Correct? false))))
    (:then_3
      (Transformation|SetWorldRotation (Variables|Default|GetKnife3) (Math|Rotator|MakeRotator 9e+01 0.0 (Variables|Default|GetRotateDegree3)) false false)
      (Variables|Default|SetKnight3%20CurrentRotation (Variables|/Script/Engine.SceneComponent|GetRelativeRotation (Variables|Default|GetKnife3)))
      (if (== (.yaw (Variables|Default|GetKnight3%20CurrentRotation)) (.yaw (Variables|Default|GetKnight3%20End%20Rotation)))
        (Variables|Default|SetKnight3Correct? true)
        (else
          (Variables|Default|SetKnight3Correct? false))))))

(event EventBeginPlay
  ;[1 1 1] Knight Puzzle
  ;;[1 1 1] Hub Controls
  (Variables|Default|SetStart? true))

(event EventOnInteract
  (params (Actor :type Actor%20Object%20Reference))
  (bind _knife3 (Variables|Default|GetKnife3))
  (bind _knight1 (Variables|Default|GetKnight1))
  (bind _knight2 (Variables|Default|GetKnight2))
  (bind _knife (Variables|Default|GetKnife))
  ;[1 1 1] Knight Puzzle
  ;;[1 0.2098 0.172] Check Rotation
  (if (Variables|Default|GetActive?)
    (Variables|Default|SetActive? false)
    (Utilities|FlowControl|Sequence
      (:then_0
        (if (Variables|Default|GetInteract?)
          (bind _output_get (Variables|Default|SetKnightCurrentRotation (Variables|/Script/Engine.SceneComponent|GetRelativeRotation _knife)))
          (Variables|Default|SetKnightUpdatedRotation (Math|Rotator|CombineRotators _output_get "0.000000,45.000000,0.000000"))
          (bind _knight_rotation (Timeline|Knight%20Rotation PlayFromStart)
            (:Update
              (Transformation|SetRelativeRotation _knife (Math|Rotator|Lerp(Rotator) (Variables|Default|GetKnightCurrentRotation) (Variables|Default|GetKnightUpdatedRotation) _knight_rotation true) false false)
              (Utilities|FlowControl|Delay 1.1)
              (Variables|Default|SetActive? true)
              (if (== (.yaw (Variables|Default|GetKnightUpdatedRotation)) (.yaw (Variables|Default|GetKnight%20End%20Rotation)))
                (Variables|Default|SetKnightCorrect? true)
                ;;[0.3989 0.9101 1] Win Condition
                (if (or (Variables|Default|GetAllCorrect?) (Math|Boolean|ANDBoolean (Variables|Default|GetKnightCorrect?) (Variables|Default|GetKnight1Correct?) (Variables|Default|GetKnight2Correct?) (Variables|Default|GetKnight3Correct?))) :!label _label
                  (Variables|Default|SetAllCorrect? true)
                  (CallFunction|EndGame))
                (else
                  (Variables|Default|SetKnightCorrect? false)))))))
      (:then_1
        (if (Variables|Default|GetInteract1?)
          (bind _output_get_2 (Variables|Default|SetKnight1%20CurrentRotation (Variables|/Script/Engine.SceneComponent|GetRelativeRotation _knight1)))
          (Variables|Default|SetKnight1UpdatedRotation (Math|Rotator|CombineRotators _output_get_2 "0.000000,45.000000,0.000000"))
          (bind _knight1_rotation (Timeline|Knight1%20Rotation PlayFromStart)
            (:Update
              (Transformation|SetRelativeRotation _knight1 (Math|Rotator|Lerp(Rotator) (Variables|Default|GetKnight1%20CurrentRotation) (Variables|Default|GetKnight1UpdatedRotation) _knight1_rotation true) false false)
              (Utilities|FlowControl|Delay 1.1)
              (Variables|Default|SetActive? true)
              (if (== (.yaw (Variables|Default|GetKnight1UpdatedRotation)) (.yaw (Variables|Default|GetKnight1%20End%20Rotation)))
                (Variables|Default|SetKnight1Correct? true)
                (goto _label)
                (else
                  (Variables|Default|SetKnight1Correct? false)))))))
      (:then_2
        (if (Variables|Default|GetInteract2?)
          (bind _output_get_3 (Variables|Default|SetKnight2%20CurrentRotation (Variables|/Script/Engine.SceneComponent|GetRelativeRotation _knight2)))
          (Variables|Default|SetKnight2UpdatedRotation (Math|Rotator|CombineRotators _output_get_3 "0.000000,45.000000,0.000000"))
          (bind _knight2_rotation (Timeline|Knight2%20Rotation PlayFromStart)
            (:Update
              (Transformation|SetRelativeRotation _knight2 (Math|Rotator|Lerp(Rotator) (Variables|Default|GetKnight2%20CurrentRotation) (Variables|Default|GetKnight2UpdatedRotation) _knight2_rotation true) false false)
              (Utilities|FlowControl|Delay 1.1)
              (Variables|Default|SetActive? true)
              (if (== (.yaw (Variables|Default|GetKnight2UpdatedRotation)) (.yaw (Variables|Default|GetKnight2%20End%20Rotation)))
                (Variables|Default|SetKnight2Correct? true)
                (goto _label)
                (else
                  (Variables|Default|SetKnight2Correct? false)))))))
      (:then_3
        (if (Variables|Default|GetInteract3?)
          (bind _output_get_4 (Variables|Default|SetKnight3%20CurrentRotation (Variables|/Script/Engine.SceneComponent|GetRelativeRotation _knife3)))
          (Variables|Default|SetKnight3UpdatedRotation (Math|Rotator|CombineRotators _output_get_4 "0.000000,45.000000,0.000000"))
          (bind _knight3_rotation (Timeline|Knight3%20Rotation PlayFromStart)
            (:Update
              (Transformation|SetRelativeRotation _knife3 (Math|Rotator|Lerp(Rotator) (Variables|Default|GetKnight3%20CurrentRotation) (Variables|Default|GetKnight3UpdatedRotation) _knight3_rotation true) false false)
              (Utilities|FlowControl|Delay 1.1)
              (Variables|Default|SetActive? true)
              (if (== (.yaw (Variables|Default|GetKnight3UpdatedRotation)) (.yaw (Variables|Default|GetKnight3%20End%20Rotation)))
                (Variables|Default|SetKnight3Correct? true)
                (goto _label)
                (else
                  (Variables|Default|SetKnight3Correct? false))))))))))

(event EventBeginfromHUB
  ;[1 1 1] Knight Puzzle
  ;;[1 1 1] Hub Controls
  (if (Networking|IsServer)
    (CallFunction|ServerSetup)))

(fn ConstructionScript
  (|CallParentFunction))

(fn PlayerGate
  (params (OtherActor :type Actor%20Object%20Reference))
  (if (== (Utilities|GetClass OtherActor) "/Game/ThirdPerson/Blueprints/BP_ThirdPersonCharacter.BP_ThirdPersonCharacter_C")
    _))
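; BP_Dice is a physics die for the dice minigame that gets knocked around when it takes damage.
; AnyDamage pushes the Dice component away from the damage causer with an upward-biased impulse.
; It also applies a large torque along that direction rotated 90 degrees by RotateAVector, a helper that rotates in the XY plane and drops Z, so the die tumbles away from the hit.
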(event Game|Damage|EventAnyDamage
  (params (Damage :type Float%20%28single-precision%29) (DamageType :type Damage%20Type%20Object%20Reference) (InstigatedBy :type Controller%20Object%20Reference) (DamageCauser :type Actor%20Object%20Reference))
  (bind _returnvalue (Transformation|GetActorLocation DamageCauser))
  (bind _dice (Variables|Default|GetDice))
  (bind _returnvalue_2 (Transformation|GetWorldLocation _dice))
  (bind _returnvalue_3 (- _returnvalue_2 _returnvalue))
  (Physics|AddImpulse (Variables|Default|GetDice) (* (Math|Vector|Normalize (+ _returnvalue_3 "0.000000,0.000000,500.000000")) 1e+03) "None" false)
  (bind _outvector (CallFunction|RotateAVector (* (Math|Vector|Normalize _returnvalue_3) 5e+06) 9e+01))
  (Class|PrimitiveComponent|AddTorqueinRadians (Variables|Default|GetDice) _outvector "None" false))

(fn ConstructionScript)

(fn RotateAVector
  (params (Vector :type Vector) (Angle :type Float%20%28double-precision%29))
  (LocalVariables|SetInVector Vector)
  (LocalVariables|SetInAngle Angle)
  (LocalVariables|Seta (Math|Vector|MakeVector (Math|Trig|Cos(Degrees) (LocalVariables|GetInAngle)) (Math|Trig|Sin(Degrees) (LocalVariables|GetInAngle)) 0.0))
  (LocalVariables|Setb (Math|Vector|MakeVector (* (Math|Trig|Sin(Degrees) (LocalVariables|GetInAngle)) -1.0) (Math|Trig|Cos(Degrees) (LocalVariables|GetInAngle)) 0.0))
  (return (+ (* (LocalVariables|Geta) (.X (Math|Vector|BreakVector (LocalVariables|GetInVector)))) (* (LocalVariables|Getb) (.Y (Math|Vector|BreakVector (LocalVariables|GetInVector)))))))
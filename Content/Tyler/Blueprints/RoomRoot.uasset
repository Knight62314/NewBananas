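; Base room actor that child rooms extend with their own begin, end, timer-expiry and enemy-killed logic, reporting wins and losses to the HUB.
; An optional countdown picks its duration by counting player characters, then plays a rate-scaled timeline in reverse to update a timer widget.
; It also spawns melee enemies relative to the room, tracks them, and handles their removal or mass destruction.
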(event Custom|StopRoomTimer
  ;[1 1 1] Timer
  (Widget|RemovefromParent (Variables|RoomDetails|GetTimerWidget))
  (bind _timeleft (Timeline|Room%20Timer Stop)
    (:Update
      (Variables|/Script/UMG.TextBlock|SetText (Variables|/Game/Tyler/Blueprints/Widgets/TimerWidget.TimerWidget_C|GetTime (Variables|RoomDetails|GetTimerWidget)) (Utilities|Text|ToText(String) (Utilities|String|ToString(Integer) (Math|Float|Floor (* _timeleft (Utilities|Array|Get(acopy) (Variables|Timer|GetTimes) (Variables|Timer|GetTimerIndex))))))))
    (:Finished
      (Widget|RemovefromParent (Variables|RoomDetails|GetTimerWidget))
      (CallFunction|RoomTimerFinished))))

(event Custom|StartRoomTimerFromHUB
  ;[1 1 1] Timer
  (if (Variables|Timer|GetDoTimer?)
    (Variables|Timer|SetTimes (Utilities|Array|MakeArray (Variables|Timer|GetTimeFor1Player) (Variables|Timer|GetTimeFor2Players) (Variables|Timer|GetTimeFor3Players) (Variables|Timer|GetTimeFor4Players)))
    (bind _returnvalue (UserInterface|CreateWidget "/Game/Tyler/Blueprints/Widgets/TimerWidget.TimerWidget_C"))
    (bind _output_get (Variables|RoomDetails|SetTimerWidget _returnvalue))
    (UserInterface|Viewport|AddtoViewport _output_get 0)
    (bind _outactors (Actor|GetAllActorsOfClass "/Game/ThirdPerson/Blueprints/BP_ThirdPersonCharacter.BP_ThirdPersonCharacter_C"))
    (Variables|Timer|SetTimerIndex (- (Utilities|Array|Length _outactors) 1))
    (Components|Timeline|SetPlayRate (Variables|Default|GetRoom%20Timer) (Math|Float|SafeDivide 1.0 (Utilities|Array|Get(acopy) (Variables|Timer|GetTimes) (Variables|Timer|GetTimerIndex))))
    (bind _timeleft (Timeline|Room%20Timer ReverseFromEnd)
      (:Update
        (Variables|/Script/UMG.TextBlock|SetText (Variables|/Game/Tyler/Blueprints/Widgets/TimerWidget.TimerWidget_C|GetTime (Variables|RoomDetails|GetTimerWidget)) (Utilities|Text|ToText(String) (Utilities|String|ToString(Integer) (Math|Float|Floor (* _timeleft (Utilities|Array|Get(acopy) (Variables|Timer|GetTimes) (Variables|Timer|GetTimerIndex))))))))
      (:Finished
        (Widget|RemovefromParent (Variables|RoomDetails|GetTimerWidget))
        (CallFunction|RoomTimerFinished)))))

(event Custom|RemoveMeleeEnemy
  (params (Enemy :type Melee%20Enemy%20Character%20Object%20Reference))
  (Utilities|Array|RemoveItem (Variables|Default|GetMeleeEnemies) Enemy)
  (CallFunction|EnemyKilled))

(event Custom|EndFromHUB
  ;[1 1 1] Overriden by Children
)

(event Custom|RoomTimerFinished
  ;[1 1 1] Overriden by Children
)

(event Custom|RoomWon
  (Default|MovetoHUBFunction (Variables|RoomDetails|GetHUB) self)
  (CallFunction|StopRoomTimer))

(event Custom|RoomLost
  (Development|PrintString "Life UI")
  (Default|LoseLife (Variables|RoomDetails|GetHUB) self))

(event Custom|BeginFromHUB
  ;[1 1 1] Overriden by Children
)

(event Custom|EnemyKilled
  ;[1 1 1] Overriden by Children
)

(fn ConstructionScript)

(fn SpawnMeleeEnemy
  (params (Location :type Vector))
  (bind _self self)
  (bind _returnvalue (Game|SpawnActorfromClass "/Game/AI_Entities/Demo_Enemy/Melee_Enemy/Melee_Enemy_Character.Melee_Enemy_Character_C" (Math|Transform|MakeTransform (+ Location (Transformation|GetWorldLocation (Variables|Default|GetDefaultSceneRoot))) "0.000000,-90.000000,0.000000") "AdjustIfPossibleButAlwaysSpawn" "MultiplyWithRoot" 0 0))
  (Variables|/Game/AI_Entities/Demo_Enemy/Melee_Enemy/Melee_Enemy_Character.Melee_Enemy_Character_C|SetRoom _returnvalue _self)
  (Utilities|Array|Add (Variables|Default|GetMeleeEnemies) _returnvalue)
  (Development|PrintString (Utilities|GetObjectName _self) true true "(R=0.000000,G=0.660000,B=1.000000,A=1.000000)" 5.0)
  (if (Utilities|IsValid _returnvalue)
    (Development|PrintString "Good" true true "(R=0.000000,G=1.000000,B=0.000000,A=1.000000)")
    (else
      (Development|PrintString "Bad" true true "(R=1.000000,G=0.000000,B=0.000000,A=1.000000)"))))

(fn KillAllMeleeEnemies
  (for _array_element (Variables|Default|GetMeleeEnemies)
    (Actor|DestroyActor _array_element))
  (Utilities|Array|Clear (Variables|Default|GetMeleeEnemies)))
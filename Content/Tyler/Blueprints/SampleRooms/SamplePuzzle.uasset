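; SamplePuzzle is a sample puzzle room Blueprint that reports the room as lost when the player walks into its trigger box.
; BeginfromHUB prints the node the room was entered from and resets the Solved flag.
; The Box overlap checks for the exact BP_ThirdPersonCharacter class, then sets Solved and calls RoomLost, so it fires only once until the next reset.
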(event OnComponentBeginOverlap(Box)
  (params (OverlappedComponent :type Primitive%20Component%20Object%20Reference) (OtherActor :type Actor%20Object%20Reference) (OtherComp :type Primitive%20Component%20Object%20Reference) (OtherBodyIndex :type Integer) (bFromSweep :type Boolean) (SweepResult :type Hit%20Result%20Structure%20%28by%20ref%29))
  (if (and (== (Utilities|GetClass OtherActor) "/Game/ThirdPerson/Blueprints/BP_ThirdPersonCharacter.BP_ThirdPersonCharacter_C") (not (Variables|Default|GetSolved)))
    (Variables|Default|SetSolved true)
    (CallFunction|RoomLost)))

(event EventBeginfromHUB
  (Development|PrintString (Utilities|String|Append "Enter From Node: " (Utilities|String|ToString(Integer) (Variables|Default|GetEnterFromNode))) true true "(R=0.000000,G=0.660000,B=1.000000,A=1.000000)" 5.0)
  (Variables|Default|SetSolved false))

(fn ConstructionScript
  (|CallParentFunction))
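; BP_GDCMenu sets up the GDC lobby menu and character selection for one to four players.
; On BeginPlay it adds the lobby widget, then reads the game mode's player count and layers four character select widgets above it.
; Each active player owns and focuses their slot; empty slots fall to player 0, whose own slot is created last to keep focus.
; ReadyCheck focuses the lobby's start button once ReadyInt matches the player count.
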(event Custom|ReadyCheck
  (bind _asgdcmenu_game_mode (Utilities|Casting|CastToGDCMenu_GameMode (Game|GetGameMode)))
  (if (== (Variables|/Game/Steven/MainMenu/GDCMenu_GameMode.GDCMenu_GameMode_C|GetPlayerCount _asgdcmenu_game_mode) (Variables|Default|GetReadyInt))
    (Input|SetInputModeGameandUI (Game|GetPlayerController 0) (Variables|Default|GetLobby) "DoNotLock" true false)
    (Widget|SetFocus (Variables|/Game/Steven/MainMenu/WB_GDCLobby.WB_GDCLobby_C|GetStartGameBTN (Variables|Default|GetLobby)))))

(event EventBeginPlay
  (bind _returnvalue (UserInterface|CreateWidget "/Game/Steven/MainMenu/WB_GDCLobby.WB_GDCLobby_C" (Game|GetPlayerController 0)))
  (UserInterface|Viewport|AddtoViewport _returnvalue 0)
  (Variables|Default|SetLobby _returnvalue)
  (Utilities|FlowControl|DelayUntilNextTick)
  (bind _asgdcmenu_game_mode (Utilities|Casting|CastToGDCMenu_GameMode (Game|GetGameMode)))
  (switch int (Variables|/Game/Steven/MainMenu/GDCMenu_GameMode.GDCMenu_GameMode_C|GetPlayerCount _asgdcmenu_game_mode)
    (:1
      (CallFunction|CreateCharacterSelect "/Game/Steven/MainMenu/CharacterSelect4_GDC.CharacterSelect4_GDC_C")
      (CallFunction|CreateCharacterSelect "/Game/Steven/MainMenu/CharacterSelect2_GDC.CharacterSelect2_GDC_C")
      (CallFunction|CreateCharacterSelect "/Game/Steven/MainMenu/CharacterSelect3_GDC.CharacterSelect3_GDC_C")
      (CallFunction|CreateCharacterSelect "/Game/Steven/MainMenu/CharacterSelect1_GDC.CharacterSelect1_GDC_C"))
    (:2
      (CallFunction|CreateCharacterSelect "/Game/Steven/MainMenu/CharacterSelect2_GDC.CharacterSelect2_GDC_C" 1)
      (CallFunction|CreateCharacterSelect "/Game/Steven/MainMenu/CharacterSelect4_GDC.CharacterSelect4_GDC_C")
      (CallFunction|CreateCharacterSelect "/Game/Steven/MainMenu/CharacterSelect3_GDC.CharacterSelect3_GDC_C")
      (CallFunction|CreateCharacterSelect "/Game/Steven/MainMenu/CharacterSelect1_GDC.CharacterSelect1_GDC_C"))
    (:3
      (CallFunction|CreateCharacterSelect "/Game/Steven/MainMenu/CharacterSelect3_GDC.CharacterSelect3_GDC_C" 2)
      (CallFunction|CreateCharacterSelect "/Game/Steven/MainMenu/CharacterSelect2_GDC.CharacterSelect2_GDC_C" 1)
      (CallFunction|CreateCharacterSelect "/Game/Steven/MainMenu/CharacterSelect4_GDC.CharacterSelect4_GDC_C")
      (CallFunction|CreateCharacterSelect "/Game/Steven/MainMenu/CharacterSelect1_GDC.CharacterSelect1_GDC_C"))
    (:4
      (CallFunction|CreateCharacterSelect "/Game/Steven/MainMenu/CharacterSelect4_GDC.CharacterSelect4_GDC_C" 3)
      (CallFunction|CreateCharacterSelect "/Game/Steven/MainMenu/CharacterSelect3_GDC.CharacterSelect3_GDC_C" 2)
      (CallFunction|CreateCharacterSelect "/Game/Steven/MainMenu/CharacterSelect2_GDC.CharacterSelect2_GDC_C" 1)
      (CallFunction|CreateCharacterSelect "/Game/Steven/MainMenu/CharacterSelect1_GDC.CharacterSelect1_GDC_C"))))

(fn ConstructionScript)

(fn CreateCharacterSelect
  (params (WidgetClass :type User%20Widget%20Class%20Reference) (PlayerIndex :type Integer))
  (bind _returnvalue (Game|GetPlayerController PlayerIndex))
  (bind _returnvalue_2 (UserInterface|CreateWidget WidgetClass _returnvalue))
  (UserInterface|Viewport|AddtoViewport _returnvalue_2 1)
  (Input|SetInputModeGameandUI _returnvalue _returnvalue_2 "DoNotLock" true false))
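; Actor component on CharacterParent_BP that turns Attack, Special and Movement inputs into character abilities.
; Attack runs a four-step combo by AttackIndex, buffering presses made mid-attack for ComboAttack, or triggers a jump attack while falling.
; Special and Movement are gated by cooldown waits and flags, with Special firing the character's effect on a montage notify.
; The component manages ability state, while the owning character implements each move.
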(event Custom|ComboAttack
  (bind _as_character_parent_bp (Variables|Default|GetAs%20Character%20Parent%20BP))
  ;[0.05098 0.05098 0.05098] Attacking
  ;;[0.05098 0.05098 0.05098] Continue Combo
  (if (Variables|Default|GetSaveAttack?)
    (Variables|Default|SetSaveAttack? false)
    ;;[0.05098 0.05098 0.05098] Select Attack
    (switch int (Variables|Default|GetAttackIndex)
      (:0
        (Default|Attack1 _as_character_parent_bp))
      (:1
        (Default|Attack2 _as_character_parent_bp))
      (:2
        (Default|Attack3 _as_character_parent_bp))
      (:3
        (Default|Attack4 _as_character_parent_bp)))))

(event Custom|StopCombo
  ;[0.05098 0.05098 0.05098] Attacking
  ;;[0.05098 0.05098 0.05098] End Combo
  (Variables|Default|SetIsAttacking? false)
  (Variables|Default|SetAttackIndex 0))

(event Custom|Special
  ;[0.05098 0.05098 0.05098] Special Item
  ;;[0.05098 0.05098 0.05098] Special Animation
  (Variables|Default|SetCanSpecial? false)
  (Animation|Montage|PlayMontage (Variables|/Script/Engine.Character|GetMesh (Variables|Default|GetAs%20Character%20Parent%20BP)) "/Game/Nate/BaseAniamtions/BaseBodyAnims/Combat/Base_PowerUp1_L_Montage.Base_PowerUp1_L_Montage"
    (:OnCompleted
      (Variables|Default|SetCanAttack? true)
      (Variables|Default|SetCanMovement? true))
    (:OnNotifyBegin
      (Default|Special (Variables|Default|GetAs%20Character%20Parent%20BP)))))

(event Custom|JumpAttack
  ;[0.05098 0.05098 0.05098] Attacking
  ;;[0.05098 0.05098 0.05098] Jump Attack
  (if (not (Variables|Default|GetIsAttacking?))
    (Variables|Default|SetIsAttacking? true)
    (Default|JumpAttack (Variables|Default|GetAs%20Character%20Parent%20BP))))

(event Custom|FirstAttack
  (bind _as_character_parent_bp (Variables|Default|GetAs%20Character%20Parent%20BP))
  ;[0.05098 0.05098 0.05098] Attacking
  ;;[0.05098 0.05098 0.05098] First Attack
  (if (Variables|Default|GetIsAttacking?)
    (Variables|Default|SetSaveAttack? true)
    (else
      (Variables|Default|SetIsAttacking? true)
      ;;[0.05098 0.05098 0.05098] Select Attack
      (switch int (Variables|Default|GetAttackIndex)
        (:0
          (Default|Attack1 _as_character_parent_bp))
        (:1
          (Default|Attack2 _as_character_parent_bp))
        (:2
          (Default|Attack3 _as_character_parent_bp))
        (:3
          (Default|Attack4 _as_character_parent_bp))))))

(event EventBeginPlay
  (bind _ascharacter_parent_bp (Utilities|Casting|CastToCharacterParent_BP (Components|GetOwner)))
  (Variables|Default|SetAs%20Character%20Parent%20BP _ascharacter_parent_bp))

(event Input|ActionEvents|InputActionAttack
  (params (Key :type Key%20Structure :default "None"))
  ;[0.05098 0.05098 0.05098] Attacking
  ;;[0.05098 0.05098 0.05098] Start Attack
  (:Pressed
    (if (Variables|Default|GetCanAttack?)
      (if (AI|Components|NavMovement|IsFalling (Variables|/Script/Engine.Character|GetCharacterMovement (Variables|Default|GetAs%20Character%20Parent%20BP)))
        (CallFunction|JumpAttack)
        (else
          (CallFunction|FirstAttack))))))

(event Input|ActionEvents|InputActionMovement
  (params (Key :type Key%20Structure :default "None"))
  ;[0.05098 0.05098 0.05098] Movement Ability
  (:Pressed
    (if (Math|Boolean|ANDBoolean (== (Variables|/Game/ThirdPerson/Blueprints/CharacterParent_BP.CharacterParent_BP_C|GetMovementWait (Variables|Default|GetAs%20Character%20Parent%20BP)) 0.0) (Variables|Default|GetCanMovement?) (not (Variables|Default|GetIsAttacking?)))
      (Variables|Default|SetCanMovement? false)
      (Variables|Default|SetCanSpecial? false)
      (Default|Movement (Variables|Default|GetAs%20Character%20Parent%20BP)))))

(event Input|ActionEvents|InputActionSpecial
  (params (Key :type Key%20Structure :default "None"))
  ;[0.05098 0.05098 0.05098] Special Item
  ;;[0.05098 0.05098 0.05098] Special Input
  (:Pressed
    (if (and (== (Variables|/Game/ThirdPerson/Blueprints/CharacterParent_BP.CharacterParent_BP_C|GetItemWait (Variables|Default|GetAs%20Character%20Parent%20BP)) 0.0) (Variables|Default|GetCanSpecial?))
      (Variables|Default|SetCanAttack? false)
      (Variables|Default|SetCanMovement? false)
      (CallFunction|StopCombo)
      (CallFunction|Special))))
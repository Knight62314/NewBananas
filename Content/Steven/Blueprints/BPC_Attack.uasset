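; Attack component for CharacterParent_BP characters that gates the Special and Movement ability inputs.
; It caches the owning character on BeginPlay and checks that character's wait values plus local state flags before either ability runs.
; Special locks attack and movement, plays a power-up montage, then re-enables both on completion, leaving CanSpecial off.
; Movement is a stub that only clears the movement and special flags.
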(event Custom|Special
  ;[0.05098 0.05098 0.05098] Special Item
  ;;[0.05098 0.05098 0.05098] Special Animation
  (Variables|Default|SetCanSpecial? false)
  (Animation|Montage|PlayMontage (Variables|/Script/Engine.Character|GetMesh (Variables|Default|GetAs%20Character%20Parent%20BP)) "/Game/Nate/BaseAniamtions/BaseBodyAnims/Combat/Base_PowerUp1_L_Montage.Base_PowerUp1_L_Montage"
    (:OnCompleted
      (Variables|Default|SetCanAttack? true)
      (Variables|Default|SetCanMovement? true))))

(event EventBeginPlay
  (bind _ascharacter_parent_bp (Utilities|Casting|CastToCharacterParent_BP (Components|GetOwner)))
  (Variables|Default|SetAs%20Character%20Parent%20BP _ascharacter_parent_bp))

(event Input|ActionEvents|InputActionMovement
  (params (Key :type Key%20Structure :default "None"))
  ;[0.05098 0.05098 0.05098] Movement Ability
  (:Pressed
    (if (Math|Boolean|ANDBoolean (== (Variables|/Game/ThirdPerson/Blueprints/CharacterParent_BP.CharacterParent_BP_C|GetMovementWait (Variables|Default|GetAs%20Character%20Parent%20BP)) 0.0) (Variables|Default|GetCanMovement?) (not (Variables|Default|GetIsAttacking?)))
      (Variables|Default|SetCanMovement? false)
      (Variables|Default|SetCanSpecial? false))))

(event Input|ActionEvents|InputActionSpecial
  (params (Key :type Key%20Structure :default "None"))
  ;[0.05098 0.05098 0.05098] Special Item
  ;;[0.05098 0.05098 0.05098] Special Input
  (:Pressed
    (if (and (== (Variables|/Game/ThirdPerson/Blueprints/CharacterParent_BP.CharacterParent_BP_C|GetSpecialWait (Variables|Default|GetAs%20Character%20Parent%20BP)) 0.0) (Variables|Default|GetCanSpecial?))
      (Variables|Default|SetCanAttack? false)
      (Variables|Default|SetCanMovement? false)
      (CallFunction|Special))))
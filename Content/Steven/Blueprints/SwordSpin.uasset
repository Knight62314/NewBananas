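; SwordSpin is a Blueprint that deals damage to actors overlapping its hit boxes, apparently for a spinning sword attack.
; Four box components share the same overlap logic, each applying a small fixed damage to any actor not tagged "Tar".
; Damage is credited to the parent actor as causer, so it is built to work as a child actor.
; The graph contains no movement or spin logic.
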(event OnComponentBeginOverlap(Box)
  (params (OverlappedComponent :type Primitive%20Component%20Object%20Reference) (OtherActor :type Actor%20Object%20Reference) (OtherComp :type Primitive%20Component%20Object%20Reference) (OtherBodyIndex :type Integer) (bFromSweep :type Boolean) (SweepResult :type Hit%20Result%20Structure%20%28by%20ref%29))
  (if (not (Actor|ActorHasTag OtherActor "Tar"))
    (Game|Damage|ApplyDamage OtherActor 1.0 0 (Actor|GetParentActor))))

(event OnComponentBeginOverlap(Box1)
  (params (OverlappedComponent :type Primitive%20Component%20Object%20Reference) (OtherActor :type Actor%20Object%20Reference) (OtherComp :type Primitive%20Component%20Object%20Reference) (OtherBodyIndex :type Integer) (bFromSweep :type Boolean) (SweepResult :type Hit%20Result%20Structure%20%28by%20ref%29))
  (if (not (Actor|ActorHasTag OtherActor "Tar"))
    (Game|Damage|ApplyDamage OtherActor 1.0 0 (Actor|GetParentActor))))

(event OnComponentBeginOverlap(Box2)
  (params (OverlappedComponent :type Primitive%20Component%20Object%20Reference) (OtherActor :type Actor%20Object%20Reference) (OtherComp :type Primitive%20Component%20Object%20Reference) (OtherBodyIndex :type Integer) (bFromSweep :type Boolean) (SweepResult :type Hit%20Result%20Structure%20%28by%20ref%29))
  (if (not (Actor|ActorHasTag OtherActor "Tar"))
    (Game|Damage|ApplyDamage OtherActor 1.0 0 (Actor|GetParentActor))))

(event OnComponentBeginOverlap(Box3)
  (params (OverlappedComponent :type Primitive%20Component%20Object%20Reference) (OtherActor :type Actor%20Object%20Reference) (OtherComp :type Primitive%20Component%20Object%20Reference) (OtherBodyIndex :type Integer) (bFromSweep :type Boolean) (SweepResult :type Hit%20Result%20Structure%20%28by%20ref%29))
  (if (not (Actor|ActorHasTag OtherActor "Tar"))
    (Game|Damage|ApplyDamage OtherActor 1.0 0 (Actor|GetParentActor))))

(event EventBeginPlay)

(event EventTick
  (params (DeltaSeconds :type Float%20%28single-precision%29)))

(fn ConstructionScript)
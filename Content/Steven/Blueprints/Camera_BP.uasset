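; Camera rig actor that tracks the player character, apparently for the side-scroller's camera.
; Each tick it moves its Arrow component to a relative position built from the player's location, with X and Y swapped and one negated.
; It then sets the actor's yaw to the look-at direction from the Arrow to the player.
; Unconnected leftovers would attach characters' side-view cameras to the Arrow and print its rotation.
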(event EventBeginPlay)

(event EventTick
  (params (DeltaSeconds :type Float%20%28single-precision%29))
  (bind _returnvalue (Game|GetPlayerCharacter 0))
  (bind _returnvalue_2 (Transformation|GetActorLocation _returnvalue))
  (Utilities|FlowControl|Sequence
    (:then_0
      (Components|MoveComponentTo (Variables|Default|GetArrow) (Math|Vector|MakeVector (* (.y _returnvalue_2) -1.0) (.x _returnvalue_2) (.z _returnvalue_2)) "0, 0, 0" false false 0.2 false))
    (:then_1
      (Transformation|SetActorRotation (Math|Rotator|MakeRotator 0.0 0.0 (.yaw (Math|Rotator|FindLookatRotation (Transformation|GetWorldLocation (Variables|Default|GetArrow)) (Transformation|GetActorLocation (Game|GetPlayerCharacter 0)))))))))

(fn ConstructionScript)
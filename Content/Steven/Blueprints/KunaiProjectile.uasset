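; Kunai projectile that reacts to box overlaps on behalf of its owning CharacterParent_BP, then bounces off and destroys itself.
; Players other than the owner are launched along X based on the owner's facing, alongside a negligible Damage_Light hit.
; A non-player overlap triggers the owner's MeleeHit at the kunai, once only.
; Bounce disables collision and uses a timeline to lerp the kunai away while spinning before destruction.
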(event OnComponentBeginOverlap(Box)
  (params (OverlappedComponent :type Primitive%20Component%20Object%20Reference) (OtherActor :type Actor%20Object%20Reference) (OtherComp :type Primitive%20Component%20Object%20Reference) (OtherBodyIndex :type Integer) (bFromSweep :type Boolean) (SweepResult :type Hit%20Result%20Structure%20%28by%20ref%29))
  (bind _as_character_parent_bp (Variables|Default|GetAs%20Character%20Parent%20BP))
  (if (.Bool (Utilities|IsActorPlayer OtherActor))
    (bind _players (CallFunction|GetAllPlayers))
    (for _array_element _players
      (if (not (== _array_element (Components|GetOwner)))
        (if (== _array_element OtherActor)
          (bind _newparam (Default|FacingRight? _as_character_parent_bp (Variables|/Game/ThirdPerson/Blueprints/CharacterParent_BP.CharacterParent_BP_C|GetCursorRotation _as_character_parent_bp)))
          (if _newparam
            (Character|LaunchCharacter _array_element "-1000.000000,0.000000,0.000000" false false)
            (else
              (Character|LaunchCharacter _array_element "1000.000000,0.000000,0.000000" false false)))
          (Game|Damage|ApplyDamage 0 1e-06 0 (Components|GetOwner) "/Game/Steven/Blueprints/Damage_Light.Damage_Light_C")
          (CallFunction|Bounce))))
    (else
      (Utilities|FlowControl|DoOnce false
        (:Completed
          (Default|MeleeHit (Variables|Default|GetAs%20Character%20Parent%20BP) 0.0 9e+01 4e+01 (Variables|Default|GetKunai))
          (CallFunction|Bounce))))))

(event Custom|Bounce
  (bind _kunai (Variables|Default|GetKunai))
  (bind _kunai_2 (Variables|Default|GetKunai))
  (bind _kunai_3 (Variables|Default|GetKunai))
  (bind _returnvalue (Transformation|GetWorldRotation _kunai))
  (bind _returnvalue_2 (Transformation|GetWorldRotation _kunai_2))
  (Collision|SetCollisionEnabled (Variables|Default|GetBox) "NoCollision")
  (bind _output_get (Variables|Default|SetStartLocation (Transformation|GetWorldLocation (Variables|Default|GetKunai))))
  (Variables|Default|SetEndLocation (+ _output_get (* (Math|Vector|Normalize (+ (Math|Vector|GetUpVector _returnvalue) (Math|Vector|GetRightVector _returnvalue))) 2e+02)))
  (Variables|Default|SetStartRotation (Transformation|GetWorldRotation _kunai_2))
  (Variables|Default|SetEndRotation (Math|Rotator|MakeRotator (+ (.roll _returnvalue_2) 7.2e+02) (.pitch _returnvalue_2) (.yaw _returnvalue_2)))
  (bind _newtrack_0 (Timeline|KunaiBounce PlayFromStart)
    (:Update
      (Transformation|SetWorldLocation _kunai_3 (Math|Vector|Lerp(Vector) (Variables|Default|GetStartLocation) (Variables|Default|GetEndLocation) _newtrack_0) false false)
      (Transformation|SetWorldRotation _kunai_3 (Math|Rotator|Lerp(Rotator) (Variables|Default|GetStartRotation) (Variables|Default|GetEndRotation) _newtrack_0) false false))
    (:Finished
      (Actor|DestroyActor))))

(event EventBeginPlay
  (bind _ascharacter_parent_bp (Utilities|Casting|CastToCharacterParent_BP (Components|GetOwner)))
  (Variables|Default|SetAs%20Character%20Parent%20BP _ascharacter_parent_bp))

(fn ConstructionScript)
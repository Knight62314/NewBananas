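; TestCube is a damageable test cube actor that also damages whatever it collides with.
; AnyDamage forwards to ReportDamage, which subtracts from Health and either briefly flashes the cube red through a timed material swap or destroys the actor once Health runs out.
; The Cube component's hit event applies a small fixed damage to the other actor.
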(event OnComponentHit(Cube)
  (params (HitComponent :type Primitive%20Component%20Object%20Reference) (OtherActor :type Actor%20Object%20Reference) (OtherComp :type Primitive%20Component%20Object%20Reference) (NormalImpulse :type Vector :default "0, 0, 0") (Hit :type Hit%20Result%20Structure%20%28by%20ref%29))
  (Game|Damage|ApplyDamage OtherActor 1.0 0 0))

(event Custom|ReportDamage
  (params (Damage :type Float%20%28double-precision%29))
  (bind _cube (Variables|Default|GetCube))
  (bind _output_get (Variables|Default|SetHealth (- (Variables|Default|GetHealth) Damage)))
  (if (> _output_get 0.0)
    (Rendering|Material|SetMaterial _cube 0 "/AnimationSharing/AnimSharingRed.AnimSharingRed")
    (Utilities|FlowControl|Delay 0.2)
    (Rendering|Material|SetMaterial _cube 0 "/Engine/BasicShapes/BasicShapeMaterial.BasicShapeMaterial")
    (else
      (Actor|DestroyActor))))

(event EventBeginPlay)

(event Collision|EventActorBeginOverlap
  (params (OtherActor :type Actor%20Object%20Reference)))

(event EventTick
  (params (DeltaSeconds :type Float%20%28single-precision%29)))

(event Game|Damage|EventAnyDamage
  (params (Damage :type Float%20%28single-precision%29) (DamageType :type Damage%20Type%20Object%20Reference) (InstigatedBy :type Controller%20Object%20Reference) (DamageCauser :type Actor%20Object%20Reference))
  (CallFunction|ReportDamage Damage))

(fn ConstructionScript)
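; BP_AISpawner is a spawner actor that creates a batch of NOE melee enemy characters when play begins.
; A DoN node looped back on itself spawns each Melee_Enemy_Character, starting at the Billboard's location and stepping diagonally in X and Y.
; The self-destroy and debug print sit behind a counter check that stays true within the DoN limit, so they appear unreachable for positive counts.
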(event EventBeginPlay
  (Variables|Default|SetSpawnLoc (Transformation|GetWorldLocation (Variables|Default|GetBillboard)))
  (bind _counter (Utilities|FlowControl|DoN (Variables|Default|GetNOE) :!label _label)
    (:Exit
      (Game|SpawnActorfromClass "/Game/AI_Entities/Demo_Enemy/Melee_Enemy/Melee_Enemy_Character.Melee_Enemy_Character_C" (Math|Transform|MakeTransform (Variables|Default|GetSpawnLoc) "0.000000,-90.000000,0.000000" "1.000000,1.000000,1.000000") "Undefined" "MultiplyWithRoot" 0 0)
      (Variables|Default|SetSpawnLoc (+ (Variables|Default|GetSpawnLoc) "100.000000,100.000000,0.000000"))
      (if (<= _counter (Variables|Default|GetNOE))
        (goto _label)
        (else
          (Actor|DestroyActor)
          (Development|PrintString "Hello"))))))

(fn ConstructionScript)
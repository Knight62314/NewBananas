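; BP_HordeAISpawner spawns a horde of melee enemy characters when play begins, starting at the location of its Billboard component.
; A DoN node wired back into itself acts as a loop, spawning up to NOE enemies.
; Each spawn ignores collision, is inserted at the front of MeleeArray, and shifts the next spawn point diagonally along X and Y.
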(event EventBeginPlay
  (Variables|Default|SetSpawnLoc (Transformation|GetWorldLocation (Variables|Default|GetBillboard)))
  (bind _counter (Utilities|FlowControl|DoN (Variables|Default|GetNOE) :!label _label)
    (:Exit
      (bind _returnvalue (Game|SpawnActorfromClass "/Game/AI_Entities/Demo_Enemy/Melee_Enemy/Melee_Enemy_Character.Melee_Enemy_Character_C" (Math|Transform|MakeTransform (Variables|Default|GetSpawnLoc) "0.000000,-90.000000,0.000000" "1.000000,1.000000,1.000000") "AlwaysSpawn" "MultiplyWithRoot" 0 0))
      (bind _output_get (Variables|Default|SetEnemy _returnvalue))
      (Utilities|Array|Insert (Variables|Default|GetMeleeArray) _output_get)
      (Variables|Default|SetSpawnLoc (+ (Variables|Default|GetSpawnLoc) "100.000000,100.000000,0.000000"))
      (if (<= _counter (Variables|Default|GetNOE))
        (goto _label)))))

(fn ConstructionScript)
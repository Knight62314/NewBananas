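; BP_AOE_Effect is a lingering enemy area effect that deals light damage to an actor tagged "Tar" entering its collision.
; Overlap replaces the affected list with that actor, runs ApplyAOE immediately and via a non-looping timer, then destroys the effect after a delay.
; End overlap removes the actor and clears the timer, while BeginPlay sets a lifespan.
; The looping ApplyDamge timer is unwired, and DestroyAOE is empty.
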(event OnComponentBeginOverlap(AOE_Collision)
  (params (OverlappedComponent :type Primitive%20Component%20Object%20Reference) (OtherActor :type Actor%20Object%20Reference) (OtherComp :type Primitive%20Component%20Object%20Reference) (OtherBodyIndex :type Integer) (bFromSweep :type Boolean) (SweepResult :type Hit%20Result%20Structure%20%28by%20ref%29))
  (if (Actor|ActorHasTag OtherActor "Tar")
    (Variables|Default|SetAffectedActors (Utilities|Array|MakeArray OtherActor))
    (CallFunction|ApplyAOE)
    (Utilities|Time|SetTimerbyFunctionName 0 "ApplyAOE" (Variables|Default|GetDamageInterval))
    (Development|PrintString "Hello")
    (Utilities|FlowControl|Delay 5.0)
    (Development|PrintString "AOE")
    (Actor|DestroyActor)))

(event OnComponentEndOverlap(AOE_Collision)
  (params (OverlappedComponent :type Primitive%20Component%20Object%20Reference) (OtherActor :type Actor%20Object%20Reference) (OtherComp :type Primitive%20Component%20Object%20Reference) (OtherBodyIndex :type Integer))
  (if (Actor|ActorHasTag OtherActor "Tar")
    (Utilities|Array|RemoveItem (Variables|Default|GetAffectedActors) OtherActor)
    (Utilities|Time|ClearTimerbyFunctionName 0 "ApplyAOE")
    (Development|PrintString "End")))

(event Custom|Apply%20Damge
  (for _array_element (Variables|Default|GetAffectedActors)
    (Game|Damage|ApplyDamage _array_element (Variables|Default|GetDamgePerTick) 0 0 "/Game/Steven/Blueprints/Damage_Light.Damage_Light_C")
    (Development|PrintString "N")))

(event EventBeginPlay
  (Actor|SetLifeSpan (Variables|Default|GetLingerDuration)))

(event EventTick
  (params (DeltaSeconds :type Float%20%28single-precision%29)))

(fn ConstructionScript)

(fn ApplyAOE
  (for _array_element (Variables|Default|GetAffectedActors)
    (Game|Damage|ApplyDamage _array_element (Variables|Default|GetDamgePerTick) 0 0 "/Game/Steven/Blueprints/Damage_Light.Damage_Light_C")
    (Development|PrintString "T")))

(fn DestroyAOE)
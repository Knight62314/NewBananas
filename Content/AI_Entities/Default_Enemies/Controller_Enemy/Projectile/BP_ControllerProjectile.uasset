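; Projectile for the Controller enemy that deals light damage and leaves an area-of-effect actor where it explodes.
; A looping timer explodes it once it travels its maximum distance from spawn.
; Overlapping anything except the Controller runs a short sphere trace toward that actor, ignoring Enemy and Room tags, damages the hit, then attaches, stops and explodes.
; Explosion spawns BP_AOE_Effect at a fixed near-zero height and destroys the projectile.
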(event OnComponentBeginOverlap(Box)
  (params (OverlappedComponent :type Primitive%20Component%20Object%20Reference) (OtherActor :type Actor%20Object%20Reference) (OtherComp :type Primitive%20Component%20Object%20Reference) (OtherBodyIndex :type Integer) (bFromSweep :type Boolean) (SweepResult :type Hit%20Result%20Structure%20%28by%20ref%29))
  (bind _returnvalue (Transformation|GetActorLocation))
  (bind _returnvalue_2 (Transformation|GetActorLocation OtherActor))
  (bind _returnvalue_3 (Math|Rotator|FindLookatRotation _returnvalue _returnvalue_2))
  (if (not (== "/Game/AI_Entities/Default_Enemies/Controller_Enemy/Enemy_Controller_Character.Enemy_Controller_Character_C" (Utilities|GetClass OtherActor)))
    (bind _outactors (Actor|GetAllActorswithTag "Enemy"))
    (bind _outactors_2 (Actor|GetAllActorswithTag "Room"))
    (Utilities|Array|AppendArray _outactors _outactors_2)
    (bind _outhit (Collision|SphereTraceByChannel _returnvalue (+ _returnvalue (* (Math|Vector|MakeVector (Math|Trig|Cos(Degrees) (.yaw _returnvalue_3)) (Math|Trig|Sin(Degrees) (.yaw _returnvalue_3)) 0.0) 25.0)) 9e+01 "TraceTypeQuery2" false _outactors "None"))
    (Game|Damage|ApplyDamage (.HitActor (Collision|BreakHitResult _outhit)) 2.0 0 self "/Game/Steven/Blueprints/Damage_Light.Damage_Light_C")
    (Transformation|AttachActorToActor OtherActor "None" "KeepWorld" "KeepWorld" "KeepWorld" true)
    (Components|Movement|StopMovementImmediately (Variables|Default|GetProjectileMovement))
    (CallFunction|ProjectileExplosion)
    (Utilities|FlowControl|Delay 0.2)
    (Actor|DestroyActor)))

(event EventBeginPlay
  (Variables|Default|SetStartLocation (Transformation|GetActorLocation))
  (Utilities|Time|SetTimerbyFunctionName 0 "CheckDistanceTraveled" 0.1 true))

(event Collision|EventActorBeginOverlap
  (params (OtherActor :type Actor%20Object%20Reference)))

(event EventTick
  (params (DeltaSeconds :type Float%20%28single-precision%29)))

(fn ConstructionScript)

(fn CheckDistanceTraveled
  (Variables|Default|SetDistanceTraveled (Math|Vector|VectorLength (- (Transformation|GetActorLocation) (Variables|Default|GetStartLocation))))
  (if (>= (Variables|Default|GetDistanceTraveled) (Variables|Default|GetMaxDistance))
    (CallFunction|ProjectileExplosion)
    (Utilities|Time|ClearTimerbyFunctionName 0 "CheckDistanceTraveled")))

(fn ProjectileExplosion
  (bind _returnvalue (Transformation|GetActorTransform))
  (Game|SpawnActorfromClass "/Game/AI_Entities/Default_Enemies/Controller_Enemy/Projectile/BP_AOE_Effect.BP_AOE_Effect_C" (Math|Transform|MakeTransform (Math|Vector|MakeVector (.x (.location _returnvalue)) (.y (.location _returnvalue)) 0.2) "0, 0, 0" (.scale _returnvalue)) "Undefined" "MultiplyWithRoot" 0 0)
  (Actor|DestroyActor))
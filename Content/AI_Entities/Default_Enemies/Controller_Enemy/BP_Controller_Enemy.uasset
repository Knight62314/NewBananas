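; Melee enemy character that spawns as a random Fox, Frog, Owl or Turtle, set up in the construction script with matching head, materials and eye tuning.
; Tick drives an eye morph target toward the attack target.
; AI-triggered Attack plays a left/right slash montage by yaw, sphere-tracing on its notify to apply light damage.
; Non-lethal hits flash the material and play directional reactions by damage type; lethal hits do nothing, as removal logic is unconnected.
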(event Custom|PickEnemyCharacter
  (bind _head (Variables|Default|GetHead))
  (bind _head_2 (Variables|Default|GetHead))
  (Components|SkeletalMesh|SetSkeletalMeshAsset _head (Utilities|Array|Get(acopy) (Variables|Default|GetCharacterHead) (Math|Conversions|ToInteger(Byte) (Variables|Default|GetEnemyCharacter))))
  (Rendering|Material|SetMaterial _head 0 (Utilities|Array|Get(acopy) (Variables|Default|GetCharacterMaterial) (Math|Conversions|ToInteger(Byte) (Variables|Default|GetEnemyCharacter))))
  (Rendering|Material|SetMaterial (Variables|Character|GetMesh) 0 (Utilities|Array|Get(acopy) (Variables|Default|GetCharacterMaterial) (Math|Conversions|ToInteger(Byte) (Variables|Default|GetEnemyCharacter))))
  (switch Utilities|FlowControl|Switch|SwitchonCharacter_State (Variables|Default|GetEnemyCharacter)
    (:NewEnumerator0
      (Variables|Default|SetEyeRotation 1.0)
      (Variables|Default|SetColor (Math|Color|MakeColor 0 20 100 255)))
    (:NewEnumerator1
      (Variables|Default|SetEyeRotation -1.0)
      (Variables|Default|SetCenterEyeFrog 0.5)
      (Variables|Default|SetColor (Math|Color|MakeColor 10 50 10 255)))
    (:NewEnumerator2
      (Variables|Default|SetEyeRotation -1.0)
      (Variables|Default|SetCenterEyeFrog 0.5)
      (Variables|Default|SetColor (Math|Color|MakeColor 0 10 20 255))
      (Rendering|Material|SetMaterial _head_2 0 "/Game/Nate/Animals/Frog/Frog_V1/Black_Eyes.Black_Eyes")
      (Rendering|Material|SetMaterial _head_2 1 "/Game/Nate/Character_Materials/Owl_Skin_BW.Owl_Skin_BW"))
    (:NewEnumerator3
      (Variables|Default|SetEyeRotation -0.5)
      (Variables|Default|SetCenterEyeFrog 0.5)
      (Variables|Default|SetColor (Math|Color|MakeColor 30 60 5 255))
      (Rendering|Material|SetMaterial (Variables|Default|GetHead) 1 "/Game/Nate/Animals/Frog/Frog_V1/Black_Eyes.Black_Eyes"))))

(event Custom|Attack
  (bind _returnvalue (Transformation|GetActorLocation))
  (bind _mesh (Variables|Character|GetMesh))
  ;[1 1 1] From AI BlackBoard
  (Variables|Default|SetTargetLcoation (Transformation|GetActorLocation (Variables|Default|GetAttack%20Target)))
  (Variables|Default|SetSlashing? true)
  (if (or (> (.yaw (Math|Rotator|FindLookatRotation (Transformation|GetActorLocation) (Variables|Default|GetTargetLcoation))) 9e+01) (< (.yaw (Math|Rotator|FindLookatRotation (Transformation|GetActorLocation) (Variables|Default|GetTargetLcoation))) -9e+01))
    (Animation|Montage|PlayMontage _mesh "/Game/Nate/BaseAniamtions/BaseBodyAnims/Combat/Fox_Slash_L_Montage.Fox_Slash_L_Montage"
      (:then
        (Utilities|FlowControl|Delay 0.4 :!label _label)
        (Variables|Default|SetSlashing? false))
      (:OnNotifyBegin
        (bind _outactors (Actor|GetAllActorsOfClass "/Game/AI_Entities/Default_Enemies/Grunt_Enemy/Melee_Enemy_Character.Melee_Enemy_Character_C" :!label _label_2))
        (bind _outhit (Collision|SphereTraceByChannel _returnvalue (+ _returnvalue (* (Math|Vector|MakeVector (Math|Trig|Cos(Degrees) (.yaw (Math|Rotator|FindLookatRotation (Transformation|GetActorLocation) (Variables|Default|GetTargetLcoation)))) (Math|Trig|Sin(Degrees) (.yaw (Math|Rotator|FindLookatRotation (Transformation|GetActorLocation) (Variables|Default|GetTargetLcoation)))) 0.0) 2.5e+02)) 9e+01 "TraceTypeQuery1" false _outactors "None"))
        (Game|Damage|ApplyDamage (.HitActor (Collision|BreakHitResult _outhit)) 1.0 0 self "/Game/Steven/Damage_Light.Damage_Light_C")))
    (else
      (Animation|Montage|PlayMontage _mesh "/Game/Nate/BaseAniamtions/BaseBodyAnims/Combat/Fox_Slash_R_Montage.Fox_Slash_R_Montage"
        (:then
          (goto _label))
        (:OnNotifyBegin
          (goto _label_2))))))

(event Custom|Teleport
  (params (Location :type Vector)))

(event EventTick
  (params (DeltaSeconds :type Float%20%28single-precision%29))
  ;[1 1 1] Attack Target Animations
  (Utilities|IsValid (Variables|Default|GetAttack%20Target)
    (:Is%20Valid
      (Components|SkeletalMesh|SetMorphTarget (Variables|Default|GetHead) (Utilities|Array|Get(acopy) (Variables|Default|GetEyes%20L/R) (Math|Conversions|ToInteger(Byte) (Variables|Default|GetEnemyCharacter))) (+ (* (Math|Trig|Cos(Degrees) (.yaw (Math|Rotator|FindLookatRotation (Transformation|GetActorLocation) (Transformation|GetActorLocation (Variables|Default|GetAttack%20Target))))) (Variables|Default|GetEyeRotation)) (Variables|Default|GetCenterEyeFrog)) true))))

(event Game|Damage|EventAnyDamage
  (params (Damage :type Float%20%28single-precision%29) (DamageType :type Damage%20Type%20Object%20Reference) (InstigatedBy :type Controller%20Object%20Reference) (DamageCauser :type Actor%20Object%20Reference))
  (bind _mesh (Variables|Character|GetMesh))
  ;[1 1 1] Enemy Hit Reaction
  (Utilities|IsValid DamageCauser
    (:Is%20Valid
      (Variables|Default|SetDamage%20Causer DamageCauser)
      (Variables|Default|SetDamageType (Utilities|GetClass DamageType))
      (if (not (< (- (Variables|Default|GetHealth) Damage) 0.0))
        (Variables|Default|SetHealth (- (Variables|Default|GetHealth) Damage))
        (Rendering|Material|SetMaterial (Variables|Character|GetMesh) 0 (Utilities|Array|Get(acopy) (Variables|Default|GetCharacterMaterial_Hit) (Math|Conversions|ToInteger(Byte) (Variables|Default|GetEnemyCharacter))))
        (if (Utilities|Enum|Equal(Enum) (Variables|Default|GetEnemyCharacter) "NewEnumerator2")
          (Rendering|Material|SetMaterial (Variables|Default|GetHead) 1 (Utilities|Array|Get(acopy) (Variables|Default|GetCharacterMaterial_Hit) (Math|Conversions|ToInteger(Byte) (Variables|Default|GetEnemyCharacter))))
          (else
            (Rendering|Material|SetMaterial (Variables|Default|GetHead) 0 (Utilities|Array|Get(acopy) (Variables|Default|GetCharacterMaterial_Hit) (Math|Conversions|ToInteger(Byte) (Variables|Default|GetEnemyCharacter))))))
        (if (Variables|Default|GetSlashing?)
          (Variables|Default|SetHitReactionInt 0 :!label _label)
          (elif (== (Variables|Default|GetDamageType) "/Game/Steven/Damage_Light.Damage_Light_C")
            (Variables|Default|SetHitReactionInt 1)
            (elif (== (Variables|Default|GetDamageType) "/Game/Steven/Damage_Medium.Damage_Medium_C")
              (Variables|Default|SetHitReactionInt 2)
              (else
                (goto _label)))))
        (if (or (> (.yaw (Math|Rotator|FindLookatRotation (Transformation|GetActorLocation) (Transformation|GetActorLocation (Variables|Default|GetDamage%20Causer)))) 9e+01) (< (.yaw (Math|Rotator|FindLookatRotation (Transformation|GetActorLocation) (Transformation|GetActorLocation (Variables|Default|GetDamage%20Causer)))) -9e+01))
          (Animation|Montage|PlayMontage _mesh (Utilities|Array|Get(acopy) (Variables|Default|GetHitReactionMontagesL) (Variables|Default|GetHitReactionInt))
            (:then
              _))
          (else
            (Animation|Montage|PlayMontage _mesh (Utilities|Array|Get(acopy) (Variables|Default|GetHitReactionMontagesR) (Variables|Default|GetHitReactionInt))
              (:then
                _))))
        (Utilities|FlowControl|Delay 0.3)
        (CallFunction|PickEnemyCharacter)))))

(fn ConstructionScript
  (switch int (Math|Random|RandomIntegerinRange 0 3)
    (:0
      (Variables|Default|SetEnemyCharacter "NewEnumerator0"))
    (:1
      (Variables|Default|SetEnemyCharacter "NewEnumerator1"))
    (:2
      (Variables|Default|SetEnemyCharacter "NewEnumerator2"))
    (:3
      (Variables|Default|SetEnemyCharacter "NewEnumerator3")))
  (CallFunction|PickEnemyCharacter))

(fn GetMeleeRange
  (return 1.5e+02))
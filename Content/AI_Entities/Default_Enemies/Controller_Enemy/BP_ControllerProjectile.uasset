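; Projectile for the Controller enemy that deals light damage on impact, then destroys itself.
; When its box overlaps anything other than the Controller class, it runs a short horizontal sphere trace toward that actor, ignoring Enemy- and Room-tagged actors, and damages the hit actor.
; It then attaches to the overlapped actor, stops moving and is destroyed after a brief delay.
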(event OnComponentBeginOverlap(Box)
  (params (OverlappedComponent :type Primitive%20Component%20Object%20Reference) (OtherActor :type Actor%20Object%20Reference) (OtherComp :type Primitive%20Component%20Object%20Reference) (OtherBodyIndex :type Integer) (bFromSweep :type Boolean) (SweepResult :type Hit%20Result%20Structure%20%28by%20ref%29))
  (bind _returnvalue (Transformation|GetActorLocation))
  (bind _returnvalue_2 (Transformation|GetActorLocation OtherActor))
  (bind _returnvalue_3 (Math|Rotator|FindLookatRotation _returnvalue _returnvalue_2))
  (if (not (== "/Game/AI_Entities/Default_Enemies/Controller_Enemy/Enemy_Controller_Character.Enemy_Controller_Character_C" (Utilities|GetClass OtherActor)))
    (bind _outactors (Actor|GetAllActorswithTag "Enemy"))
    (bind _outactors_2 (Actor|GetAllActorswithTag "Room"))
    (Utilities|Array|AppendArray _outactors _outactors_2)
    (bind _outhit (Collision|SphereTraceByChannel _returnvalue (+ _returnvalue (* (Math|Vector|MakeVector (Math|Trig|Cos(Degrees) (.yaw _returnvalue_3)) (Math|Trig|Sin(Degrees) (.yaw _returnvalue_3)) 0.0) 25.0)) 9e+01 "TraceTypeQuery1" false _outactors "ForOneFrame"))
    (Game|Damage|ApplyDamage (.HitActor (Collision|BreakHitResult _outhit)) 2.0 0 self "/Game/Steven/Blueprints/Damage_Light.Damage_Light_C")
    (Transformation|AttachActorToActor OtherActor "None" "KeepWorld" "KeepWorld" "KeepWorld" true)
    (Components|Movement|StopMovementImmediately (Variables|Default|GetProjectileMovement))
    (Utilities|FlowControl|Delay 0.2)
    (Actor|DestroyActor)))

(event EventBeginPlay
  (bind _asbp_third_person_character (Utilities|Casting|CastToBP_ThirdPersonCharacter (Components|GetOwner)))
  (Variables|Default|SetAs%20BP%20Third%20Person%20Character _asbp_third_person_character))

(event Collision|EventActorBeginOverlap
  (params (OtherActor :type Actor%20Object%20Reference)))

(event EventTick
  (params (DeltaSeconds :type Float%20%28single-precision%29)))

(fn ConstructionScript)